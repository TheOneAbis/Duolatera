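; VR game mode that numbers joining players and styles their hands.
; On PostLogin it prints the new player's name, waits briefly, then casts the controlled pawn to VRPawn.
; It writes a running player count into the pawn's PlayerID, increments the counter, then calls SetHandsMaterial on that pawn.
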(event EventPostLogin
  (params (NewPlayer :type Player%20Controller%20Object%20Reference))
  (Development|PrintString (Utilities|GetDisplayName NewPlayer))
  (Utilities|FlowControl|Delay 0.5)
  (bind _asvrpawn (Utilities|Casting|CastToVRPawn (Pawn|GetControlledPawn NewPlayer)))
  (Variables|/Game/Blueprints/Actors/VRPawn.VRPawn_C|SetPlayerID _asvrpawn (Variables|Default|GetAddedPlayer))
  (Variables|Default|SetAddedPlayer (+ (Variables|Default|GetAddedPlayer) 1))
  (Default|SetHandsMaterial _asvrpawn))

(fn ConstructionScript)