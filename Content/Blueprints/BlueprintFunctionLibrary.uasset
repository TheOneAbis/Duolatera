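; Blueprint function library with a helper that plays a haptic effect on the VR hand of a given motion controller.
; It casts the component's owner to VRPawn and continues only when that pawn is locally controlled.
; The effect plays through the pawn's owning PlayerController, on the left hand if the motion source is LeftGrip and on the right otherwise.
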(fn TriggerPlaysHapticEffect
  (params (motionControllerComp :type Motion%20Controller%20Component%20Object%20Reference) (hapticEffect :type Haptic%20Feedback%20Effect%20Base%20Object%20Reference))
  (bind _asvrpawn (Utilities|Casting|CastToVRPawn (Components|GetOwner motionControllerComp)))
  (if (Pawn|IsLocallyControlled _asvrpawn)
    (bind _asplayer_controller (Utilities|Casting|CastToPlayerController (Components|GetOwner _asvrpawn)))
    (Class|PlayerController|PlayHapticEffect _asplayer_controller hapticEffect (select (Utilities|Name|Equal(Name) (Variables|/Script/HeadMountedDisplay.MotionControllerComponent|GetMotionSource motionControllerComp) "LeftGrip") "Left" "Right") 1.0 false)))