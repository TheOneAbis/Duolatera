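; VR game instance that persists checkpoint progress and lets players resume their position when rejoining their last multiplayer session.
; Init loads or creates the BP_Checkpoint save object, and SaveToCheckpoint saves only when progress advances.
; Network or travel errors record session ID and a navmesh-projected player transform, tear down VOIP and session, then open Menu.
; CheckForReturning matches the stored session ID, letting ReturnToLastSession restore that transform locally and on the server.
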(event Custom|SaveCurrentSession
  ;[1 1 1] Save the session info.
  (Variables|/Game/Blueprints/BP_Checkpoint.BP_Checkpoint_C|SetLastSessionID (Variables|Default|GetCheckPoint) (Class|AdvancedSessionsLibrary|GetCurrentSessionIDasString))
  (CallFunction|SaveLastLegalTransform)
  (|AsyncSaveGametoSlot 0 "Save"))

(event Custom|CheckForReturning
  (params (Joining%20Session :type Blueprint%20Session%20Result%20Structure))
  (if (== (Variables|/Game/Blueprints/BP_Checkpoint.BP_Checkpoint_C|GetLastSessionID (Variables|Default|GetCheckPoint)) (Class|AdvancedSessionsLibrary|GetSessionIDasString Joining%20Session))
    (Variables|Default|SetisLastSession true)
    (Development|PrintString "WelcomeBack" true true "(R=1.000000,G=0.000000,B=0.000000,A=1.000000)" 2e+01)
    (else
      (Variables|Default|SetisLastSession false)
      (Development|PrintString "NewSession" true true "(R=1.000000,G=0.000000,B=0.000000,A=1.000000)" 2e+01))))

(event Custom|ReturnToLastSession
  (bind _checkpoint (Variables|Default|GetCheckPoint))
  (bind _lastknowntransform (Variables|/Game/Blueprints/BP_Checkpoint.BP_Checkpoint_C|GetLastKnownTransform _checkpoint))
  ;[1 1 1] Put player on last known location if they are returning.
  (if (Variables|Default|GetisLastSession)
    (bind _asvrpawn (Utilities|Casting|CastToVRPawn (Game|Player|GetPlayerPawn 0)))
    (Transformation|SetActorTransform _asvrpawn _lastknowntransform)
    (Default|ServerUpdateTM _asvrpawn _lastknowntransform)
    (Variables|Default|SetisLastSession false)))

(event Custom|SaveLastLegalTransform
  (bind _asvrpawn (Utilities|Casting|CastToVRPawn (Game|Player|GetPlayerPawn 0)))
  (bind (_islegal _closestlegalloc) (CallFunction|CheckifLegalPos (Transformation|GetWorldLocation (Variables|/Game/Blueprints/Actors/VRPawn.VRPawn_C|GetCamera _asvrpawn))))
  (if _islegal
    (bind _asvrpawn_2 (Utilities|Casting|CastToVRPawn (Game|Player|GetPlayerPawn 0)))
    (Variables|/Game/Blueprints/BP_Checkpoint.BP_Checkpoint_C|SetLastKnownTransform (Variables|Default|GetCheckPoint) (Math|Transform|MakeTransform (Math|Vector|MakeVector (.X (Math|Vector|BreakVector _closestlegalloc)) (.Y (Math|Vector|BreakVector _closestlegalloc)) (.z (.location (Transformation|GetActorTransform _asvrpawn_2)))) (Math|Rotator|MakeRotator (.roll (.rotation (Transformation|GetActorTransform _asvrpawn_2))) (.pitch (.rotation (Transformation|GetActorTransform _asvrpawn_2))) (.yaw (Transformation|GetWorldRotation (Variables|/Game/Blueprints/Actors/VRPawn.VRPawn_C|GetCamera _asvrpawn_2)))) (.scale (Transformation|GetActorTransform _asvrpawn_2))))))

(event Custom|SaveToCheckpoint
  (params (Checkpoint :type Integer))
  (if (> Checkpoint (Variables|/Game/Blueprints/BP_Checkpoint.BP_Checkpoint_C|GetLastCheckPoint (Variables|Default|GetCheckpoint)))
    (Variables|Default|SetActToLoad Checkpoint)
    (Variables|/Game/Blueprints/BP_Checkpoint.BP_Checkpoint_C|SetLastCheckPoint (Variables|Default|GetCheckpoint) Checkpoint)
    (bind _bsuccess (|AsyncSaveGametoSlot (Variables|Default|GetCheckpoint) "Save")
      (:then
        (if _bsuccess
          (Development|PrintString "Checkpoint Saved" true true "(R=0.000000,G=1.000000,B=0.500000,A=1.000000)" 5.0))))))

(event EventInit
  (bind _returnvalue (SaveGame|DoesSaveGameExist "Save"))
  (if _returnvalue
    (bind _returnvalue_2 (SaveGame|LoadGamefromSlot "Save"))
    (bind _asbp_checkpoint (Utilities|Casting|CastToBP_Checkpoint _returnvalue_2))
    (Variables|Default|SetCheckpoint _asbp_checkpoint)
    (else
      (bind _returnvalue_3 (SaveGame|CreateSaveGameObject "/Game/Blueprints/BP_Checkpoint.BP_Checkpoint_C"))
      (bind _output_get (Variables|Default|SetCheckpoint _returnvalue_3))
      (SaveGame|SaveGametoSlot _output_get "Save"))))

(event EventHandleNetworkError
  (params (FailureType :type ENetworkFailure%20Enum :default "NetDriverAlreadyExists") (bIsServer :type Boolean))
  (Development|PrintString (Utilities|String|EnumtoString FailureType) true true "(R=1.000000,G=0.000000,B=0.000000,A=1.000000)" 1e+01)
  (bind _asvrpawn (Utilities|Casting|CastToVRPawn (Game|Player|GetPlayerPawn 0)))
  (CallFunction|SaveCurrentSession)
  (Default|DestroyVOIP _asvrpawn)
  (Utilities|FlowControl|Delay 1.0)
  (|DestroySession (Game|GetPlayerController 0)
    (:OnSuccess
      (Game|OpenLevel(byObjectReference) "/Game/Levels/Menu.Menu")
      (Development|PrintString "VRGI: network error occurred, session end" true true "(R=1.000000,G=0.000000,B=0.004328,A=1.000000)" 3e+01))))

(event EventHandleTravelError
  (params (FailureType :type ETravelFailure%20Enum :default "NoLevel"))
  (Development|PrintString (Utilities|String|EnumtoString FailureType) true true "(R=1.000000,G=0.300000,B=0.000000,A=1.000000)" 1e+01)
  (bind _asvrpawn (Utilities|Casting|CastToVRPawn (Game|Player|GetPlayerPawn 0)))
  (CallFunction|SaveCurrentSession)
  (Default|DestroyVOIP _asvrpawn)
  (Utilities|FlowControl|Delay 1.0)
  (|DestroySession (Game|GetPlayerController 0)
    (:OnSuccess
      (Game|OpenLevel(byObjectReference) "/Game/Levels/Menu.Menu")
      (Development|PrintString "VRGI: network error occurred, session end" true true "(R=1.000000,G=0.000000,B=0.004328,A=1.000000)" 3e+01))))

(event EventShutdown
  (bind _asvrpawn (Utilities|Casting|CastToVRPawn (Game|Player|GetPlayerPawn 0)))
  (Input|DisableInput _asvrpawn 0))

(fn CheckifLegalPos
  (params (Position :type Vector))
  (bind (_projectedlocation _returnvalue) (AI|Navigation|ProjectPointtoNavigation Position 0 0 "500.000000,500.000000,500.000000"))
  (return _returnvalue _projectedlocation))