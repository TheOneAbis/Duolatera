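; BP_Door is a hinged door actor that swings open and closed.
; One timeline drives a yaw lerp on the Door's relative rotation up to a quarter turn, playing from the start to open and reversing to close.
; An IsOpen flag lets Toggle pick the direction and stops DoorInteractOpen and DoorInteractClose from repeating the current state.
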(event Custom|Open%20Door
  (Variables|Default|SetIsOpen true)
  (bind _timelinedoor (Timeline|OpenDoor PlayFromStart)
    (:Update
      (Transformation|SetRelativeRotation (Variables|Default|GetDoor) (Math|Rotator|MakeRotator 0.0 0.0 (Math|Float|Lerp 0.0 9e+01 _timelinedoor)) false false))))

(event Custom|Close%20Door
  (Variables|Default|SetIsOpen false)
  (bind _timelinedoor (Timeline|OpenDoor Reverse)
    (:Update
      (Transformation|SetRelativeRotation (Variables|Default|GetDoor) (Math|Rotator|MakeRotator 0.0 0.0 (Math|Float|Lerp 0.0 9e+01 _timelinedoor)) false false))))

(event EventTick
  (params (DeltaSeconds :type Float%20%28single-precision%29)))

(event EventToggle
  (if (Variables|Default|GetIsOpen)
    (CallFunction|CloseDoor)
    (else
      (CallFunction|OpenDoor))))

(event EventBeginPlay)

(event Collision|EventActorBeginOverlap
  (params (OtherActor :type Actor%20Object%20Reference)))

(event EventDoorInteractClose
  (if (Variables|Default|GetIsOpen)
    (CallFunction|CloseDoor)
    (Variables|Default|SetIsOpen false)))

(event EventDoorInteractOpen
  (if (not (Variables|Default|GetIsOpen))
    (CallFunction|OpenDoor)
    (Variables|Default|SetIsOpen true)))

(fn ConstructionScript)