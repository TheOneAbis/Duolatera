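; Trigger actor that swaps streamed sublevels and saves a checkpoint once the required number of players stand inside its volume.
; The server tracks overlapping Player-tagged actors, then blocking-loads the target level, unloads the previous one and Act1, and refreshes the VR game state.
; The overlap count's RepNotify triggers the save through the VR game instance and updates the online session's Act setting.
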(event OnComponentBeginOverlap(LoadVolumn)
  (params (OverlappedComponent :type Primitive%20Component%20Object%20Reference) (OtherActor :type Actor%20Object%20Reference) (OtherComp :type Primitive%20Component%20Object%20Reference) (OtherBodyIndex :type Integer) (bFromSweep :type Boolean) (SweepResult :type Hit%20Result%20Structure%20%28by%20ref%29))
  (bind _overlapactor (Variables|Default|GetOverlapActor))
  (Networking|SwitchHasAuthority
    (:Authority
      (if (Actor|ActorHasTag OtherActor "Player")
        (Utilities|Set|Add _overlapactor OtherActor)
        (Variables|Default|SetOverlappingPlayer (Utilities|Set|Length _overlapactor))
        (if (== (Variables|Default|GetOverlappingPlayer) (Variables|Default|GetRequiredPlayers))
          (CallFunction|LoadSubLevel))))))

(event OnComponentEndOverlap(LoadVolumn)
  (params (OverlappedComponent :type Primitive%20Component%20Object%20Reference) (OtherActor :type Actor%20Object%20Reference) (OtherComp :type Primitive%20Component%20Object%20Reference) (OtherBodyIndex :type Integer))
  (bind _overlapactor (Variables|Default|GetOverlapActor))
  (Networking|SwitchHasAuthority
    (:Authority
      (if (Actor|ActorHasTag OtherActor "Player")
        (Utilities|Set|Remove _overlapactor OtherActor)
        (Variables|Default|SetOverlappingPlayer (Utilities|Set|Length _overlapactor))))))

(event Custom|LoadSubLevel
  (if (and (Utilities|IsValidSoftObjectReference (Variables|Default|GetLevelToLoad)) (Utilities|IsValidSoftObjectReference (Variables|Default|GetLevelToUnload)))
    (if (not (Class|LevelStreaming|IsLevelLoaded (Class|GameplayStatics|GetStreamingLevel (Variables|Default|GetLevelToLoadName))))
      (Class|GameplayStatics|LoadStreamLevelbySoftObjectPtr (Variables|Default|GetLevelToLoad) true true)
      (Class|GameplayStatics|UnloadStreamLevelbySoftObjectPtr (Variables|Default|GetLevelToUnload) true)
      (Class|GameplayStatics|UnloadStreamLevelbySoftObjectPtr "/Game/Levels/Act1.Act1" true)
      (bind _asvrgame_state (Utilities|Casting|CastToVRGameState (Game|GetGameState)))
      (Default|RefreshGameState _asvrgame_state))))

(event Custom|SaveGame
  (bind _checkpointnum (Variables|Default|GetCheckPointNum))
  (bind _asvrgame_instance (Utilities|Casting|CastToVRGameInstance (Game|GetGameInstance)))
  (Default|SavetoCheckpoint _asvrgame_instance _checkpointnum)
  (|UpdateSession (Utilities|Array|MakeArray (Class|AdvancedSessionsLibrary|MakeLiteralSessionPropertyString "Act" (Utilities|String|Append "Act " (Utilities|String|ToString(Integer) _checkpointnum)))) 2 0 false true true true false true))

(event EventBeginPlay)

(event Collision|EventActorBeginOverlap
  (params (OtherActor :type Actor%20Object%20Reference)))

(event EventTick
  (params (DeltaSeconds :type Float%20%28single-precision%29)))

(fn ConstructionScript)

(fn OnRepOverlappingPlayer
  (if (== (Variables|Default|GetOverlappingPlayer) (Variables|Default|GetRequiredPlayers))
    (CallFunction|SaveGame)))