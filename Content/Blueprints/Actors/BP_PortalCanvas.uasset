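; VR portal canvas actor that shows strokes drawn on it, with an overworld or underworld look for surface and frame set at construction.
; New points become line segments stamped by a draw material into a render target, which masks the layered canvas material.
; Each draw source's last point is cached to join strokes, and closing the portal clears the target.
; Portal references come from VRGameState, with an event fallback if portals are not yet created.
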(event Custom|OnPortalsCreated_Event
  (params (OverPortal :type BP%20Portal%20Object%20Reference) (UnderPortal :type BP%20Portal%20Object%20Reference))
  ;[0.4089 0.6042 0.3103] If we're not in the Gameworld, this will execute before VRGameState, meaning the portals won't be created yet. So, listen for that to happen, then set the portal references again.
  (Variables|Default|SetoverPortal OverPortal)
  (Variables|Default|SetunderPortal UnderPortal))

(event Custom|DrawOnPortal
  (params (drawSource :type Actor%20Object%20Reference) (newPoints :type Array%20of%20Vector%202D%20Structures) (lastDrawnPoint :type Vector%202D%20Structure))
  (bind _mid_draw (Variables|Default|GetMID_Draw))
  (bind _lastdrawnpts (Variables|Default|GetlastDrawnPts))
  (bind _value (Utilities|Map|Find _lastdrawnpts drawSource))
  (Utilities|FlowControl|Sequence
    (:then_0
      (if (not (> (.X (Math|Vector2D|BreakVector2D lastDrawnPoint)) 5e+01))
        (Utilities|Array|Insert newPoints lastDrawnPoint)
        (if (Utilities|Operators|EqualEqual lastDrawnPoint _value 0.0)
          _
          (else
            (Utilities|Array|Insert newPoints _value)))
        (for _index (range 0 (- (Utilities|Array|LastIndex newPoints) 1))
          (Rendering|Material|SetVectorParameterValue _mid_draw "ImpactUV1" (Math|Conversions|ToLinearColor(Vector) (Math|Conversions|ToVector(Vector2D) (+ (/ (Utilities|Array|Get(acopy) newPoints _index) "(X=100.000000,Y=-100.000000)") "(X=0.500000,Y=0.500000)"))) :!class /Script/Engine.MaterialInstanceDynamic)
          (Rendering|Material|SetVectorParameterValue _mid_draw "ImpactUV2" (Math|Conversions|ToLinearColor(Vector) (Math|Conversions|ToVector(Vector2D) (+ (/ (Utilities|Array|Get(acopy) newPoints (+ _index 1)) "(X=100.000000,Y=-100.000000)") "(X=0.500000,Y=0.500000)"))) :!class /Script/Engine.MaterialInstanceDynamic)
          (Rendering|DrawMaterialtoRenderTarget (Variables|Default|GetRT_Hit) (Variables|Default|GetMID_Draw)))))
    (:then_1
      (Utilities|Map|Add (Variables|Default|GetlastDrawnPts) drawSource (Utilities|Array|Get(acopy) newPoints (Utilities|Array|LastIndex newPoints))))))

(event Custom|OnPortalClosed_Event
  (params (closedCanvas :type Portal%20Canvas%20Object%20Reference))
  (Rendering|ClearRenderTarget2D (Variables|Default|GetRT_Hit)))

(event EventBeginPlay
  (Utilities|FlowControl|Sequence
    (:then_0
      (bind _asvrgame_state (Utilities|Casting|CastToVRGameState (Game|GetGameState)))
      (Variables|Default|SetoverPortal (Variables|/Game/Blueprints/VRGameState.VRGameState_C|GetoverPortal _asvrgame_state))
      (bind _output_get (Variables|Default|SetunderPortal (Variables|/Game/Blueprints/VRGameState.VRGameState_C|GetunderPortal _asvrgame_state)))
      ;[0.4089 0.6042 0.3103] If we're not in the Gameworld, this will execute before VRGameState, meaning the portals won't be created yet. So, listen for that to happen, then set the portal references again.
      (Utilities|IsValid _output_get
        (:Is%20Not%20Valid
          (EventDispatchers|AssignOnPortalsCreated _asvrgame_state (delegate Custom|OnPortalsCreated_Event)))))
    (:then_1
      (bind _returnvalue (Rendering|CreateRenderTarget2D 1024 1024 "RTF_RGBA16f"))
      (bind _output_get_2 (Variables|Default|SetRT_Hit _returnvalue))
      (Class|MaterialInstanceDynamic|SetTextureParameterValuebyInfo (Variables|Default|GetMID_PortalCanvasDraw) (Utilities|Struct|MakeMaterialParameterInfo "DrawMask" "BlendParameter" 0) _output_get_2)
      (Rendering|ClearRenderTarget2D (Variables|Default|GetRT_Hit))
      (bind _returnvalue_2 (Rendering|Material|CreateDynamicMaterialInstance "/Game/Assets/Materials/Portals/M_Draw.M_Draw" "MID_Draw" "None" :!class /Script/Engine.KismetMaterialLibrary))
      (bind _output_get_3 (Variables|Default|SetMID_Draw _returnvalue_2))
      (Rendering|Material|SetScalarParameterValue _output_get_3 "Thickness" (Variables|Default|GetDrawThickness) :!class /Script/Engine.MaterialInstanceDynamic))
    (:then_2
      (EventDispatchers|AssignOnDrawPointsAdded (delegate Custom|DrawOnPortal))
      (EventDispatchers|AssignOnPortalClosed (delegate Custom|OnPortalClosed_Event)))))

(fn ConstructionScript
  (bind _proceduralmesh (Variables|Default|GetProceduralMesh))
  (bind _portalframe (Variables|Default|GetPortalFrame))
  (Utilities|FlowControl|Sequence
    (:then_0
      (bind _returnvalue (Rendering|Material|CreateDynamicMaterialInstance "/Game/Assets/Materials/Portals/MI_PortalCanvasDraw.MI_PortalCanvasDraw" "MID_PortalCanvasDraw" "None" :!class /Script/Engine.KismetMaterialLibrary))
      (bind _output_get (Variables|Default|SetMID_PortalCanvasDraw _returnvalue))
      (Rendering|Material|SetMaterial _proceduralmesh 0 _output_get)
      (Rendering|Material|SetMaterial _proceduralmesh 1 _output_get)
      (Rendering|Material|SetScalarParameterValuebyInfo _output_get (Utilities|Struct|MakeMaterialParameterInfo "TaggablePatternScale" "LayerParameter" 0) (Variables|Default|GetTaggableScale))
      (Rendering|Material|SetScalarParameterValuebyInfo _output_get (Utilities|Struct|MakeMaterialParameterInfo "IsUnderworld" "LayerParameter" 1) (Math|Conversions|ToFloat(Boolean) (Variables|Default|GetisUnderworldCanvas))))
    (:then_1
      (if (Variables|Default|GetisUnderworldCanvas)
        (bind _returnvalue_2 (Rendering|Material|CreateDynamicMaterialInstance _portalframe 0 (Variables|Default|GetFrameUnderworldMI) "None" :!class /Script/Engine.PrimitiveComponent))
        (Rendering|Material|SetMaterial _portalframe 0 _returnvalue_2)
        (else
          (bind _returnvalue_3 (Rendering|Material|CreateDynamicMaterialInstance _portalframe 0 (Variables|Default|GetFrameOverworldMI) "None" :!class /Script/Engine.PrimitiveComponent))
          (Rendering|Material|SetMaterial _portalframe 0 _returnvalue_3))))))