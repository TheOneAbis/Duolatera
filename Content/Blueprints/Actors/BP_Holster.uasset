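; Holster actor that returns its pistol (laser tool) to the holster and disables the gun mesh's physics.
; InitializeHolster listens for the pistol's grab-component drop, which triggers a server RPC that waits three seconds and snaps the pistol back if it is not held.
; Any pistol overlapping the box is also attached immediately, on authority only.
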(event OnComponentBeginOverlap(Box)
  (params (OverlappedComponent :type Primitive%20Component%20Object%20Reference) (OtherActor :type Actor%20Object%20Reference) (OtherComp :type Primitive%20Component%20Object%20Reference) (OtherBodyIndex :type Integer) (bFromSweep :type Boolean) (SweepResult :type Hit%20Result%20Structure%20%28by%20ref%29))
  (bind _aspistol (Utilities|Casting|CastToPistol OtherActor))
  (Networking|SwitchHasAuthority
    (:Authority
      (Transformation|AttachComponentToComponent _aspistol (Variables|Default|GetHolster) "None" "SnapToTarget" "SnapToTarget" "SnapToTarget" true)
      (bind _aspistol_2 (Utilities|Casting|CastToPistol OtherActor))
      (Physics|SetSimulatePhysics (Variables|/Game/Blueprints/Actors/Pistol.Pistol_C|GetSkeletalMeshGun _aspistol_2) false))))

(event Custom|OnPistolDropped
  (CallFunction|RPCServerTryRetractLazerTool))

(event Custom|InitializeHolster
  (EventDispatchers|BindEventtoOnDropped (Variables|/Game/Blueprints/Actors/Pistol.Pistol_C|GetGrabComponentSnap (Variables|Default|GetPistolReference)) (delegate Custom|OnPistolDropped)))

(event Custom|RPC_Server_TryRetractLazerTool
  (bind _pistolreference (Variables|Default|GetPistolReference))
  (Utilities|FlowControl|Delay 3.0)
  (bind _isheld (Default|CheckifHeld (Variables|/Game/Blueprints/Actors/Pistol.Pistol_C|GetGrabComponentSnap (Variables|Default|GetPistolReference))))
  (if (not _isheld)
    (Transformation|AttachComponentToComponent _pistolreference (Variables|Default|GetHolster) "None" "SnapToTarget" "SnapToTarget" "SnapToTarget" true)
    (Physics|SetSimulatePhysics (Variables|/Game/Blueprints/Actors/Pistol.Pistol_C|GetSkeletalMeshGun _pistolreference) false)))

(fn ConstructionScript)

(fn OnRepBIsPistolinHand)

(fn SetPistolReference
  (params (PistolReference :type Pistol%20Object%20Reference))
  (Variables|Default|SetPistolReference PistolReference))