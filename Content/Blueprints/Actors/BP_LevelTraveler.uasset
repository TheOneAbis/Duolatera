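; BP_LevelTraveler is an actor that moves the multiplayer session to another level through server travel.
; On authority, Activate calls a multicast to disable voice chat on player pawn 0 and start its HUD transition fade with text.
; It then waits briefly before traveling to LevelToOpen.
; A separate server RPC event enters at the delay, skipping the voice and fade step.
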(event Custom|RPC_Server_Servertravel
  (Utilities|FlowControl|Delay 3.0)
  (Class|AdvancedSessionsLibrary|ServerTravel (Variables|Default|GetlevelToOpen) false false))

(event Custom|DisableVoiceChats%20%28Multi%29
  (bind _asvrpawn (Utilities|Casting|CastToVRPawn (Game|Player|GetPlayerPawn 0)))
  (Default|DisableVoiceChat _asvrpawn)
  (bind _aswb_hud (Utilities|Casting|CastToWB_HUD (UserInterface|GetWidget (Variables|/Game/Blueprints/Actors/VRPawn.VRPawn_C|GetHUD _asvrpawn))))
  (Default|BeginLevelTransitionFade _aswb_hud (Variables|Default|GetFadeScreenText)))

(event EventActivate
  (Networking|SwitchHasAuthority
    (:Authority
      (CallFunction|DisableVoiceChats(Multi))
      (Utilities|FlowControl|Delay 3.0)
      (Class|AdvancedSessionsLibrary|ServerTravel (Variables|Default|GetlevelToOpen) false false))))

(fn ConstructionScript)