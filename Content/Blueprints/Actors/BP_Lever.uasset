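; A VR lever actor that can be dragged by a grabbing hand or animated between two positions.
; While grabbed, it projects the hand onto the lever's swing plane and clamps height to the pivot to set rotation.
; The IsDown RepNotify plays or reverses a rotation timeline and calls BeginInteract or EndInteract.
; The overlap events are empty, and the authority and haptic logic that would toggle IsDown is disconnected.
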(event OnComponentBeginOverlap(Box)
  (params (OverlappedComponent :type Primitive%20Component%20Object%20Reference) (OtherActor :type Actor%20Object%20Reference) (OtherComp :type Primitive%20Component%20Object%20Reference) (OtherBodyIndex :type Integer) (bFromSweep :type Boolean) (SweepResult :type Hit%20Result%20Structure%20%28by%20ref%29))
  ;[0.5156 0.5156 0.5156] Begin Overlap
)

(event OnComponentEndOverlap(Box)
  (params (OverlappedComponent :type Primitive%20Component%20Object%20Reference) (OtherActor :type Actor%20Object%20Reference) (OtherComp :type Primitive%20Component%20Object%20Reference) (OtherBodyIndex :type Integer))
  ;[0.6094 0.6094 0.6094] End Overlap
)

(event Custom|OpenLeverActorInteract
  ;[0.6198 0.6198 0.6198] OnRep Events
  (CallFunction|OpenLever)
  (Class|Interactable|BeginInteract 0))

(event Custom|Open%20Lever
  ;[0.6458 0.6458 0.6458] Timeline for Door open and close
  (bind _alpha (Timeline|LeverTimeline Play)
    (:Update
      (Transformation|SetRelativeRotation (Variables|Default|GetLever) (Math|Rotator|Lerp(Rotator) "-40.000000,0.000000,0.000000" "-120.000000,0.000000,0.000000" _alpha) false false))))

(event Custom|Close%20Lever
  ;[0.6458 0.6458 0.6458] Timeline for Door open and close
  (bind _alpha (Timeline|LeverTimeline Reverse)
    (:Update
      (Transformation|SetRelativeRotation (Variables|Default|GetLever) (Math|Rotator|Lerp(Rotator) "-40.000000,0.000000,0.000000" "-120.000000,0.000000,0.000000" _alpha) false false))))

(event Custom|CloseLeverActorInteract
  ;[0.6198 0.6198 0.6198] OnRep Events
  (CallFunction|CloseLever)
  (Class|Interactable|EndInteract 0))

(event EventBeginPlay
  (Default|GetRootComponent (Variables|Default|GetGrabComponent) (Variables|Default|GetDefaultSceneRoot)))

(event EventOnConstrainedGrabbed
  (params (grabbingCompRef :type Transform))
  (bind _lever (Variables|Default|GetLever))
  (bind _grabcomponent (Variables|Default|GetGrabComponent))
  (bind _grabcomponent_2 (Variables|Default|GetGrabComponent))
  (bind _lever_2 (Variables|Default|GetLever))
  (bind _returnvalue (Transformation|GetWorldLocation _lever_2))
  (bind _root_component (Variables|/Game/Blueprints/Components/GrabComponent.GrabComponent_C|GetRoot%20Component _grabcomponent))
  (bind _root_component_2 (Variables|/Game/Blueprints/Components/GrabComponent.GrabComponent_C|GetRoot%20Component _grabcomponent_2))
  (bind _returnvalue_2 (Math|Vector|GetRightVector _root_component_2))
  (bind _returnvalue_3 (Transformation|GetWorldLocation _root_component))
  (bind _returnvalue_4 (- (.location grabbingCompRef) _returnvalue))
  (bind _returnvalue_5 (Math|Vector|DotProduct _returnvalue_4 _returnvalue_2))
  (bind _returnvalue_6 (* _returnvalue_5 _returnvalue_2))
  (bind _returnvalue_7 (- _returnvalue_4 _returnvalue_6))
  (bind _returnvalue_8 (+ _returnvalue_3 _returnvalue_7))
  (bind (_x _y _z) (Math|Vector|BreakVector _returnvalue_8))
  (Transformation|SetWorldRotation (Variables|Default|GetLever) (Math|Rotator|MakeRotfromZY (- (Math|Vector|MakeVector _x _y (Math|Float|Max(Float) _z (.z (Transformation|GetWorldLocation (Variables|Default|GetLever))))) (Transformation|GetWorldLocation _lever)) (Math|Vector|GetRightVector _lever)) false false))

(event EventOnConstrainedReleased
  (Development|PrintString "Released"))

(fn ConstructionScript)

(fn OnRepBIsDown
  (if (Variables|Default|GetbIsDown)
    (CallFunction|OpenLeverActorInteract)
    (else
      (CallFunction|CloseLeverActorInteract))))