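; Chest actor that, when activated, opens and raises holster and pistol elevators.
; BeginPlay caches the world locations of the ChestD part and both elevators.
; Activate sets an Opened flag and plays one timeline that lerps ChestD mostly along world X with a slight lift, while both elevators rise together along Z.
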(event Custom|OpenAndRaise
  (bind _initiall_glass (Variables|Default|GetInitialL_glass))
  (bind _holsterela (Variables|Default|GetHolsterEla))
  (bind _pistolela (Variables|Default|GetPistolEla))
  (bind _timeline (Timeline|TimeLine Play)
    (:Update
      (Transformation|SetWorldLocation (Variables|Default|GetChest_D) (Math|Vector|Lerp(Vector) _initiall_glass (+ _initiall_glass (Math|Vector|MakeVector (+ 9e+01 0.0) 0.0 (+ 5.0 0.0))) _timeline) false false)
      (Transformation|SetWorldLocation (Variables|Default|GetHolsterElavator) (Math|Vector|Lerp(Vector) _holsterela (+ _holsterela (Math|Vector|MakeVector 0.0 0.0 4e+01)) _timeline) false false)
      (Transformation|SetWorldLocation (Variables|Default|GetPistolElavaor) (Math|Vector|Lerp(Vector) _pistolela (+ _pistolela (Math|Vector|MakeVector 0.0 0.0 4e+01)) _timeline) false false))))

(event EventBeginPlay
  (Variables|Default|SetInitialL_glass (Transformation|GetWorldLocation (Variables|Default|GetChest_D)))
  (Variables|Default|SetHolsterEla (Transformation|GetWorldLocation (Variables|Default|GetHolsterElavator)))
  (Variables|Default|SetPistolEla (Transformation|GetWorldLocation (Variables|Default|GetPistolElavaor))))

(event Collision|EventActorBeginOverlap
  (params (OtherActor :type Actor%20Object%20Reference)))

(event EventTick
  (params (DeltaSeconds :type Float%20%28single-precision%29)))

(event EventActivate
  (Variables|Default|SetOpened true)
  (CallFunction|OpenandRaise))

(fn ConstructionScript)