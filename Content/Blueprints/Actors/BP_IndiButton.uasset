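; A one-shot pressable VR button actor that slides inward and toggles a linked door interactable.
; Overlapping its Box while unpressed triggers a haptic effect using the overlapping component, then sets IsPressed on the server if the actor is a VRPawn.
; The IsPressed RepNotify animates the button from its stored start position and calls Toggle on the Interactable through BPI_Door_Interactable.
; Nothing in the graph resets the pressed state.
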(event OnComponentBeginOverlap(Box)
  (params (OverlappedComponent :type Primitive%20Component%20Object%20Reference) (OtherActor :type Actor%20Object%20Reference) (OtherComp :type Primitive%20Component%20Object%20Reference) (OtherBodyIndex :type Integer) (bFromSweep :type Boolean) (SweepResult :type Hit%20Result%20Structure%20%28by%20ref%29))
  ;[0.5573 0.5573 0.5573] Begin Overlap
  (if (not (Variables|Default|GetbIsPressed))
    (Utilities|FlowControl|Sequence
      (:then_0
        (CallFunction|TriggerPlaysHapticEffect OtherComp (Variables|Default|GetHapticEffect)))
      (:then_1
        (Utilities|Casting|CastToVRPawn OtherActor)
        (Networking|SwitchHasAuthority
          (:Authority
            (if (not (Variables|Default|GetbIsPressed))
              (Variables|Default|SetbIsPressed true))))))))

(event Custom|TriggerButtonMoveDoor
  ;[0.526 0.526 0.526] OnRep Event
  (Components|MoveComponentTo (Variables|Default|GetButton) (- (Variables|Default|GetButtonStart) "0.000000,20.000000,0.000000") "0, 0, 0" false false 0.1 false)
  (bind _asbpi_door_interactable (Utilities|Casting|CastToBPI_Door_Interactable (Variables|Default|GetInteractable)))
  (Default|Toggle _asbpi_door_interactable))

(event EventBeginPlay
  ;[1 1 1] Button Start Location
  (Variables|Default|SetButtonStart (Variables|/Script/Engine.SceneComponent|GetRelativeLocation (Variables|Default|GetButton))))

(fn ConstructionScript)

(fn OnRepBIsPressed
  (CallFunction|TriggerBUttonMoveDoor))