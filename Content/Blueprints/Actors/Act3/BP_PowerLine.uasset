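; BP_PowerLine is an Act 3 power line actor whose meshes change glow intensity when activated or deactivated.
; Activate plays a Fade timeline that lerps Glow from dim to bright, and Deactivate reverses it.
; Glow's OnRep function pushes the value to the "Glow" material parameter on every static mesh component.
; The construction script assigns Glow to itself, triggering that function to apply the initial value.
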(event EventActivate
  (bind _alpha (Timeline|Fade Play)
    (:Update
      (Variables|Default|Setglow (Math|Float|Lerp 3e+01 6e+01 _alpha)))))

(event EventDeactivate
  (bind _alpha (Timeline|Fade Reverse)
    (:Update
      (Variables|Default|Setglow (Math|Float|Lerp 3e+01 6e+01 _alpha)))))

(fn ConstructionScript
  (Variables|Default|Setglow (Variables|Default|Getglow)))

(fn OnRepGlow
  (for _array_element (Actor|GetComponentsByClass "/Script/Engine.StaticMeshComponent")
    (Rendering|Material|SetScalarParameterValueonMaterials _array_element "Glow" (Variables|Default|Getglow))))