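; BP_Act3Music is the Act 3 music actor, layering music to match the progress of a referenced SymbolColumn.
; On authority, it binds to the column's progress and reset events, which set or zero the replicated MusicLayers count.
; Its RepNotify sets LayerNGain float parameters on the audio component, turning the active layers on and the rest of the four off.
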(event Custom|OnProgressAdvanced_Event
  (params (Current%20Progress :type Integer))
  (Variables|Default|SetMusicLayers Current%20Progress))

(event Custom|OnColumnReset_Event
  (Variables|Default|SetMusicLayers 0))

(event EventBeginPlay
  (bind _symbolcolumn (Variables|Default|GetSymbolColumn))
  (Networking|SwitchHasAuthority
    (:Authority
      (EventDispatchers|AssignOnProgressAdvanced _symbolcolumn (delegate Custom|OnProgressAdvanced_Event))
      (EventDispatchers|AssignOnColumnReset _symbolcolumn (delegate Custom|OnColumnReset_Event)))))

(fn ConstructionScript)

(fn OnRepMusicLayers
  (bind _musiclayers (Variables|Default|GetMusicLayers))
  (bind _audiocomponent (Variables|Default|GetAudioComponent))
  (for _index (range 1 _musiclayers)
    (Audio|Parameter|SetFloatParameter _audiocomponent (Utilities|String|StringToName (Utilities|String|BuildString(Integer) "Layer" "" _index "Gain")) 1.0 :!class /Script/Engine.AudioComponent))
  (for _index_2 (range (+ _musiclayers 1) 4)
    (Audio|Parameter|SetFloatParameter _audiocomponent (Utilities|String|StringToName (Utilities|String|BuildString(Integer) "Layer" "" _index_2 "Gain")) 0.0 :!class /Script/Engine.AudioComponent)))