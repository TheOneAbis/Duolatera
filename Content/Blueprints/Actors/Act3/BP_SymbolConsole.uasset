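; Act 3 puzzle console, paired with a partner console, where correct symbols must be selected on both within a time window.
; The first selection locks its console and starts a multicast timer display on both.
; Matching the control column's required glyphs advances both, while mistakes or timeouts reset and temporarily disable them.
; Completing the column extrudes a grabbable SymbolKey and moves the ring sensor; input bindings are authority-only.
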(event Custom|OnInteractBegin_Event
  (params (interactedActor :type Interactable%20Object%20Reference))
  (bind _partnerconsole (Variables|SymbolConsole|GetpartnerConsole))
  (for _array_element (Variables|Default|GetUntaggedConsoleSymbols)
    (if (== _array_element interactedActor)
      (Variables|Default|SetselectedSymbol _array_element)
      (else
        (Default|SetSymbolState _array_element "NewEnumerator1"))))
  (if (Variables|BP_SymbolConsole_C|GetawaitingOtherInput (Variables|SymbolConsole|GetpartnerConsole))
    (if (and (SymbolConsole|IsSelectedSymbolCorrect) (SymbolConsole|IsSelectedSymbolCorrect (Variables|SymbolConsole|GetpartnerConsole)))
      (CallFunction|AdvanceState)
      (CallFunction|AdvanceState _partnerconsole)
      (else
        (CallFunction|DisableConsole 1.5 :!label _label)
        (CallFunction|DisableConsole (Variables|SymbolConsole|GetpartnerConsole) 1.5)))
    (else
      (Variables|Default|SetawaitingOtherInput true)
      (SymbolConsole|SetConsoleLocked true)
      (CallFunction|SetAnimateTimer(Multi) true)
      (CallFunction|SetAnimateTimer(Multi) _partnerconsole true)
      (Timeline|TimedInput PlayFromStart
        (:Finished
          (goto _label))))))

(event Custom|Set%20Symbol%20States
  (params (ConsoleState :type SymbolState%20Enum :default "NewEnumerator0") (UntaggedOnly :type Boolean))
  (for _array_element (select UntaggedOnly (Variables|Default|GetUntaggedConsoleSymbols) (Variables|SymbolConsole|GetConsoleSymbols))
    (Default|SetSymbolState _array_element ConsoleState)))

(event Custom|Disable%20Console
  (params (Reenable%20delay :type Float%20%28double-precision%29))
  (Utilities|FlowControl|Sequence
    (:then_0
      (Variables|Default|SetUntaggedConsoleSymbols (Variables|SymbolConsole|GetConsoleSymbols))
      (CallFunction|SetAnimateTimer(Multi) false)
      (Timeline|TimedInput Stop
        (:Finished
          (CallFunction|DisableConsole 1.5)
          (CallFunction|DisableConsole (Variables|SymbolConsole|GetpartnerConsole) 1.5))))
    (:then_1
      (Variables|Default|SetawaitingOtherInput false)
      (SymbolConsole|SetConsoleLocked true)
      (CallFunction|SetSymbolStates "NewEnumerator0" false)
      (Variables|Default|SetselectedSymbol 0)
      (Class|Activatable|RemoveActivator (Variables|SymbolConsole|GetSymbolDisplayColumn) self)
      (Default|Reset (Variables|SymbolConsole|GetSymbolControlColumn) true)
      (Default|CallOnConsoleDisabled)
      (if (>= Reenable%20delay 0.0)
        (Utilities|FlowControl|Delay Reenable%20delay)
        (SymbolConsole|SetConsoleLocked false)
        (Class|Activatable|AddActivator (Variables|SymbolConsole|GetSymbolDisplayColumn) self)
        (Default|CallOnConsoleEnabled)))))

(event Custom|AdvanceState
  (Utilities|Array|RemoveItem (Variables|Default|GetUntaggedConsoleSymbols) (Variables|Default|GetselectedSymbol))
  (Default|AdvanceProgress (Variables|SymbolConsole|GetSymbolControlColumn))
  (Variables|Default|SetawaitingOtherInput false)
  (SymbolConsole|SetConsoleLocked false)
  (CallFunction|SetAnimateTimer(Multi) false)
  (Timeline|TimedInput Stop
    (:Finished
      (CallFunction|DisableConsole 1.5)
      (CallFunction|DisableConsole (Variables|SymbolConsole|GetpartnerConsole) 1.5))))

(event Custom|OnColumnComplete_Event
  (bind _symbolkey (Variables|SymbolConsole|GetSymbolKey))
  (bind _symbolkey_2 (Variables|SymbolConsole|GetSymbolKey))
  ;[0.4531 0.1392 0.1121] Begins Phase 2
  (Variables|/Game/Blueprints/Components/GrabComponent.GrabComponent_C|SetbSimulateOnDrop (Variables|/Game/Blueprints/Actors/Act3/BP_GrabbableSymbol.BP_GrabbableSymbol_C|GetGrabComponent _symbolkey_2) true)
  (Utilities|FlowControl|Sequence
    (:then_0
      (Default|SetSymbolState _symbolkey_2 "NewEnumerator1")
      (Variables|Default|SetkeyStartPt (Transformation|GetActorLocation _symbolkey_2))
      (bind _distance (Timeline|SymbolExtrude PlayFromStart)
        (:Update
          (Transformation|SetActorLocation _symbolkey (+ (Variables|Default|GetkeyStartPt) (* (Transformation|GetActorUpVector _symbolkey) _distance)) false false))
        (:Finished
          (Variables|/Game/Blueprints/Components/GrabComponent.GrabComponent_C|SetcanGrab (Variables|/Game/Blueprints/Actors/Act3/BP_GrabbableSymbol.BP_GrabbableSymbol_C|GetGrabComponent _symbolkey) true)
          (Physics|SetSimulatePhysics (Variables|/Game/Blueprints/Actors/BP_Symbol.BP_Symbol_C|GetFrame _symbolkey) true))))
    (:then_1
      (CallFunction|HideRingSensor))))

(event Custom|Set%20Animate%20Timer%20%28Multi%29
  (params (Should%20Animate :type Boolean))
  (bind _output_get (Variables|Default|SettimerAlpha (Math|Float|SelectFloat 1.0 0.0 Should%20Animate)))
  (Rendering|Material|SetScalarParameterValueonMaterials (Variables|Default|GetTimerDisplay) "Fill" _output_get)
  (Actor|Tick|SetActorTickEnabled Should%20Animate))

(event Custom|Debug
  (bind _symbolkey (Variables|SymbolConsole|GetSymbolKey))
  (bind _symbolkey_2 (Variables|SymbolConsole|GetSymbolKey))
  ;[0.4531 0.1392 0.1121] Begins Phase 2
  (Utilities|FlowControl|Delay 3.0)
  (Variables|/Game/Blueprints/Components/GrabComponent.GrabComponent_C|SetbSimulateOnDrop (Variables|/Game/Blueprints/Actors/Act3/BP_GrabbableSymbol.BP_GrabbableSymbol_C|GetGrabComponent _symbolkey_2) true)
  (Utilities|FlowControl|Sequence
    (:then_0
      (Default|SetSymbolState _symbolkey_2 "NewEnumerator1")
      (Variables|Default|SetkeyStartPt (Transformation|GetActorLocation _symbolkey_2))
      (bind _distance (Timeline|SymbolExtrude PlayFromStart)
        (:Update
          (Transformation|SetActorLocation _symbolkey (+ (Variables|Default|GetkeyStartPt) (* (Transformation|GetActorUpVector _symbolkey) _distance)) false false))
        (:Finished
          (Variables|/Game/Blueprints/Components/GrabComponent.GrabComponent_C|SetcanGrab (Variables|/Game/Blueprints/Actors/Act3/BP_GrabbableSymbol.BP_GrabbableSymbol_C|GetGrabComponent _symbolkey) true)
          (Physics|SetSimulatePhysics (Variables|/Game/Blueprints/Actors/BP_Symbol.BP_Symbol_C|GetFrame _symbolkey) true))))
    (:then_1
      (CallFunction|HideRingSensor))))

(event Custom|HideRingSensor
  (bind _ringsensor (Variables|SymbolConsole|GetringSensor))
  (bind _returnvalue (Transformation|GetActorLocation _ringsensor))
  (bind (_direction _ringsensorheight _powerlineglow) (Timeline|RingSensorAnimation PlayFromStart)
    (:Update
      (Transformation|SetActorLocation _ringsensor (Math|Vector|MakeVector (.x _returnvalue) (.y _returnvalue) _ringsensorheight) false false)
      (Variables|/Game/Blueprints/Actors/Act3/BP_PowerLine.BP_PowerLine_C|Setglow (Variables|SymbolConsole|GetpowerLine) _powerlineglow))))

(event EventBeginPlay
  (Networking|SwitchHasAuthority
    (:Authority
      (Utilities|FlowControl|Sequence
        (:then_0
          (Variables|Default|SetUntaggedConsoleSymbols (Variables|SymbolConsole|GetConsoleSymbols))
          (for _array_element (Variables|SymbolConsole|GetConsoleSymbols)
            (EventDispatchers|AssignOnInteractBegin _array_element (delegate Custom|OnInteractBegin_Event))))
        (:then_1
          (EventDispatchers|AssignOnColumnComplete (Variables|SymbolConsole|GetSymbolControlColumn) (delegate Custom|OnColumnComplete_Event)))
        (:then_2
          (Class|Activatable|AddActivator (Variables|SymbolConsole|GetSymbolDisplayColumn) self))))))

(event EventTick
  (params (DeltaSeconds :type Float%20%28single-precision%29))
  (bind _output_get (Variables|Default|SettimerAlpha (- (Variables|Default|GettimerAlpha) (/ DeltaSeconds 2.5))))
  (Rendering|Material|SetScalarParameterValueonMaterials (Variables|Default|GetTimerDisplay) "Fill" _output_get))

(event EventActivate
  (Variables|Default|Setactive true)
  (if (not (Variables|Default|Getlocked))
    (CallFunction|SetSymbolStates "NewEnumerator2" true)))

(event EventDeactivate
  (Variables|Default|Setactive false)
  (if (not (Variables|Default|Getlocked))
    (CallFunction|SetSymbolStates "NewEnumerator1" true)))

(fn ConstructionScript)

(fn SetConsoleLocked
  (params (Locked :type Boolean))
  (bind _output_get (Variables|Default|Setlocked Locked))
  (if _output_get
    _
    (elif (Variables|Default|Getactive)
      (CallFunction|SetSymbolStates "NewEnumerator2" true)
      (else
        (CallFunction|SetSymbolStates "NewEnumerator1" true))))
  (return))

(fn IsSelectedSymbolCorrect
  (return (Utilities|Enum|Equal(Enum) (Default|GetRequiredGlyph (Variables|SymbolConsole|GetSymbolControlColumn)) (Variables|/Game/Blueprints/Actors/BP_Symbol.BP_Symbol_C|GetGlyph (Variables|Default|GetselectedSymbol)))))