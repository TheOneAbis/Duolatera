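; BP_SymbolColumn is an Act 3 puzzle column of four BP_Symbol child actors with randomized, non-repeating glyphs.
; Authority-bound symbol state changes drive activators on linked objects, straighten fixed parts, and activate final objects once every symbol is fixed.
; Separate progress events light symbols in order and report completion or reset.
; Destabilizing multicasts a timeline spin, then Tick swings unfixed parts erratically as entropy grows, optionally clearing fixed progress.
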(event Custom|Set%20Completed%20Symbol%20States
  (params (New%20State :type SymbolState%20Enum :default "NewEnumerator0"))
  (bind _unactivatedsymbols (Variables|Default|GetunactivatedSymbols))
  (bind _activationprogress (Variables|Default|GetActivationProgress))
  ;[0.5389 0.3235 0.7396] Sets the states of all revealed symbols
  (if (>= _activationprogress (- (Utilities|Array|Length _unactivatedsymbols) 1))
    (for _array_element _unactivatedsymbols
      (Default|SetSymbolState _array_element New%20State))
    (else
      (for _index (range 0 (- _activationprogress 1))
        (Default|SetSymbolState (Utilities|Array|Get(acopy) _unactivatedsymbols _index) New%20State)))))

(event Custom|Set%20Top%20Symbol%20Visible
  (params (visible :type Boolean))
  (bind _symbols (Variables|Default|Getsymbols))
  (bind _activationprogress (Variables|Default|GetActivationProgress))
  ;[1 0.4683 0.7751] Displays/Hides the column's topmost symbol (the one after its most recently activated one)
  (bind _output_get (Variables|Default|SetisTopmostLit visible))
  (if (< _activationprogress (Utilities|Array|Length _symbols))
    (Default|SetSymbolState (Utilities|Array|Get(acopy) _symbols _activationprogress) (select _output_get "NewEnumerator1" "NewEnumerator0"))))

(event Custom|StateChanged
  (params (Old%20State :type SymbolState%20Enum :default "NewEnumerator0") (New%20State :type SymbolState%20Enum :default "NewEnumerator0") (ChangedSymbol :type BP%20Symbol%20Object%20Reference))
  (bind _symbols (Variables|Default|Getsymbols))
  (bind _objects_to_activate (Variables|SymbolColumn|GetObjects%20to%20Activate))
  (bind _unactivatedsymbols (Variables|Default|GetunactivatedSymbols))
  (bind _rootcomponent (Variables|/Script/Engine.Actor|GetRootComponent ChangedSymbol))
  (bind _returnvalue (Utilities|Array|FindItem _symbols ChangedSymbol))
  (bind _returnvalue_2 (Transformation|GetAttachParent _rootcomponent))
  (bind _returnvalue_3 (Transformation|GetAttachParent _returnvalue_2))
  (if (and (> New%20State 2) (<= Old%20State 2))
    (for _array_element _objects_to_activate
      (Class|Activatable|AddActivator _array_element ChangedSymbol))
    (Default|CallOnColumnSymbolTagged ChangedSymbol _returnvalue)
    (else
      (for _array_element_2 _objects_to_activate
        (Class|Activatable|RemoveActivator _array_element_2 ChangedSymbol))
      (if (and (> Old%20State 2) (<= New%20State 2))
        (Default|CallOnColumnSymbolUntagged ChangedSymbol _returnvalue)
        (elif (== New%20State 4)
          (Transformation|SetRelativeRotation (Variables|/Script/Engine.Actor|GetRootComponent ChangedSymbol) (Math|Rotator|MakeRotator 0.0 0.0 0.0) false false)
          (bind _returnvalue_4 (Utilities|Array|RemoveItem _unactivatedsymbols ChangedSymbol))
          (Utilities|FlowControl|Sequence
            (:then_0
              (bind _output_get (Variables|Default|SetsymbolInitRot (.yaw (Variables|/Script/Engine.SceneComponent|GetRelativeRotation _returnvalue_3))))
              (bind _alpha (Timeline|FixColumnPartTimeline PlayFromStart)
                (:Update
                  (Transformation|SetRelativeRotation _returnvalue_3 (Math|Rotator|MakeRotator 0.0 0.0 (Math|Float|Lerp _output_get 0.0 _alpha)) false false))))
            (:then_1
              (if (and _returnvalue_4 (Utilities|Array|IsEmpty _unactivatedsymbols))
                (for _array_element_3 (Variables|SymbolColumn|GetFinal%20Objects%20to%20Activate)
                  (Class|Activatable|AddActivator _array_element_3 self))
                (Default|CallOnColumnActivated)))))))))

(event Custom|Reset
  (params (RandomizeOnReset :type Boolean))
  ;[1 0.3199 0.28] Resets the column's activation state back to 0. Optionally randomizes its symbol glyphs when reset occurs.
  (CallFunction|SetTopSymbolVisible false)
  (CallFunction|SetCompletedSymbolStates "NewEnumerator0")
  (Variables|Default|SetActivationProgress 0)
  (Utilities|FlowControl|Delay 0.5)
  (if RandomizeOnReset
    (CallFunction|RandomizeSymbolGlyphs))
  (Default|CallOnColumnReset))

(event Custom|Advance%20Progress
  (bind _activationprogress (Variables|Default|GetActivationProgress))
  ;[0.6146 0.4311 0.2853] Advances the column's activation progress. Column is fully activated when all 4 of its symbols are lit.
  (if (< _activationprogress (Utilities|Array|Length (Variables|Default|Getsymbols)))
    (bind _result (Math|Integer|IncrementInt _activationprogress)
      (:%20%20
        (CallFunction|SetCompletedSymbolStates "NewEnumerator1")
        (CallFunction|SetTopSymbolVisible (Variables|Default|GetisTopmostLit))
        (Default|CallOnProgressAdvanced _result)
        (if (== (Variables|Default|GetActivationProgress) (Utilities|Array|Length (Variables|Default|Getsymbols)))
          (Default|CallOnColumnComplete))))))

(event Custom|Destabilize
  (params (ResetProgress :type Boolean) (EntropyScale :type Float%20%28double-precision%29))
  (bind _final_objects_to_activate (Variables|SymbolColumn|GetFinal%20Objects%20to%20Activate))
  ;[1 0.6542 0.2113] Destabilize the column, reshuffling the glyphs and optionally resetting their states
  (if ResetProgress
    (Variables|Default|SetunactivatedSymbols (Variables|Default|Getsymbols))
    (if (not (Utilities|Array|IsEmpty _final_objects_to_activate))
      (if (Class|Activatable|IsActivator (Utilities|Array|Get(acopy) _final_objects_to_activate) self)
        (for _array_element _final_objects_to_activate
          (Class|Activatable|RemoveActivator _array_element self))
        (Default|CallOnColumnDeactivated))))
  (CallFunction|DestabilizeSpecificSymbols(Multi) (Variables|Default|GetunactivatedSymbols) EntropyScale))

(event Custom|Destabilize%20Specific%20Symbols%20%28Multi%29
  (params (symbols :type Array%20of%20BP%20Symbol%20Object%20References) (entropyScale :type Float%20%28double-precision%29))
  (Variables|Default|SetentropyScale entropyScale)
  (Variables|Default|Setentropy 0.0)
  (for _index (range 0 3)
    (Utilities|Array|SetArrayElem (Variables|Default|GettargetAngles) _index (* (Math|Float|SelectFloat 1.0 -1.0 (Math|Random|RandomBool)) (Math|Random|RandomFloatinRange 0.5 1.0)))
    (Utilities|Array|SetArrayElem (Variables|Default|GetcolumnSpeeds) _index (Math|Random|RandomFloatinRange 14.0 23.0)))
  (Actor|Tick|SetActorTickEnabled false)
  (Variables|Default|SetflipRotation (not (Variables|Default|GetflipRotation)))
  (bind _radians (Timeline|RotationTimeline PlayFromStart)
    (:Update
      (for (_array_element _array_index) symbols
        (Transformation|SetRelativeRotation (Transformation|GetAttachParent (Transformation|GetAttachParent (Variables|/Script/Engine.Actor|GetRootComponent _array_element))) (Math|Rotator|MakeRotator 0.0 0.0 (* (Math|Float|SelectFloat 1.0 -1.0 (Math|Conversions|ToBoolean(Integer) (Math|Integer|%(Integer) (+ _array_index (Variables|Default|GetflipRotation)) 2))) _radians)) false false)))
    (:Finished
      (Actor|Tick|SetActorTickEnabled true))))

(event EventBeginPlay
  (Variables|Default|SetunactivatedSymbols (Variables|Default|Getsymbols))
  (Networking|SwitchHasAuthority
    (:Authority
      (Variables|Default|SetcolumnParts (Utilities|Array|MakeArray (Variables|Default|GetColumn0) (Variables|Default|GetColumn1) (Variables|Default|GetColumn2) (Variables|Default|GetColumn3)))
      (CallFunction|RandomizeSymbolGlyphs)
      (for _array_element (Variables|Default|Getsymbols)
        (EventDispatchers|BindEventtoOnSymbolStateChanged _array_element (delegate Custom|StateChanged))))))

(event EventActivate
  ;[1 0.4683 0.7751] Displays/Hides the column's topmost symbol (the one after its most recently activated one)
  (CallFunction|SetTopSymbolVisible true))

(event EventDeactivate
  ;[1 0.4683 0.7751] Displays/Hides the column's topmost symbol (the one after its most recently activated one)
  (CallFunction|SetTopSymbolVisible false))

(event EventTick
  (params (DeltaSeconds :type Float%20%28single-precision%29))
  (bind _targetangles (Variables|Default|GettargetAngles))
  ;[1 0.09687 0.2066] Animate the column parts moving erratically
  (Variables|Default|Setentropy (+ (* DeltaSeconds (Variables|Default|GetentropyScale)) (Variables|Default|Getentropy)))
  (for (_array_element _array_index) (Variables|Default|GetunactivatedSymbols)
    (Utilities|Array|SetArrayElem _targetangles _array_index (* (Math|Float|SelectFloat -1.0 1.0 (>= (.yaw (Variables|/Script/Engine.SceneComponent|GetRelativeRotation (Transformation|GetAttachParent (Transformation|GetAttachParent (Variables|/Script/Engine.Actor|GetRootComponent _array_element))))) (Utilities|Array|Get(acopy) _targetangles _array_index))) (+ (* DeltaSeconds (Math|Float|Power (+ (Variables|Default|Getentropy) 0.2) 8.0) 1.0) (Math|Float|Absolute(Float) (Utilities|Array|Get(acopy) _targetangles _array_index)))))
    (Transformation|SetRelativeRotation (Transformation|GetAttachParent (Transformation|GetAttachParent (Variables|/Script/Engine.Actor|GetRootComponent _array_element))) (Math|Rotator|MakeRotator 0.0 0.0 (+ (.yaw (Variables|/Script/Engine.SceneComponent|GetRelativeRotation (Transformation|GetAttachParent (Transformation|GetAttachParent (Variables|/Script/Engine.Actor|GetRootComponent _array_element))))) (* DeltaSeconds (Utilities|Array|Get(acopy) _targetangles _array_index) (Utilities|Array|Get(acopy) (Variables|Default|GetcolumnSpeeds) _array_index)))) false false)))

(fn ConstructionScript
  (for _array_element (Utilities|Array|MakeArray (Variables|Default|GetSymbol0) (Variables|Default|GetSymbol1) (Variables|Default|GetSymbol2) (Variables|Default|GetSymbol3))
    (bind _asbp_symbol (Utilities|Casting|CastToBP_Symbol (Variables|/Script/Engine.ChildActorComponent|GetChildActor _array_element)))
    (Variables|/Game/Blueprints/Actors/BP_Symbol.BP_Symbol_C|SetSymbol%20Type _asbp_symbol (Variables|SymbolColumn|GetColumn%20Symbol%20Type))
    (Utilities|Array|Add (Variables|Default|Getsymbols) _asbp_symbol)))

(fn RandomizeSymbolGlyphs
  (bind _glyphstochoose (LocalVariables|GetglyphsToChoose))
  (for _array_element (Variables|Default|Getsymbols)
    (bind _output_get (LocalVariables|SetchosenIndex (Math|Random|RandomInteger (Utilities|Array|Length _glyphstochoose))))
    (Variables|/Game/Blueprints/Actors/BP_Symbol.BP_Symbol_C|SetGlyph _array_element (Utilities|Array|Get(acopy) _glyphstochoose _output_get))
    (Utilities|Array|RemoveIndex _glyphstochoose _output_get))
  (return))

(fn GetRequiredGlyph
  (bind _symbols (Variables|Default|Getsymbols))
  (return (Variables|/Game/Blueprints/Actors/BP_Symbol.BP_Symbol_C|GetGlyph (Utilities|Array|Get(acopy) _symbols (Math|Integer|Min(Integer) (- (Utilities|Array|Length _symbols) 1) (Variables|Default|GetActivationProgress))))))

(fn GetColumnGlyphs
  (bind _glyphs (LocalVariables|Getglyphs))
  (for _array_element (Variables|Default|Getsymbols)
    (Utilities|Array|Add _glyphs (Variables|/Game/Blueprints/Actors/BP_Symbol.BP_Symbol_C|GetGlyph _array_element)))
  (return _glyphs))