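; Multi-phase VR symbol puzzle for Act 3, linking Overworld and Underworld glyph columns.
; Two inserted grabbable symbols enable a server-driven, shuffled left/right memory sequence, shown through symbol highlights and multicast Niagara shapes.
; Completing it starts phase 3, where tagging the one matching glyph pair across worlds stabilizes it.
; Mismatched simultaneous tags reset progress, while a Tick timer periodically reshuffles glyphs, shortening as pairs stabilize until all eight keep the power lines lit.
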(event OnComponentBeginOverlap(RightSlot)
  (params (OverlappedComponent :type Primitive%20Component%20Object%20Reference) (OtherActor :type Actor%20Object%20Reference) (OtherComp :type Primitive%20Component%20Object%20Reference) (OtherBodyIndex :type Integer) (bFromSweep :type Boolean) (SweepResult :type Hit%20Result%20Structure%20%28by%20ref%29))
  ;[0.4323 0.3634 0.2364] Handles insertion of symbols into their slots to begin the phase 2 memory sequence
  (Networking|SwitchHasAuthority
    (:Authority
      (bind _asbp_grabbable_symbol (Utilities|Casting|CastToBP_GrabbableSymbol OtherActor))
      (CallFunction|InsertSymbol _asbp_grabbable_symbol false OverlappedComponent))))

(event OnComponentBeginOverlap(LeftSlot)
  (params (OverlappedComponent :type Primitive%20Component%20Object%20Reference) (OtherActor :type Actor%20Object%20Reference) (OtherComp :type Primitive%20Component%20Object%20Reference) (OtherBodyIndex :type Integer) (bFromSweep :type Boolean) (SweepResult :type Hit%20Result%20Structure%20%28by%20ref%29))
  ;[0.4323 0.3634 0.2364] Handles insertion of symbols into their slots to begin the phase 2 memory sequence
  (Networking|SwitchHasAuthority
    (:Authority
      (bind _asbp_grabbable_symbol (Utilities|Casting|CastToBP_GrabbableSymbol OtherActor))
      (CallFunction|InsertSymbol _asbp_grabbable_symbol true OverlappedComponent))))

(event Custom|InteractRight_Event
  (params (interactedActor :type Interactable%20Object%20Reference))
  (bind _overworldcolumns (Variables|Phase3|GetoverworldColumns))
  (bind _underworldcolumns (Variables|Phase3|GetunderworldColumns))
  (bind _output (Utilities|Array|Get(acopy) _underworldcolumns 1))
  (bind _output_2 (Utilities|Array|Get(acopy) _overworldcolumns 1))
  (bind _output_3 (Utilities|Array|Get(acopy) _overworldcolumns))
  (bind _output_4 (Utilities|Array|Get(acopy) _underworldcolumns))
  ;[0.3523 0.3895 0.5156] Phase 2 Memory sequence; Interacting with the correct symbol advances the sequence, interacting with the wrong one fails it
  (bind _asbp_symbol (Utilities|Casting|CastToBP_Symbol interactedActor))
  (if (and (not (Utilities|Array|Get(acopy) (Variables|Phase2|GetcolumnSequence) (Variables|Phase2|GetsequenceProgress))) (Utilities|Enum|Equal(Enum) (Variables|/Game/Blueprints/Actors/BP_Symbol.BP_Symbol_C|GetGlyph _asbp_symbol) (Default|GetRequiredGlyph (Variables|SequenceSystem|GetunderworldRightColumn))))
    (Default|AdvanceProgress (Variables|SequenceSystem|GetunderworldRightColumn))
    (bind _result (Math|Integer|IncrementInt (Variables|Phase2|GetsequenceProgress))
      (:%20%20
        (if (== _result 4)
          (for _array_element (Variables|Phase2|GetinsertedSymbols)
            (Default|SetSymbolState _array_element "NewEnumerator2"))
          (elif (== _result 8)
            ;[1 0 0.04671] Begin Phase 3
            (Utilities|FlowControl|DoOnce false
              (:Completed
                (for _array_element_2 (Variables|Phase3|GetunderworldColumns)
                  (EventDispatchers|UnbindallEventsfromOnColumnComplete _array_element_2))
                (Utilities|FlowControl|Sequence
                  (:then_0
                    (EventDispatchers|AssignOnColumnSymbolTagged _output_4 (delegate Custom|OnColumnSymbolTagged_UnderLeft))
                    (EventDispatchers|AssignOnColumnSymbolUntagged _output_4 (delegate Custom|OnColumnSymbolUntagged_UnderLeft)))
                  (:then_1
                    (EventDispatchers|AssignOnColumnSymbolTagged _output (delegate Custom|OnColumnSymbolTagged_UnderRight))
                    (EventDispatchers|AssignOnColumnSymbolUntagged _output (delegate Custom|OnColumnSymbolUntagged_UnderRight)))
                  (:then_2
                    (EventDispatchers|AssignOnColumnSymbolTagged _output_3 (delegate Custom|OnColumnSymbolTagged_OverLeft))
                    (EventDispatchers|AssignOnColumnSymbolUntagged _output_3 (delegate Custom|OnColumnSymbolUntagged_OverLeft)))
                  (:then_3
                    (EventDispatchers|AssignOnColumnSymbolTagged _output_2 (delegate Custom|OnColumnSymbolTagged_OverRight))
                    (EventDispatchers|AssignOnColumnSymbolUntagged _output_2 (delegate Custom|OnColumnSymbolUntagged_OverRight)))
                  (:then_4
                    (CallFunction|CorruptColumns true)
                    (for _array_element_3 (Variables|Phase3|GetPowerLines)
                      (Variables|/Game/Blueprints/Actors/Act3/BP_PowerLine.BP_PowerLine_C|Setglow _array_element_3 3e+01))))))))))
    (else
      (CallFunction|CancelSequence))))

(event Custom|InteractLeft_Event
  (params (interactedActor :type Interactable%20Object%20Reference))
  (bind _overworldcolumns (Variables|Phase3|GetoverworldColumns))
  (bind _underworldcolumns (Variables|Phase3|GetunderworldColumns))
  (bind _output (Utilities|Array|Get(acopy) _underworldcolumns 1))
  (bind _output_2 (Utilities|Array|Get(acopy) _overworldcolumns 1))
  (bind _output_3 (Utilities|Array|Get(acopy) _overworldcolumns))
  (bind _output_4 (Utilities|Array|Get(acopy) _underworldcolumns))
  ;[0.3523 0.3895 0.5156] Phase 2 Memory sequence; Interacting with the correct symbol advances the sequence, interacting with the wrong one fails it
  (bind _asbp_symbol (Utilities|Casting|CastToBP_Symbol interactedActor))
  (if (and (Utilities|Array|Get(acopy) (Variables|Phase2|GetcolumnSequence) (Variables|Phase2|GetsequenceProgress)) (Utilities|Enum|Equal(Enum) (Default|GetRequiredGlyph (Variables|SequenceSystem|GetunderworldLeftColumn)) (Variables|/Game/Blueprints/Actors/BP_Symbol.BP_Symbol_C|GetGlyph _asbp_symbol)))
    (Default|AdvanceProgress (Variables|SequenceSystem|GetunderworldLeftColumn))
    (bind _result (Math|Integer|IncrementInt (Variables|Phase2|GetsequenceProgress))
      (:%20%20
        (if (== _result 4)
          (for _array_element (Variables|Phase2|GetinsertedSymbols)
            (Default|SetSymbolState _array_element "NewEnumerator2"))
          (elif (== _result 8)
            ;[1 0 0.04671] Begin Phase 3
            (Utilities|FlowControl|DoOnce false
              (:Completed
                (for _array_element_2 (Variables|Phase3|GetunderworldColumns)
                  (EventDispatchers|UnbindallEventsfromOnColumnComplete _array_element_2))
                (Utilities|FlowControl|Sequence
                  (:then_0
                    (EventDispatchers|AssignOnColumnSymbolTagged _output_4 (delegate Custom|OnColumnSymbolTagged_UnderLeft))
                    (EventDispatchers|AssignOnColumnSymbolUntagged _output_4 (delegate Custom|OnColumnSymbolUntagged_UnderLeft)))
                  (:then_1
                    (EventDispatchers|AssignOnColumnSymbolTagged _output (delegate Custom|OnColumnSymbolTagged_UnderRight))
                    (EventDispatchers|AssignOnColumnSymbolUntagged _output (delegate Custom|OnColumnSymbolUntagged_UnderRight)))
                  (:then_2
                    (EventDispatchers|AssignOnColumnSymbolTagged _output_3 (delegate Custom|OnColumnSymbolTagged_OverLeft))
                    (EventDispatchers|AssignOnColumnSymbolUntagged _output_3 (delegate Custom|OnColumnSymbolUntagged_OverLeft)))
                  (:then_3
                    (EventDispatchers|AssignOnColumnSymbolTagged _output_2 (delegate Custom|OnColumnSymbolTagged_OverRight))
                    (EventDispatchers|AssignOnColumnSymbolUntagged _output_2 (delegate Custom|OnColumnSymbolUntagged_OverRight)))
                  (:then_4
                    (CallFunction|CorruptColumns true)
                    (for _array_element_3 (Variables|Phase3|GetPowerLines)
                      (Variables|/Game/Blueprints/Actors/Act3/BP_PowerLine.BP_PowerLine_C|Setglow _array_element_3 3e+01))))))))))
    (else
      (CallFunction|CancelSequence))))

(event Custom|Deactivate%20Particles%20%28Multi%29
  ;[0.5781 0.5781 0.5781] Deactivate or Activate particle emitters on server and client
  (Components|Activation|Deactivate (Variables|Default|GetLeftShapeEmitter))
  (Components|Activation|Deactivate (Variables|Default|GetRightShapeEmitter)))

(event Custom|debug
  (bind _overworldcolumns (Variables|Phase3|GetoverworldColumns))
  (bind _underworldcolumns (Variables|Phase3|GetunderworldColumns))
  (bind _output (Utilities|Array|Get(acopy) _underworldcolumns 1))
  (bind _output_2 (Utilities|Array|Get(acopy) _overworldcolumns 1))
  (bind _output_3 (Utilities|Array|Get(acopy) _overworldcolumns))
  (bind _output_4 (Utilities|Array|Get(acopy) _underworldcolumns))
  (Utilities|FlowControl|DelayUntilNextTick)
  (for _index (range 0 4)
    (for _array_element (Variables|Phase3|GetunderworldColumns)
      (Default|AdvanceProgress _array_element))
    (for _array_element_2 (Variables|Phase3|GetoverworldColumns)
      (Default|AdvanceProgress _array_element_2)))
  ;[1 0 0.04671] Begin Phase 3
  (Utilities|FlowControl|DoOnce false
    (:Completed
      (for _array_element_3 (Variables|Phase3|GetunderworldColumns)
        (EventDispatchers|UnbindallEventsfromOnColumnComplete _array_element_3))
      (Utilities|FlowControl|Sequence
        (:then_0
          (EventDispatchers|AssignOnColumnSymbolTagged _output_4 (delegate Custom|OnColumnSymbolTagged_UnderLeft))
          (EventDispatchers|AssignOnColumnSymbolUntagged _output_4 (delegate Custom|OnColumnSymbolUntagged_UnderLeft)))
        (:then_1
          (EventDispatchers|AssignOnColumnSymbolTagged _output (delegate Custom|OnColumnSymbolTagged_UnderRight))
          (EventDispatchers|AssignOnColumnSymbolUntagged _output (delegate Custom|OnColumnSymbolUntagged_UnderRight)))
        (:then_2
          (EventDispatchers|AssignOnColumnSymbolTagged _output_3 (delegate Custom|OnColumnSymbolTagged_OverLeft))
          (EventDispatchers|AssignOnColumnSymbolUntagged _output_3 (delegate Custom|OnColumnSymbolUntagged_OverLeft)))
        (:then_3
          (EventDispatchers|AssignOnColumnSymbolTagged _output_2 (delegate Custom|OnColumnSymbolTagged_OverRight))
          (EventDispatchers|AssignOnColumnSymbolUntagged _output_2 (delegate Custom|OnColumnSymbolUntagged_OverRight)))
        (:then_4
          (CallFunction|CorruptColumns true)
          (for _array_element_4 (Variables|Phase3|GetPowerLines)
            (Variables|/Game/Blueprints/Actors/Act3/BP_PowerLine.BP_PowerLine_C|Setglow _array_element_4 3e+01)))))))

(event Custom|Activate%20Particles%20%28Multi%29
  (bind _array (Utilities|Array|MakeArray false false false false false false false false))
  (bind _leftshapeemitter (Variables|Default|GetLeftShapeEmitter))
  (bind _rightshapeemitter (Variables|Default|GetRightShapeEmitter))
  ;[0.5781 0.5781 0.5781] Deactivate or Activate particle emitters on server and client
  (Class|NiagaraDataInterfaceArrayFunctionLibrary|SetNiagaraArrayBool _leftshapeemitter "IsShapedArray" _array)
  (Components|Activation|Activate _leftshapeemitter true)
  (Class|NiagaraDataInterfaceArrayFunctionLibrary|SetNiagaraArrayBool _rightshapeemitter "IsShapedArray" _array)
  (Components|Activation|Activate _rightshapeemitter true))

(event Custom|OnColumnSymbolUntagged_UnderRight
  (params (Untagged%20Symbol :type BP%20Symbol%20Object%20Reference) (Untagged%20Symbol%20Index :type Integer))
  ;[0.3836 0.474 0.1602] Phase 3 symbol activation logic
  (if (not (== (Variables|/Game/Blueprints/Actors/BP_Symbol.BP_Symbol_C|GetState Untagged%20Symbol) 0))
    (Default|SetSymbolState (Utilities|Array|Get(acopy) (Variables|/Game/Blueprints/Actors/Act3/BP_SymbolColumn.BP_SymbolColumn_C|Getsymbols (Utilities|Array|Get(acopy) (Variables|Phase3|GetoverworldColumns))) Untagged%20Symbol%20Index) "NewEnumerator1")))

(event Custom|OnColumnSymbolUntagged_OverRight
  (params (Untagged%20Symbol :type BP%20Symbol%20Object%20Reference) (Untagged%20Symbol%20Index :type Integer))
  ;[0.3836 0.474 0.1602] Phase 3 symbol activation logic
  (if (not (== (Variables|/Game/Blueprints/Actors/BP_Symbol.BP_Symbol_C|GetState Untagged%20Symbol) 0))
    (Default|SetSymbolState (Utilities|Array|Get(acopy) (Variables|/Game/Blueprints/Actors/Act3/BP_SymbolColumn.BP_SymbolColumn_C|Getsymbols (Utilities|Array|Get(acopy) (Variables|Phase3|GetunderworldColumns))) Untagged%20Symbol%20Index) "NewEnumerator1")))

(event Custom|OnColumnSymbolUntagged_OverLeft
  (params (Untagged%20Symbol :type BP%20Symbol%20Object%20Reference) (Untagged%20Symbol%20Index :type Integer))
  ;[0.3836 0.474 0.1602] Phase 3 symbol activation logic
  (if (not (== (Variables|/Game/Blueprints/Actors/BP_Symbol.BP_Symbol_C|GetState Untagged%20Symbol) 0))
    (Default|SetSymbolState (Utilities|Array|Get(acopy) (Variables|/Game/Blueprints/Actors/Act3/BP_SymbolColumn.BP_SymbolColumn_C|Getsymbols (Utilities|Array|Get(acopy) (Variables|Phase3|GetunderworldColumns) 1)) Untagged%20Symbol%20Index) "NewEnumerator1")))

(event Custom|CancelSequence
  ;[0.151 0.151 0.151] Set states of symbols from phase 1 to inactive, deactivating this actor and failing the sequence. Then set them to activatable to allow another attempt.
  (for _array_element (Variables|Phase2|GetinsertedSymbols)
    (Default|SetSymbolState _array_element "NewEnumerator0") ; Setting the inserted symbols' states to inactive ends up calling this actor's Deactivate event
  )
  (Utilities|FlowControl|Delay 2.0)
  (for _array_element_2 (Variables|Phase2|GetinsertedSymbols)
    (Default|SetSymbolState _array_element_2 "NewEnumerator2")))

(event Custom|OnColumnSymbolUntagged_UnderLeft
  (params (Untagged%20Symbol :type BP%20Symbol%20Object%20Reference) (Untagged%20Symbol%20Index :type Integer))
  ;[0.3836 0.474 0.1602] Phase 3 symbol activation logic
  (if (not (== (Variables|/Game/Blueprints/Actors/BP_Symbol.BP_Symbol_C|GetState Untagged%20Symbol) 0))
    (Default|SetSymbolState (Utilities|Array|Get(acopy) (Variables|/Game/Blueprints/Actors/Act3/BP_SymbolColumn.BP_SymbolColumn_C|Getsymbols (Utilities|Array|Get(acopy) (Variables|Phase3|GetoverworldColumns) 1)) Untagged%20Symbol%20Index) "NewEnumerator1")))

(event Custom|OnColumnSymbolTagged_UnderLeft
  (params (Tagged%20Symbol :type BP%20Symbol%20Object%20Reference) (Tagged%20Symbol%20Index :type Integer))
  (bind _overworldcolumns (Variables|Phase3|GetoverworldColumns))
  (bind _output (Utilities|Array|Get(acopy) _overworldcolumns 1))
  (bind _symbols (Variables|/Game/Blueprints/Actors/Act3/BP_SymbolColumn.BP_SymbolColumn_C|Getsymbols _output))
  (bind _output_2 (Utilities|Array|Get(acopy) _symbols Tagged%20Symbol%20Index))
  ;[0.3836 0.474 0.1602] Phase 3 symbol activation logic
  (if (Utilities|Enum|Equal(Enum) (Variables|/Game/Blueprints/Actors/BP_Symbol.BP_Symbol_C|GetState _output_2) "NewEnumerator1")
    (Default|SetSymbolState _output_2 "NewEnumerator2")
    (elif (Utilities|Enum|Equal(Enum) (Variables|/Game/Blueprints/Actors/BP_Symbol.BP_Symbol_C|GetGlyph Tagged%20Symbol) (Variables|/Game/Blueprints/Actors/BP_Symbol.BP_Symbol_C|GetGlyph _output_2))
      (CallFunction|StabilizeSymbols _output_2 Tagged%20Symbol)
      (else
        (CallFunction|CorruptColumns true)))))

(event Custom|OnColumnSymbolTagged_OverLeft
  (params (Tagged%20Symbol :type BP%20Symbol%20Object%20Reference) (Tagged%20Symbol%20Index :type Integer))
  (bind _underworldcolumns (Variables|Phase3|GetunderworldColumns))
  (bind _output (Utilities|Array|Get(acopy) _underworldcolumns 1))
  (bind _symbols (Variables|/Game/Blueprints/Actors/Act3/BP_SymbolColumn.BP_SymbolColumn_C|Getsymbols _output))
  (bind _output_2 (Utilities|Array|Get(acopy) _symbols Tagged%20Symbol%20Index))
  ;[0.3836 0.474 0.1602] Phase 3 symbol activation logic
  (if (Utilities|Enum|Equal(Enum) (Variables|/Game/Blueprints/Actors/BP_Symbol.BP_Symbol_C|GetState _output_2) "NewEnumerator1")
    (Default|SetSymbolState _output_2 "NewEnumerator2")
    (elif (Utilities|Enum|Equal(Enum) (Variables|/Game/Blueprints/Actors/BP_Symbol.BP_Symbol_C|GetGlyph _output_2) (Variables|/Game/Blueprints/Actors/BP_Symbol.BP_Symbol_C|GetGlyph Tagged%20Symbol))
      (CallFunction|StabilizeSymbols Tagged%20Symbol _output_2)
      (else
        (CallFunction|CorruptColumns true)))))

(event Custom|StabilizeSymbols
  (params (OverSymbol :type BP%20Symbol%20Object%20Reference) (UnderSymbol :type BP%20Symbol%20Object%20Reference))
  ;[0.3836 0.474 0.1602] Phase 3 symbol activation logic
  (Default|SetSymbolState OverSymbol "NewEnumerator4")
  (bind _result (Math|Integer|IncrementInt (Variables|Phase3|GetactivatedSymbols))
    (:%20%20
      (Actor|Tick|SetActorTickEnabled (not (== _result 8)))
      (if (== _result 8)
        ;;[0.6354 0.4023 0.2449] Keep power lines lit if this is the last set of symbols being stabilized
        (for _array_element (Variables|Phase3|GetPowerLines)
          (Class|Activatable|AddActivator _array_element self))
        (else
          (CallFunction|CorruptColumns false))))))

(event Custom|OnColumnSymbolTagged_UnderRight
  (params (Tagged%20Symbol :type BP%20Symbol%20Object%20Reference) (Tagged%20Symbol%20Index :type Integer))
  (bind _overworldcolumns (Variables|Phase3|GetoverworldColumns))
  (bind _output (Utilities|Array|Get(acopy) _overworldcolumns))
  (bind _symbols (Variables|/Game/Blueprints/Actors/Act3/BP_SymbolColumn.BP_SymbolColumn_C|Getsymbols _output))
  (bind _output_2 (Utilities|Array|Get(acopy) _symbols Tagged%20Symbol%20Index))
  ;[0.3836 0.474 0.1602] Phase 3 symbol activation logic
  (if (Utilities|Enum|Equal(Enum) (Variables|/Game/Blueprints/Actors/BP_Symbol.BP_Symbol_C|GetState _output_2) "NewEnumerator1")
    (Default|SetSymbolState _output_2 "NewEnumerator2")
    (elif (Utilities|Enum|Equal(Enum) (Variables|/Game/Blueprints/Actors/BP_Symbol.BP_Symbol_C|GetGlyph Tagged%20Symbol) (Variables|/Game/Blueprints/Actors/BP_Symbol.BP_Symbol_C|GetGlyph _output_2))
      (CallFunction|StabilizeSymbols _output_2 Tagged%20Symbol)
      (else
        (CallFunction|CorruptColumns true)))))

(event Custom|test
  (params (NewParam :type BP%20Grabbable%20Symbol%20Object%20Reference) (NewParam2 :type Vector) (NewParam3 :type Rotator))
  (Utilities|FlowControl|Delay 0.2)
  (Transformation|SetActorLocationAndRotation NewParam NewParam2 NewParam3))

(event Custom|Show%20Sequence%20Index%20%28Multi%29
  (params (Shape%20Element :type Integer) (Symbol%20to%20Highlight :type BP%20Symbol%20Object%20Reference))
  (bind _returnvalue (Class|KismetSystemLibrary|MakeLiteralBool true))
  ;[0.6094 0.6094 0.6094] Displays the particle emitter shape of the specified element on server and client
  (Utilities|FlowControl|Sequence
    (:then_0
      (Class|NiagaraDataInterfaceArrayFunctionLibrary|SetNiagaraArrayBoolValue (Variables|Default|GetLeftShapeEmitter) "IsShapedArray" Shape%20Element _returnvalue false)
      (Class|NiagaraDataInterfaceArrayFunctionLibrary|SetNiagaraArrayBoolValue (Variables|Default|GetRightShapeEmitter) "IsShapedArray" Shape%20Element _returnvalue false))
    (:then_1
      (Default|Highlight Symbol%20to%20Highlight))))

(event Custom|Corrupt%20Columns
  (params (Reset :type Boolean))
  ;[1 0.52 0.2025] Phase 3; Handles column reset event, which happens either periodically, or when 2 symbols in opposing worlds are shot simultaneously.
  (Variables|Phase3|Settimer (+ (* (Math|Float|Power (Math|Conversions|ToFloat(Integer) (Variables|Phase3|GetactivatedSymbols)) 1.8) -0.4) (Variables|Phase3|GetdestabilizeTime)))
  (Utilities|FlowControl|Sequence
    (:then_0
      (if Reset
        (Variables|Phase3|SetactivatedSymbols 0)
        (Actor|Tick|SetActorTickEnabled false)))
    (:then_1
      (for _array_element (Variables|Phase3|GetoverworldColumns)
        (Default|Destabilize _array_element Reset (Math|Float|SelectFloat 0.0 (/ 1.0 (- (Variables|Phase3|Gettimer) 1.5)) (== (Variables|Phase3|GetactivatedSymbols) 0)))
        (Default|SetCompletedSymbolStates _array_element "NewEnumerator0"))
      (for _array_element_2 (Variables|Phase3|GetunderworldColumns)
        (Default|Destabilize _array_element_2 Reset (Math|Float|SelectFloat 0.0 (/ 1.0 (- (Variables|Phase3|Gettimer) 1.5)) (== (Variables|Phase3|GetactivatedSymbols) 0)))
        (Default|SetCompletedSymbolStates _array_element_2 "NewEnumerator0"))
      (Utilities|FlowControl|Delay 1.5)
      (CallFunction|RandomizeTargetSymbols))))

(event Custom|OnColumnSymbolTagged_OverRight
  (params (Tagged%20Symbol :type BP%20Symbol%20Object%20Reference) (Tagged%20Symbol%20Index :type Integer))
  (bind _underworldcolumns (Variables|Phase3|GetunderworldColumns))
  (bind _output (Utilities|Array|Get(acopy) _underworldcolumns))
  (bind _symbols (Variables|/Game/Blueprints/Actors/Act3/BP_SymbolColumn.BP_SymbolColumn_C|Getsymbols _output))
  (bind _output_2 (Utilities|Array|Get(acopy) _symbols Tagged%20Symbol%20Index))
  ;[0.3836 0.474 0.1602] Phase 3 symbol activation logic
  (if (Utilities|Enum|Equal(Enum) (Variables|/Game/Blueprints/Actors/BP_Symbol.BP_Symbol_C|GetState _output_2) "NewEnumerator1")
    (Default|SetSymbolState _output_2 "NewEnumerator2")
    (elif (Utilities|Enum|Equal(Enum) (Variables|/Game/Blueprints/Actors/BP_Symbol.BP_Symbol_C|GetGlyph _output_2) (Variables|/Game/Blueprints/Actors/BP_Symbol.BP_Symbol_C|GetGlyph Tagged%20Symbol))
      (CallFunction|StabilizeSymbols Tagged%20Symbol _output_2)
      (else
        (CallFunction|CorruptColumns true)))))

(event EventBeginPlay
  (Variables|Phase3|SetunderworldColumns (Utilities|Array|MakeArray (Variables|SequenceSystem|GetunderworldLeftColumn) (Variables|SequenceSystem|GetunderworldRightColumn)))
  (Networking|SwitchHasAuthority
    (:Authority
      (bind _sequence (CallFunction|CreateShuffledSequence))
      (Variables|Phase2|SetcolumnSequence _sequence)
      ;[0.3523 0.3895 0.5156] Phase 2 Memory sequence; Interacting with the correct symbol advances the sequence, interacting with the wrong one fails it
      (Utilities|FlowControl|Sequence
        (:then_0
          (for _array_element (Variables|SequenceSystem|GetsequenceSymbolsLeft)
            (EventDispatchers|AssignOnInteractBegin _array_element (delegate Custom|InteractLeft_Event))))
        (:then_1
          (for _array_element_2 (Variables|SequenceSystem|GetsequenceSymbolsRight)
            (EventDispatchers|AssignOnInteractBegin _array_element_2 (delegate Custom|InteractRight_Event))))))))

(event EventActivate
  (if (== (Variables|Phase2|GetsequenceProgress) 0)
    (CallFunction|ActivateParticles(Multi)))
  (CallFunction|SetSymbolStates "NewEnumerator1" true)
  (for _array_element (Variables|Phase2|GetinsertedSymbols)
    (Default|SetSymbolState _array_element "NewEnumerator4"))
  (Utilities|FlowControl|Delay 2.0)
  ;[0.5156 0.4042 0.1279] Highlight the glyph sequence, one after the other
  (Variables|Phase2|SetanimationIndex 0)
  (if (== (Variables|Phase2|GetsequenceProgress) 0)
    (Variables|Phase2|SetsearchIndexLeft 0)
    (Variables|Phase2|SetsearchIndexRight 0)
    (Variables|Phase2|SetleftColGlyphs (Default|GetColumnGlyphs (Variables|SequenceSystem|GetunderworldLeftColumn)))
    (Variables|Phase2|SetrightColGlyphs (Default|GetColumnGlyphs (Variables|SequenceSystem|GetunderworldRightColumn))))
  (if (< (Variables|Phase2|GetanimationIndex) 4) :!label _label
    (if (Utilities|Array|Get(acopy) (Variables|Phase2|GetcolumnSequence) (+ (Variables|Phase2|GetanimationIndex) (Variables|Phase2|GetsequenceProgress)))
      (bind _array_element_2 (Utilities|Array|ForEachLoopwithBreak (Variables|SequenceSystem|GetsequenceSymbolsLeft) :!label _label_2)
        (:LoopBody
          (if (Utilities|Enum|Equal(Enum) (Utilities|Array|Get(acopy) (Variables|Phase2|GetleftColGlyphs) (Variables|Phase2|GetsearchIndexLeft)) (Variables|/Game/Blueprints/Actors/BP_Symbol.BP_Symbol_C|GetGlyph _array_element_2))
            (Utilities|FlowControl|Sequence
              (:then_0
                (goto _label_2 Break))
              (:then_1
                (Math|Integer|IncrementInt (Variables|Phase2|GetsearchIndexLeft)
                  (:%20%20
                    (CallFunction|ShowSequenceIndex(Multi) (+ (Variables|Phase2|GetanimationIndex) (Variables|Phase2|GetsequenceProgress)) _array_element_2)
                    (Math|Integer|IncrementInt (Variables|Phase2|GetanimationIndex) :!label _label_3
                      (:%20%20
                        (Utilities|FlowControl|Delay 1.7)
                        (goto _label))))))))))
      (else
        (bind _array_element_3 (Utilities|Array|ForEachLoopwithBreak (Variables|SequenceSystem|GetsequenceSymbolsRight) :!label _label_4)
          (:LoopBody
            (if (Utilities|Enum|Equal(Enum) (Utilities|Array|Get(acopy) (Variables|Phase2|GetrightColGlyphs) (Variables|Phase2|GetsearchIndexRight)) (Variables|/Game/Blueprints/Actors/BP_Symbol.BP_Symbol_C|GetGlyph _array_element_3))
              (Utilities|FlowControl|Sequence
                (:then_0
                  (goto _label_4 Break))
                (:then_1
                  (Math|Integer|IncrementInt (Variables|Phase2|GetsearchIndexRight)
                    (:%20%20
                      (CallFunction|ShowSequenceIndex(Multi) (+ (Variables|Phase2|GetanimationIndex) (Variables|Phase2|GetsequenceProgress)) _array_element_3)
                      (goto _label_3))))))))))
    (else
      (Utilities|FlowControl|Delay 2.0)
      ;[0.1969 0.3698 0.09029] Set symbol activatability
      (CallFunction|SetSymbolStates "NewEnumerator2" true))))

(event EventDeactivate
  ;[0.5729 0.1813 0.1069] Resets the Phase 2 sequence
  (if (Utilities|Enum|Equal(Enum) (Variables|/Game/Blueprints/Actors/BP_Symbol.BP_Symbol_C|GetState (Utilities|Array|Get(acopy) (Variables|Phase2|GetinsertedSymbols))) "NewEnumerator0")
    (CallFunction|SetSymbolStates "NewEnumerator0" false)
    (Default|Reset (Variables|SequenceSystem|GetunderworldLeftColumn) false)
    (Default|Reset (Variables|SequenceSystem|GetunderworldRightColumn) false)
    (Variables|Phase2|SetsequenceProgress 0)
    (CallFunction|DeactivateParticles(Multi))
    (else
      (CallFunction|SetSymbolStates "NewEnumerator1" true))))

(event EventTick
  (params (DeltaSeconds :type Float%20%28single-precision%29))
  ;[0.6406 0.3103 0.3103] Corrupt the Columns periodically.
  (bind _output_get (Variables|Phase3|Settimer (- (Variables|Phase3|Gettimer) DeltaSeconds)))
  (if (< _output_get 0.0)
    (CallFunction|CorruptColumns false)))

(fn ConstructionScript)

(fn InsertSymbol
  (params (Inserted%20Symbol :type BP%20Grabbable%20Symbol%20Object%20Reference) (Left :type Boolean) (Overlapped%20Slot :type Scene%20Component%20Object%20Reference))
  (bind _returnvalue (Transformation|GetWorldTransform Overlapped%20Slot))
  (bind _insertedsymbols (Variables|Phase2|GetinsertedSymbols))
  (bind _output_get (LocalVariables|Setsymbol Inserted%20Symbol))
  (if (Utilities|Enum|Equal(Enum) (Variables|/Game/Blueprints/Actors/BP_Symbol.BP_Symbol_C|GetSymbol%20Type _output_get) (select Left "NewEnumerator1" "NewEnumerator0"))
    (Components|Activation|Deactivate Overlapped%20Slot)
    (Variables|/Game/Blueprints/Components/GrabComponent.GrabComponent_C|SetbSimulateOnDrop (Variables|/Game/Blueprints/Actors/Act3/BP_GrabbableSymbol.BP_GrabbableSymbol_C|GetGrabComponent _output_get) false)
    (bind _asvrpawn (Utilities|Casting|CastToVRPawn (Game|Player|GetPlayerPawn 0)))
    (Default|RPCServerTryRelease _asvrpawn (Variables|/Game/Blueprints/Actors/Act3/BP_GrabbableSymbol.BP_GrabbableSymbol_C|GetGrabComponent _output_get) (Utilities|Enum|Equal(Enum) (Default|GetHeldbyHand (Variables|/Game/Blueprints/Actors/Act3/BP_GrabbableSymbol.BP_GrabbableSymbol_C|GetGrabComponent _output_get)) "Left"))
    (Variables|/Game/Blueprints/Components/GrabComponent.GrabComponent_C|SetcanGrab (Variables|/Game/Blueprints/Actors/Act3/BP_GrabbableSymbol.BP_GrabbableSymbol_C|GetGrabComponent _output_get) false)
    (Utilities|Array|Add _insertedsymbols (LocalVariables|Getsymbol))
    (if (== (Utilities|Array|Length _insertedsymbols) 2)
      (for _array_element _insertedsymbols
        (Default|DestroyGrab(Multicast) _array_element)
        (Default|SetSymbolState _array_element "NewEnumerator2")))
    (CallFunction|Test (LocalVariables|Getsymbol) (.location _returnvalue) (.rotation _returnvalue))))

(fn SetSymbolStates
  (params (New%20State :type SymbolState%20Enum :default "NewEnumerator0") (Incomplete%20Only :type Boolean))
  (if Incomplete%20Only
    (for _array_element (Variables|SequenceSystem|GetsequenceSymbolsLeft)
      (if (not (Utilities|Enum|Equal(Enum) (Variables|/Game/Blueprints/Actors/BP_Symbol.BP_Symbol_C|GetState _array_element) "NewEnumerator4"))
        (Default|SetSymbolState _array_element New%20State)))
    (for _array_element_2 (Variables|SequenceSystem|GetsequenceSymbolsRight)
      (if (not (Utilities|Enum|Equal(Enum) (Variables|/Game/Blueprints/Actors/BP_Symbol.BP_Symbol_C|GetState _array_element_2) "NewEnumerator4"))
        (Default|SetSymbolState _array_element_2 New%20State)))
    (else
      (for _array_element_3 (Variables|SequenceSystem|GetsequenceSymbolsLeft)
        (Default|SetSymbolState _array_element_3 New%20State))
      (for _array_element_4 (Variables|SequenceSystem|GetsequenceSymbolsRight)
        (Default|SetSymbolState _array_element_4 New%20State)))))

(fn OnRepColumnSequence
  (bind _columnsequence (Variables|Phase2|GetcolumnSequence))
  (Class|NiagaraDataInterfaceArrayFunctionLibrary|SetNiagaraArrayBool (Variables|Default|GetLeftShapeEmitter) "ShapeTypeArray" _columnsequence)
  (Class|NiagaraDataInterfaceArrayFunctionLibrary|SetNiagaraArrayBool (Variables|Default|GetRightShapeEmitter) "ShapeTypeArray" _columnsequence))

(fn RandomizeTargetSymbols
  (bind _oversymbols (LocalVariables|GetoverSymbols))
  (bind _overworldcolumns (Variables|Phase3|GetoverworldColumns))
  (bind _oversymbols_2 (LocalVariables|GetoverSymbols))
  (bind _glyphs (LocalVariables|Getglyphs))
  (bind _glyphs_2 (LocalVariables|Getglyphs))
  (bind _oversymbols_3 (LocalVariables|GetoverSymbols))
  (bind _undersymbols (LocalVariables|GetunderSymbols))
  (bind _underworldcolumns (Variables|Phase3|GetunderworldColumns))
  (bind _glyphs_3 (LocalVariables|Getglyphs))
  (bind _returnvalue (Utilities|Array|Length _glyphs_2))
  (Utilities|Array|AppendArray _undersymbols (Variables|/Game/Blueprints/Actors/Act3/BP_SymbolColumn.BP_SymbolColumn_C|GetunactivatedSymbols (Utilities|Array|Get(acopy) _underworldcolumns)))
  (Utilities|Array|AppendArray _undersymbols (Variables|/Game/Blueprints/Actors/Act3/BP_SymbolColumn.BP_SymbolColumn_C|GetunactivatedSymbols (Utilities|Array|Get(acopy) _underworldcolumns 1)))
  (Utilities|Array|AppendArray _oversymbols (Variables|/Game/Blueprints/Actors/Act3/BP_SymbolColumn.BP_SymbolColumn_C|GetunactivatedSymbols (Utilities|Array|Get(acopy) _overworldcolumns 1)))
  (Utilities|Array|AppendArray _oversymbols (Variables|/Game/Blueprints/Actors/Act3/BP_SymbolColumn.BP_SymbolColumn_C|GetunactivatedSymbols (Utilities|Array|Get(acopy) _overworldcolumns)))
  (Utilities|FlowControl|Sequence
    (:then_0
      ;[0.4768 0.5469 0.2189] Step 1: For Overworld, take everyone's glyphs, shuffle them, and give them back
      (for _array_element _oversymbols_2
        (Utilities|Array|Add _glyphs (Variables|/Game/Blueprints/Actors/BP_Symbol.BP_Symbol_C|GetGlyph _array_element)))
      (Utilities|Array|Shuffle _glyphs)
      (for (_array_element_2 _array_index) _oversymbols_2
        (Variables|/Game/Blueprints/Actors/BP_Symbol.BP_Symbol_C|SetGlyph _array_element_2 (Utilities|Array|Get(acopy) (LocalVariables|Getglyphs) _array_index))
        (Default|SetSymbolState _array_element_2 (select (Math|Conversions|ToBoolean(Integer) (Math|Integer|%(Integer) (Variables|Phase3|GetactivatedSymbols) 2)) "NewEnumerator1" "NewEnumerator2"))))
    (:then_1
      ;[1 0.1524 0.1027] Step 2: Shuffle the Underworld, but make sure the only glyph in common with its Overworld counterpart is the target symbol.
      (LocalVariables|SettargetSymbol (.OutItem (Utilities|Array|Random _oversymbols_3)))
      (for (_array_element_3 _array_index_2) _oversymbols_3
        (Utilities|FlowControl|Sequence
          (:then_0
            (if (== _array_element_3 (LocalVariables|GettargetSymbol))
              (bind _output_get (Variables|/Game/Blueprints/Actors/BP_Symbol.BP_Symbol_C|SetGlyph (Utilities|Array|Get(acopy) (LocalVariables|GetunderSymbols) _array_index_2) (Variables|/Game/Blueprints/Actors/BP_Symbol.BP_Symbol_C|GetGlyph _array_element_3)))
              (Utilities|Array|RemoveIndex _glyphs_3 (Utilities|Array|FindItem _glyphs_3 _output_get))
              (else
                (bind _output_get_2 (LocalVariables|SettempGlyph (Variables|/Game/Blueprints/Actors/BP_Symbol.BP_Symbol_C|GetGlyph _array_element_3)))
                (bind _output_get_3 (LocalVariables|SetdupesRemoved _returnvalue))
                (Utilities|Array|RemoveItem _glyphs_2 _output_get_2)
                (LocalVariables|SetdupesRemoved (- _output_get_3 _returnvalue))
                (if (Utilities|Array|IsEmpty _glyphs_2)
                  (Utilities|Array|AppendArray _glyphs_2 (Utilities|Array|MakeArray (Utilities|Enum|LiteralenumGlyph "NewEnumerator0") (Utilities|Enum|LiteralenumGlyph "NewEnumerator1") (Utilities|Enum|LiteralenumGlyph "NewEnumerator2") (Utilities|Enum|LiteralenumGlyph "NewEnumerator3")))
                  (Utilities|Array|RemoveItem _glyphs_2 (LocalVariables|GettempGlyph)))
                (bind _output_get_4 (LocalVariables|SetindexRemoved (.OutIndex (Utilities|Array|Random _glyphs_2))))
                (Variables|/Game/Blueprints/Actors/BP_Symbol.BP_Symbol_C|SetGlyph (Utilities|Array|Get(acopy) (LocalVariables|GetunderSymbols) _array_index_2) (Utilities|Array|Get(acopy) (LocalVariables|Getglyphs) _output_get_4))
                (Utilities|Array|RemoveIndex _glyphs_2 _output_get_4)
                (for _index (range 0 (- (LocalVariables|GetdupesRemoved) 1))
                  (Utilities|Array|Add _glyphs_2 (LocalVariables|GettempGlyph))))))
          (:then_1
            (Default|SetSymbolState (Utilities|Array|Get(acopy) (LocalVariables|GetunderSymbols) _array_index_2) (select (Math|Conversions|ToBoolean(Integer) (Math|Integer|%(Integer) (Variables|Phase3|GetactivatedSymbols) 2)) "NewEnumerator2" "NewEnumerator1"))))))))

(fn CreateShuffledSequence
  (bind _newsequence (LocalVariables|GetnewSequence))
  (bind _sequencepart (LocalVariables|GetsequencePart))
  (Utilities|Array|Shuffle _sequencepart)
  (Utilities|Array|AppendArray _newsequence _sequencepart)
  (Utilities|Array|Shuffle _sequencepart)
  (Utilities|Array|AppendArray _newsequence _sequencepart)
  (return _newsequence))