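; BP_LookingTest is a test actor that continuously turns to face the VR player's left hand.
; On BeginPlay it finds and stores the VRPawn.
; Each Tick it builds a rotation with MakeRotFromXZ, pointing X at HandLeft while keeping world up as the Z reference, and applies it to itself.
; A FindLookAtRotation alternative is left unconnected in the graph.
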(event EventBeginPlay
  (bind _returnvalue (Actor|GetActorOfClass "/Game/Blueprints/Actors/VRPawn.VRPawn_C"))
  (Variables|Default|SetVRPawn _returnvalue))

(event EventTick
  (params (DeltaSeconds :type Float%20%28single-precision%29))
  (Transformation|SetActorRotation (Math|Rotator|MakeRotfromXZ (- (Transformation|GetWorldLocation (Variables|/Game/Blueprints/Actors/VRPawn.VRPawn_C|GetHandLeft (Variables|Default|GetVRPawn))) (Transformation|GetActorLocation)) (Math|Vector|GetUpVector "0, 0, 0"))))

(fn ConstructionScript)