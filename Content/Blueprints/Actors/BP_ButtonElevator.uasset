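; Gate-derived elevator actor that raises an assigned IndiButton along with its own mesh when the gate opens.
; BeginPlay snaps the button to the mesh and orients it from the root's forward vector with a rotation offset, warning on screen if none is assigned.
; OpenGate runs the parent logic, then a timeline lerps mesh and button vertically by Elevation and calls CloseGate when finished.
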(event EventBeginPlay
  (bind _indibutton (Variables|Default|GetindiButton))
  (bind _defaultsceneroot (Variables|/Game/Blueprints/Actors/BP_IndiButton.BP_IndiButton_C|GetDefaultSceneRoot _indibutton))
  (if (Utilities|IsValid (Variables|Default|GetindiButton))
    (bind _output_get (Variables|Default|SetelevatorInitialLocation (Transformation|GetWorldLocation (Variables|Default|GetSM_ButtonElevator))))
    (Transformation|SetWorldLocation (Variables|/Game/Blueprints/Actors/BP_IndiButton.BP_IndiButton_C|GetDefaultSceneRoot (Variables|Default|GetindiButton)) _output_get false false)
    (Transformation|SetWorldRotation _defaultsceneroot (Math|Rotator|CombineRotators (Math|Rotator|FindLookatRotation (Transformation|GetWorldLocation _defaultsceneroot) (+ (Variables|Default|GetelevatorInitialLocation) (* (Math|Vector|GetForwardVector (Variables|Default|GetRoot)) 10))) "0.000000,90.000000,0.000000") false false)
    (else
      (Development|PrintString "Warning: no indi button assigned on BP_ButtonElevator" true true "(R=1.000000,G=0.026262,B=0.000000,A=1.000000)" 2e+01))))

(event EventOpenGate
  (bind _elevatorinitiallocation (Variables|Default|GetelevatorInitialLocation))
  (if (Utilities|IsValid (Variables|Default|GetindiButton))
    (Utilities|FlowControl|Sequence
      (:then_0
        (|CallParentFunction))
      (:then_1
        ;[1 1 1] Moving the indi button
        (bind _track_0 (Timeline|TL_ButtonElevator Play)
          (:Update
            (Transformation|SetWorldLocation (Variables|Default|GetSM_ButtonElevator) (Math|Vector|Lerp(Vector) _elevatorinitiallocation (+ _elevatorinitiallocation (Math|Vector|MakeVector 0.0 0.0 (Variables|Default|Getelevation))) _track_0) false false)
            (Transformation|SetWorldLocation (Variables|/Game/Blueprints/Actors/BP_IndiButton.BP_IndiButton_C|GetDefaultSceneRoot (Variables|Default|GetindiButton)) (Math|Vector|Lerp(Vector) _elevatorinitiallocation (+ _elevatorinitiallocation (Math|Vector|MakeVector 0.0 0.0 (Variables|Default|Getelevation))) _track_0) false false))
          (:Finished
            (CallFunction|CloseGate)))))
    (else
      (Development|PrintString "Warning: no indi button assigned on BP_ButtonElevator" true true "(R=1.000000,G=0.026262,B=0.000000,A=1.000000)" 2e+01))))

(fn ConstructionScript
  (|CallParentFunction))