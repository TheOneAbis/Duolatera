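; VR grabbable item, configurable as a holster or laser pen, that attaches to the player or returns to its start transform.
; An integer selects which grabbed and attached events fire.
; Dropping it within range of the pawn's chest socket destroys it and fires attachment, also revealing the laser tool for the pen.
; Otherwise, after a cooldown, a timeline interpolates it back to the saved transform, stopping if regrabbed.
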(event OnGrabbed(GrabComponent)
  (switch int (Variables|Default|GetintToAssign)
    (:0
      (Default|CallHolsterGrabbed))
    (:1
      (Default|CallLaserPenGrabbed))))

(event Custom|OnDroppedEvent
  ;[1 1 1] Calculate the distance from the holster placeholder to the actual holster and set the material when near
  (EventDispatchers|BindEventtoOnDropped (Variables|Default|GetGrabComponent) (delegate Custom|OnGrabbableItemDropped)))

(event Custom|OnGrabbableItemDropped
  (bind _attachable (Variables|Default|GetAttachable))
  ;[1 1 1] Calculate the distance from the holster placeholder to the actual holster and set the material when near
  (Utilities|IsValid (Variables|Default|GetVRPawn)
    (:Is%20Valid
      (Utilities|FlowControl|Sequence
        (:then_0
          (Development|PrintString "On the ground")
          (Timeline|Cooldown PlayFromStart
            (:Finished
              (bind _isheld (Default|CheckifHeld (Variables|Default|GetGrabComponent)))
              (if (not _isheld)
                (Default|SetPrimitiveCompPhysics (Variables|Default|GetGrabComponent) false)
                (bind _snap (Timeline|Timeline PlayFromStart)
                  (:Update
                    (Utilities|FlowControl|Sequence
                      (:then_0
                        (bind _isheld_2 (Default|CheckifHeld (Variables|Default|GetGrabComponent)))
                        (if _isheld_2
                          (Timeline|Timeline Stop)))
                      (:then_1
                        (Transformation|SetWorldLocation _attachable (Math|Vector|Lerp(Vector) (Transformation|GetWorldLocation (Variables|Default|GetAttachable)) (Variables|Default|GetStartLocation) _snap) false true))
                      (:then_2
                        (Transformation|SetWorldRotation _attachable (Class|KismetMathLibrary|QuatRotator (Class|KismetMathLibrary|QuatSlerp (Math|Conversions|ToQuaternion(Rotator) (Transformation|GetWorldRotation (Variables|Default|GetAttachable))) (Math|Conversions|ToQuaternion(Rotator) (Variables|Default|GetStartRotation)) _snap)) false true)))))))))
        (:then_1
          (if (<= (Math|Vector|VectorLength (- (Transformation|GetSocketLocation (Variables|/Game/Blueprints/Actors/VRPawn.VRPawn_C|GetPlayerSkeletalMesh (Variables|Default|GetVRPawn)) "ChestSocket") (Transformation|GetWorldLocation (Variables|Default|GetGrabComponent)))) (Variables|Default|GetHolsterRadius))
            (bind _isheld_3 (Default|CheckifHeld (Variables|Default|GetGrabComponent)))
            (if (not _isheld_3)
              (Utilities|IsValid (Variables|Default|GetAttachable)
                (:Is%20Valid
                  (Actor|DestroyActor)
                  (switch int (Variables|Default|GetintToAssign)
                    (:0
                      (Development|PrintString "Material changed")
                      (Default|CallHolsterAttached))
                    (:1
                      (bind _returnvalue (Actor|GetActorOfClass "/Game/Blueprints/Actors/LaserTool.LaserTool_C"))
                      (Rendering|SetVisibility (Variables|/Game/Blueprints/Actors/LaserTool.LaserTool_C|GetSkeletalMeshGun _returnvalue) true false)
                      (Collision|SetCollisionProfileName (Variables|/Game/Blueprints/Actors/LaserTool.LaserTool_C|GetSkeletalMeshGun _returnvalue) "PhysicsActor" true :!class /Script/Engine.PrimitiveComponent)
                      (Default|CallLaserPenAttached))))))))))
    (:Is%20Not%20Valid
      (Development|PrintString "Not Valid"))))

(event Custom|SetAttachableLocationAndRotation
  (bind _attachable (Variables|Default|GetAttachable))
  ;[1 1 1] Set Attachable location and rotation
  (Variables|Default|SetStartLocation (Transformation|GetWorldLocation _attachable))
  (Variables|Default|SetStartRotation (Transformation|GetWorldRotation _attachable)))

(event Custom|SetItemRelativeLocationAndRotation
  (bind _grabcomponent (Variables|Default|GetGrabComponent))
  ;[1 1 1] Set Item Location and Rotation
  (CallFunction|SetAttachableLocationandRotation)
  (Variables|/Game/Blueprints/Components/GrabComponent.GrabComponent_C|SetcanGrab _grabcomponent true)
  (Variables|/Game/Blueprints/Components/GrabComponent.GrabComponent_C|SetbSimulateOnDrop _grabcomponent true)
  (Default|SetPrimitiveCompPhysics (Variables|Default|GetGrabComponent) true))

(event EventBeginPlay
  (bind _raycaststartlocation (Variables|Default|GetRayCastStartLocation))
  ;[1 1 1] Get Foor height, set holster material and set the attachables location and rotation
  (bind _returnvalue (Actor|GetActorOfClass "/Game/Blueprints/Actors/VRPawn.VRPawn_C"))
  (Variables|Default|SetVRPawn _returnvalue)
  (bind _outhit (Collision|LineTraceByChannel (Math|Vector|MakeVector (.x _raycaststartlocation) (.y _raycaststartlocation) (.z _raycaststartlocation)) (Math|Vector|MakeVector 0.0 0.0 (* (.z _raycaststartlocation) -1e+03)) "TraceTypeQuery1" false 0 "None" true "(R=1.000000,G=0.000000,B=0.000000,A=1.000000)" "(R=0.000000,G=1.000000,B=0.000000,A=1.000000)" 1e+01))
  (Variables|Default|SetFloorHeight (.z (Transformation|GetActorLocation (.HitActor (Collision|BreakHitResult _outhit))))))

(event Collision|EventActorBeginOverlap
  (params (OtherActor :type Actor%20Object%20Reference)))

(fn ConstructionScript
  (Components|StaticMesh|SetStaticMesh (Variables|Default|GetAttachable) (Variables|Default|GetSMAttachable))
  (Rendering|Material|SetMaterial (Variables|Default|GetAttachable) 0 (Variables|Default|GetMAttachable))
  (CallFunction|OnDroppedEvent))