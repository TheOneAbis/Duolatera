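; BP_WorldRegion is a region actor that switches rendering between overworld and underworld as the player crosses its UnderworldTrigger.
; On entry, actors inside the OverworldTrigger box become scene-capture-only and the BP_UnderworldSky mesh becomes main-view visible but capture-hidden; exit reverses both.
; Any actor entering the underworld trigger is made fully visible.
; BeginPlay caches the sky actor, warning unless exactly one exists.
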(event OnComponentBeginOverlap(UnderworldTrigger)
  (params (OverlappedComponent :type Primitive%20Component%20Object%20Reference) (OtherActor :type Actor%20Object%20Reference) (OtherComp :type Primitive%20Component%20Object%20Reference) (OtherBodyIndex :type Integer) (bFromSweep :type Boolean) (SweepResult :type Hit%20Result%20Structure%20%28by%20ref%29))
  (bind _skybox (Variables|Default|Getskybox))
  (bind _staticmesh (Variables|/Game/Blueprints/Actors/BP_UnderworldSky.BP_UnderworldSky_C|GetStaticMesh _skybox))
  ;[1 1 1] Sets the Overworld to be visible/invisible depending on if the player is in the underworld
  (CallFunction|SetActorVisible OtherActor true)
  (if (== OtherActor (Game|Player|GetPlayerPawn 0))
    (Utilities|FlowControl|DelayUntilNextTick)
    (CallFunction|SetOverworldVisible false)
    (Utilities|IsValid _skybox
      (:Is%20Valid
        (Class|PrimitiveComponent|SetHiddeninSceneCapture _staticmesh true)
        (Class|PrimitiveComponent|SetVisibleinSceneCaptureOnly _staticmesh false)))))

(event OnComponentEndOverlap(UnderworldTrigger)
  (params (OverlappedComponent :type Primitive%20Component%20Object%20Reference) (OtherActor :type Actor%20Object%20Reference) (OtherComp :type Primitive%20Component%20Object%20Reference) (OtherBodyIndex :type Integer))
  (bind _skybox (Variables|Default|Getskybox))
  (bind _staticmesh (Variables|/Game/Blueprints/Actors/BP_UnderworldSky.BP_UnderworldSky_C|GetStaticMesh _skybox))
  ;[1 1 1] Sets the Overworld to be visible/invisible depending on if the player is in the underworld
  (if (== OtherActor (Game|Player|GetPlayerPawn 0))
    (CallFunction|SetOverworldVisible true)
    (Utilities|IsValid _skybox
      (:Is%20Valid
        (Class|PrimitiveComponent|SetHiddeninSceneCapture _staticmesh false)
        (Class|PrimitiveComponent|SetVisibleinSceneCaptureOnly _staticmesh true)))))

(event Custom|Set%20Actor%20Visible
  (params (actor :type Actor%20Object%20Reference) (visible :type Boolean))
  ;[1 1 1] Sets the Overworld to be visible/invisible depending on if the player is in the underworld
  (for _array_element (Actor|GetComponentsByClass actor "/Script/Engine.MeshComponent")
    (Class|PrimitiveComponent|SetVisibleinSceneCaptureOnly _array_element (not visible))))

(event Custom|Set%20Overworld%20Visible
  (params (Render :type Boolean))
  (bind _overworldtrigger (Variables|Default|GetOverworldTrigger))
  ;[1 1 1] Sets the Overworld to be visible/invisible depending on if the player is in the underworld
  (bind _outactors (Collision|BoxOverlapActors (Transformation|GetWorldLocation _overworldtrigger) (Components|Box|GetScaledBoxExtent _overworldtrigger) (Utilities|Array|MakeArray "ObjectTypeQuery1" "ObjectTypeQuery2" "ObjectTypeQuery4" "ObjectTypeQuery3") 0 (Utilities|Array|MakeArray self) :!class /Script/Engine.KismetSystemLibrary))
  (for _array_element _outactors
    (CallFunction|SetActorVisible _array_element Render)))

(event EventBeginPlay
  (bind _outactors (Actor|GetAllActorsOfClass "/Game/Blueprints/Actors/BP_UnderworldSky.BP_UnderworldSky_C"))
  (if (== (Utilities|Array|Length _outactors) 1)
    (Variables|Default|Setskybox (Utilities|Array|Get(acopy) _outactors))
    (else
      (Development|PrintString (Utilities|String|BuildString(Integer) "WARNING: " "" (Utilities|Array|Length _outactors) " UNDERWORLD SKYBOXES FOUND! Make sure there is exactly ONE of these in your scene!") true true "(R=1.000000,G=0.053420,B=0.000000,A=1.000000)" 1e+01))))

(fn ConstructionScript)