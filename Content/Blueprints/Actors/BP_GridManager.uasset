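; Grid manager actor that builds a square checkers board of BP_GridNode actors at BeginPlay and spawns BP_CheckerPiece on the Y=0 row.
; Positions are offset and rotated by GridOrigin, which the construction script previews.
; Directional helpers link neighbours both ways using X+Y*GridSize indices, although GridNodes fills as X*GridSize+Y.
; IsAdjacent checks those links; FindNearestNode returns the first node closer than stored MinDistance, not necessarily the nearest.
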(event EventBeginPlay
  (bind _gridsize (Variables|Default|GetgridSize))
  (bind _gridnodes (Variables|Default|GetGridNodes))
  (bind _nodespacing (Variables|Default|Getnodespacing))
  (bind _returnvalue (- _gridsize 1))
  (for _index (range 0 _returnvalue)
    (for _index_2 (range 0 _returnvalue)
      (bind _gridoriginconversion (CallFunction|ConvertbyGridOrigin (Math|Transform|MakeTransform (Math|Vector|MakeVector (Math|Conversions|ToFloat(Integer) (* _index (Variables|Default|Getnodespacing))) (Math|Conversions|ToFloat(Integer) (* _index_2 (Variables|Default|Getnodespacing))) 0.0))))
      (bind _returnvalue_2 (Game|SpawnActorfromClass "/Game/Blueprints/Actors/BP_GridNode.BP_GridNode_C" _gridoriginconversion "Undefined" "MultiplyWithRoot" 0 0))
      (Variables|/Game/Blueprints/Actors/BP_GridNode.BP_GridNode_C|SetX _returnvalue_2 _index)
      (Variables|/Game/Blueprints/Actors/BP_GridNode.BP_GridNode_C|SetY _returnvalue_2 _index_2)
      (Utilities|Array|Add _gridnodes _returnvalue_2)))
  (for _array_element _gridnodes
    (Utilities|FlowControl|Sequence
      (:then_0
        (if (== (Variables|/Game/Blueprints/Actors/BP_GridNode.BP_GridNode_C|GetY _array_element) 0)
          (bind _gridoriginconversion_2 (CallFunction|ConvertbyGridOrigin (Math|Transform|MakeTransform (Math|Vector|MakeVector (Math|Conversions|ToFloat(Integer) (* (Variables|/Game/Blueprints/Actors/BP_GridNode.BP_GridNode_C|GetX _array_element) _nodespacing)) (Math|Conversions|ToFloat(Integer) (* (Variables|/Game/Blueprints/Actors/BP_GridNode.BP_GridNode_C|GetY _array_element) _nodespacing)) 0.0))))
          (bind _returnvalue_3 (Game|SpawnActorfromClass "/Game/Blueprints/Actors/BP_CheckerPiece.BP_CheckerPiece_C" _gridoriginconversion_2 "Undefined" "MultiplyWithRoot" 0 0))
          (Variables|/Game/Blueprints/Actors/BP_GridNode.BP_GridNode_C|SetbIsOccupied _array_element true)
          (Variables|/Game/Blueprints/Actors/BP_CheckerPiece.BP_CheckerPiece_C|SetCurrentGridNode _returnvalue_3 _array_element)))
      (:then_1
        (Utilities|EastNode _array_element))
      (:then_2
        (Utilities|WestNode _array_element))
      (:then_3
        (Utilities|SouthNode _array_element))
      (:then_4
        (Utilities|NorthNode _array_element)))))

(event Collision|EventActorBeginOverlap
  (params (OtherActor :type Actor%20Object%20Reference)))

(event EventTick
  (params (DeltaSeconds :type Float%20%28single-precision%29)))

(fn ConstructionScript
  (bind _gridorigin (Variables|Default|GetGridOrigin))
  (Transformation|SetWorldTransform (Variables|Default|GetGridOriginSceneComp) (Variables|Default|GetGridOrigin) false false)
  (Rendering|Debug|DrawDebugLine (.location _gridorigin) (+ (.location _gridorigin) (Math|Vector|RotateVector (Math|Vector|MakeVector 1e+02 1e+02 0.0) (.rotation _gridorigin))) "(R=0.729167,G=0.028996,B=0.000000,A=1.000000)" 0.0 4.0))

(fn FindNearestNode
  (params (WorldLocation :type Vector))
  (for _array_element (Variables|Default|GetGridNodes)
    (if (< (Math|Vector|Distance(Vector) (Transformation|GetWorldLocation (Variables|/Game/Blueprints/Actors/BP_GridNode.BP_GridNode_C|GetStaticMesh _array_element)) WorldLocation) (Variables|Default|GetMinDistance))
      (Variables|Default|SetMinDistance (Math|Vector|Distance(Vector) (Transformation|GetWorldLocation (Variables|/Game/Blueprints/Actors/BP_GridNode.BP_GridNode_C|GetStaticMesh _array_element)) WorldLocation))
      (return _array_element))))

(fn ConvertbyGridOrigin
  (params (localSpace :type Transform))
  (bind _gridorigin (Variables|Default|GetGridOrigin))
  (return (Math|Transform|MakeTransform (+ (.location _gridorigin) (Math|Vector|RotateVector (.location localSpace) (.rotation _gridorigin))) (.rotation _gridorigin) (.scale _gridorigin))))

(fn IsAdjacent
  (params (NodeA :type BP%20Grid%20Node%20Object%20Reference) (NodeB :type BP%20Grid%20Node%20Object%20Reference))
  (return (Utilities|Array|ContainsItem (Variables|/Game/Blueprints/Actors/BP_GridNode.BP_GridNode_C|GetConnectedNodes NodeA) NodeB)))