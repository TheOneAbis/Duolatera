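; Grabbable pistol actor that fires a portal-aware laser-tag style trace from its muzzle while interacted with.
; Interact begin enables Tick, and interact end or dropping from the snap grab component disables it.
; Each Tick runs a debug-drawn PortalLineTrace and sends any hit to the hit actor via OnTaggedMessage.
; BeginPlay colors the gun blue or green by PlayerIndex; an OnRep function applies GunMaterial.
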(event OnDropped(GrabComponentSnap)
  (Actor|Tick|SetActorTickEnabled false))

(event EventTick
  (params (DeltaSeconds :type Float%20%28single-precision%29))
  (bind _muzzlelocation (Variables|Default|GetMuzzleLocation))
  (bind (_actorstoignore _outhit _returnvalue) (Class|ExtraBlueprintFunctionLibrary|PortalLineTrace (Transformation|GetWorldLocation _muzzlelocation) (Math|Vector|GetForwardVector _muzzlelocation) 1e+03 "TraceTypeQuery1" false "ForOneFrame" true "(R=1.000000,G=0.000000,B=0.000000,A=1.000000)" "(R=0.000000,G=1.000000,B=0.000000,A=1.000000)" 1.0))
  (if _returnvalue
    (Class|Taggable|OnTagged(Message) (.HitActor (Collision|BreakHitResult _outhit)) _outhit)))

(event EventBeginPlay
  (switch int (Variables|Default|GetPlayer%20Index)
    (:0
      (Rendering|Material|SetMaterial (Variables|Default|GetSkeletalMeshGun) 0 "/Game/Assets/Materials/MaterialInstance/MI_Pistol_Blue.MI_Pistol_Blue"))
    (:1
      (Rendering|Material|SetMaterial (Variables|Default|GetSkeletalMeshGun) 0 "/Game/Assets/Materials/MaterialInstance/MI_Pistol_Green.MI_Pistol_Green"))))

(event EventOnInteractEnd
  (params (controller :type Motion%20Controller%20Component%20Object%20Reference))
  (Actor|Tick|SetActorTickEnabled false))

(event EventOnInteractBegin
  (params (controller :type Motion%20Controller%20Component%20Object%20Reference))
  (Actor|Tick|SetActorTickEnabled true))

(fn ConstructionScript)

(fn OnRepGunMaterial
  (Rendering|Material|SetMaterial (Variables|Default|GetSkeletalMeshGun) 0 (Variables|Default|GetGunMaterial)))