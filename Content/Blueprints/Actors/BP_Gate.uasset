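; Replicated iris-style gate whose sectors slide outward radially and rotate to open, toggled by Activate/Deactivate relative to OpenedAtStart.
; The Opend RepNotify runs the open/close timeline, toggles gateway collision and fires dispatchers, with sound offsets matched to animation progress.
; CalculateOpenLocRot derives each sector's target from index and count, blended via location lerp and quaternion slerp.
; Construction script gathers sectors, caches rotations and selects red Underworld or blue materials.
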(event Custom|OpenGate
  (bind _door_open_cue (Variables|Default|GetDoor%20Open%20Cue))
  (bind _gatesectors (Variables|Default|GetgateSectors))
  (Audio|Components|Audio|Stop (Variables|Default|GetDoor%20Close%20Cue))
  (Audio|Components|Audio|Play _door_open_cue (Math|Float|Lerp 0.0 (* (Variables|/Script/Engine.SoundBase|GetDuration (Variables|/Script/Engine.AudioComponent|GetSound _door_open_cue)) 0.8) (Variables|Default|GetanimTime)))
  (bind _lrtrack (Timeline|GateAnimation Play)
    (:Update
      (bind _output_get (Variables|Default|SetanimTime _lrtrack))
      (for (_array_element _array_index) _gatesectors
        (bind (_sectorlocation _sectorrotation) (CallFunction|CalculateOpenLocRot _array_element _array_index (Utilities|Array|Length _gatesectors)))
        (Transformation|SetRelativeLocationAndRotation _array_element (Math|Vector|Lerp(Vector) "0, 0, 0" _sectorlocation _output_get) (Class|KismetMathLibrary|QuatRotator (Class|KismetMathLibrary|QuatSlerp (Math|Conversions|ToQuaternion(Rotator) (Utilities|Array|Get(acopy) (Variables|Default|GetinitialTransforms) _array_index)) (Math|Conversions|ToQuaternion(Rotator) _sectorrotation) _output_get)) false false)))))

(event Custom|CloseGate
  (bind _door_close_cue (Variables|Default|GetDoor%20Close%20Cue))
  (bind _gatesectors (Variables|Default|GetgateSectors))
  (Audio|Components|Audio|Stop (Variables|Default|GetDoor%20Open%20Cue))
  (Audio|Components|Audio|Play _door_close_cue (Math|Float|Lerp (* (Variables|/Script/Engine.SoundBase|GetDuration (Variables|/Script/Engine.AudioComponent|GetSound _door_close_cue)) 0.55) 0.0 (Variables|Default|GetanimTime)))
  (bind _lrtrack (Timeline|GateAnimation Reverse)
    (:Update
      (bind _output_get (Variables|Default|SetanimTime _lrtrack))
      (for (_array_element _array_index) _gatesectors
        (bind (_sectorlocation _sectorrotation) (CallFunction|CalculateOpenLocRot _array_element _array_index (Utilities|Array|Length _gatesectors)))
        (Transformation|SetRelativeLocationAndRotation _array_element (Math|Vector|Lerp(Vector) "0, 0, 0" _sectorlocation _output_get) (Class|KismetMathLibrary|QuatRotator (Class|KismetMathLibrary|QuatSlerp (Math|Conversions|ToQuaternion(Rotator) (Utilities|Array|Get(acopy) (Variables|Default|GetinitialTransforms) _array_index)) (Math|Conversions|ToQuaternion(Rotator) _sectorrotation) _output_get)) false false)))))

(event Custom|DisableGatewayCollision
  (Collision|SetCollisionEnabled (Variables|Default|GetGatewayBlock) "NoCollision"))

(event Custom|EnableGatewayCollision
  (Collision|SetCollisionEnabled (Variables|Default|GetGatewayBlock) "QueryAndProbe"))

(event EventActivate
  (Variables|Default|SetbOpend (not (Variables|Default|GetbOpenedAtStart))))

(event EventDeactivate
  (Variables|Default|SetbOpend (Variables|Default|GetbOpenedAtStart)))

(event EventBeginPlay
  (bind _gatesectors (Variables|Default|GetgateSectors))
  (if (Variables|Default|GetbOpenedAtStart)
    (for (_array_element _array_index) _gatesectors
      (bind (_sectorlocation _sectorrotation) (CallFunction|CalculateOpenLocRot _array_element _array_index (Utilities|Array|Length _gatesectors)))
      (Transformation|SetRelativeLocationAndRotation _array_element _sectorlocation _sectorrotation false false)
      (Components|Timeline|SetNewTime (Variables|Default|GetGateAnimation) 2.0)
      (CallFunction|DisableGatewayCollision))))

(fn ConstructionScript
  (bind _gatesectors (Variables|Default|GetgateSectors))
  (bind _sm_gateframe (Variables|Default|GetSM_GateFrame))
  (Utilities|Array|Clear (Variables|Default|GetgateSectors))
  (Utilities|FlowControl|Sequence
    (:then_0
      (Utilities|Array|Add _gatesectors (Variables|Default|GetSM_GateSector))
      (Utilities|Array|Add _gatesectors (Variables|Default|GetSM_GateSector1))
      (Utilities|Array|Add _gatesectors (Variables|Default|GetSM_GateSector2))
      (Utilities|Array|Add _gatesectors (Variables|Default|GetSM_GateSector3))
      (Utilities|Array|Add _gatesectors (Variables|Default|GetSM_GateSector4))
      (Utilities|Array|Add _gatesectors (Variables|Default|GetSM_GateSector5)))
    (:then_1
      (for _array_element (Variables|Default|GetgateSectors)
        (Utilities|Array|Add (Variables|Default|GetinitialTransforms) (Variables|/Script/Engine.SceneComponent|GetRelativeRotation _array_element))))
    (:then_2
      (if (Variables|Default|GetIsUnderworldGate)
        (bind _returnvalue (Rendering|Material|CreateDynamicMaterialInstance _sm_gateframe 0 "/Game/Assets/Materials/MaterialInstance/PropMI/MI_Cel_Gate_Red.MI_Cel_Gate_Red" "None" :!class /Script/Engine.PrimitiveComponent))
        (Rendering|Material|SetMaterial _sm_gateframe 0 _returnvalue)
        (for _array_element_2 (Variables|Default|GetgateSectors)
          (bind _returnvalue_2 (Rendering|Material|CreateDynamicMaterialInstance _array_element_2 0 "/Game/Assets/Materials/MaterialInstance/PropMI/MI_Cel_GateSector_Red.MI_Cel_GateSector_Red" "None" :!class /Script/Engine.PrimitiveComponent))
          (Rendering|Material|SetMaterial (stale _array_element_3) 0 _returnvalue_2))
        (else
          (bind _returnvalue_3 (Rendering|Material|CreateDynamicMaterialInstance _sm_gateframe 0 "/Game/Assets/Materials/MaterialInstance/PropMI/MI_Cel_Gate_Blue.MI_Cel_Gate_Blue" "None" :!class /Script/Engine.PrimitiveComponent))
          (Rendering|Material|SetMaterial _sm_gateframe 0 _returnvalue_3)
          (for _array_element_3 (Variables|Default|GetgateSectors)
            (bind _returnvalue_4 (Rendering|Material|CreateDynamicMaterialInstance _array_element_3 0 "/Game/Assets/Materials/MaterialInstance/PropMI/MI_Cel_GateSector_Blue.MI_Cel_GateSector_Blue" "None" :!class /Script/Engine.PrimitiveComponent))
            (Rendering|Material|SetMaterial _array_element_3 0 _returnvalue_4)))))))

(fn OnRepBOpend
  (if (Variables|Default|GetbOpend)
    (CallFunction|OpenGate)
    (CallFunction|DisableGatewayCollision)
    (Default|CallOnOpenedDispatch)
    (else
      (CallFunction|CloseGate)
      (CallFunction|EnableGatewayCollision)
      (Default|CallOnClosedDispatch))))

(fn CalculateOpenLocRot
  (params (IndividualSector :type Static%20Mesh%20Component%20Object%20Reference) (ArrayIndex :type Integer) (TotalSectorAmount :type Integer))
  (bind _sm_gateframe (Variables|Default|GetSM_GateFrame))
  (return (+ (Math|Vector|VectorZero) (* (Math|Vector|RotateVectorAroundAxis (Math|Transform|InverseTransformDirection (Transformation|GetWorldTransform IndividualSector) (Math|Vector|GetUpVector IndividualSector)) (Math|Conversions|ToFloat(Integer) (* ArrayIndex (Math|Float|SafeDivide -3.6e+02 (Math|Conversions|ToFloat(Integer) TotalSectorAmount)))) (Math|Transform|InverseTransformDirection (Transformation|GetWorldTransform _sm_gateframe) (Math|Vector|GetForwardVector _sm_gateframe))) (Variables|Default|GetsectorMoveDistance))) (Math|Rotator|CombineRotators (Utilities|Array|Get(acopy) (Variables|Default|GetinitialTransforms) ArrayIndex) (Math|Rotator|MakeRotator (Variables|Default|GetsectorRotateAngle) 0.0 0.0))))