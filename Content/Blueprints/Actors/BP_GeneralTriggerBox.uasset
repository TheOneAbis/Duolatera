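; BP_GeneralTriggerBox is a one-shot, replicated trigger actor that toggles a target door when one designated actor overlaps its sphere.
; BeginPlay validates the accepted and triggered actor references, and only the authority sets IsTriggered on a matching overlap.
; The RepNotify runs TriggeredEvent, which calls Toggle through the door interactable interface, activates a Niagara torus burst and deactivates the swirl effect after a short delay.
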(event OnComponentBeginOverlap(Sphere)
  (params (OverlappedComponent :type Primitive%20Component%20Object%20Reference) (OtherActor :type Actor%20Object%20Reference) (OtherComp :type Primitive%20Component%20Object%20Reference) (OtherBodyIndex :type Integer) (bFromSweep :type Boolean) (SweepResult :type Hit%20Result%20Structure%20%28by%20ref%29))
  (Networking|SwitchHasAuthority
    (:Authority
      (if (Math|Boolean|ANDBoolean (Variables|Default|GetactorsValid) (== OtherActor (Variables|Default|GetacceptedActor)) (not (Variables|Default|GetisTriggered)))
        (Variables|Default|SetisTriggered true)))))

(event Custom|TriggeredEvent
  (bind _asbpi_door_interactable (Utilities|Casting|CastToBPI_Door_Interactable (Variables|Default|GettriggeredActor)))
  (Default|Toggle _asbpi_door_interactable)
  (Components|Activation|Activate (Variables|Default|GetNS_TorusBurst) false)
  (Utilities|FlowControl|Delay 0.5)
  (Components|Activation|Deactivate (Variables|Default|GetNS_Swirl)))

(event EventBeginPlay
  (Variables|Default|SetactorsValid (and (Utilities|IsValid (Variables|Default|GetacceptedActor)) (Utilities|IsValid (Variables|Default|GettriggeredActor)))))

(fn ConstructionScript)

(fn OnRepIsTriggered
  (if (Variables|Default|GetisTriggered)
    (CallFunction|TriggeredEvent)))