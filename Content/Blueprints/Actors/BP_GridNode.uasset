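; BP_GridNode is a grid node actor that classifies itself by its X and Y position within a grid of GridSize.
; On BeginPlay it waits one tick, then sets IsEdgeNode.
; The flag is true only when both coordinates lie on the first or last index, so despite its name it marks just the corner nodes.
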(event EventBeginPlay
  (bind _x (Variables|Default|GetX))
  (bind _y (Variables|Default|GetY))
  (Utilities|FlowControl|DelayUntilNextTick)
  (if (and (or (== _x 0) (== _x (- (Variables|Default|GetGridSize) 1))) (or (== _y 0) (== _y (- (Variables|Default|GetGridSize) 1))))
    (Variables|Default|SetbIsEdgeNode true)
    (else
      (Variables|Default|SetbIsEdgeNode false))))

(event Collision|EventActorBeginOverlap
  (params (OtherActor :type Actor%20Object%20Reference)))

(event EventTick
  (params (DeltaSeconds :type Float%20%28single-precision%29)))

(fn ConstructionScript)