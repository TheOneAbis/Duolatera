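; BP_HologramPlane is an Act 2 Phase 2 triangle hologram with up or down variants, chosen by IsUpsideDown in the construction script.
; It starts dark and lights dimly when the Cannon begins phase two.
; Activate brightens it, BlinkRed flashes then restores the variant color, and BlinkGreen turns green after a delay without resetting.
; Color and Intensity drive material parameters through RepNotify, so changes replicate to clients.
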(event Custom|LightUp
  (Variables|Default|SetIntensity 2.0))

(event Custom|LightBright
  (Variables|Default|SetIntensity 15.0))

(event Custom|BlinkRed
  (Variables|Default|SetIntensity 25.0)
  (Variables|Default|SetColor "1.000000,0.000000,0.000000")
  (Utilities|FlowControl|Delay 0.5)
  (Variables|Default|SetIntensity 2.0)
  (if (Variables|Default|GetisUpsideDown)
    (Variables|Default|SetColor "0.219526,0.040915,0.913099")
    (else
      (Variables|Default|SetColor "0.806952,0.064803,0.930111"))))

(event Custom|Fade
  (Variables|Default|SetIntensity 0.0))

(event Custom|BlinkGreen
  (Utilities|FlowControl|Delay 0.5)
  (Variables|Default|SetIntensity 25.0)
  (Variables|Default|SetColor "0.000000,1.000000,0.000000"))

(event EventBeginPlay
  (EventDispatchers|BindEventtoBeginPhaseTwo (Variables|Default|GetCannon) (delegate Custom|LightUp))
  (CallFunction|Fade)
  (if (Variables|Default|GetisUpsideDown)
    (Variables|Default|SetColor "0.219526,0.040915,0.913099")
    (else
      (Variables|Default|SetColor "0.806952,0.064803,0.930111"))))

(event EventTick
  (params (DeltaSeconds :type Float%20%28single-precision%29)))

(event EventActivate
  (CallFunction|LightBright))

(fn ConstructionScript
  (bind _plane (Variables|Default|GetPlane))
  (if (Variables|Default|GetisUpsideDown)
    (Rendering|Material|SetMaterial _plane 0 "/Game/Assets/Materials/MaterialInstance/MI_Triangle_DOWN.MI_Triangle_DOWN")
    (else
      (Rendering|Material|SetMaterial _plane 0 "/Game/Assets/Materials/MaterialInstance/MI_Triangle_UP.MI_Triangle_UP"))))

(fn OnRepColor
  (Rendering|Material|SetVectorParameterValueonMaterials (Variables|Default|GetPlane) "Color" (Variables|Default|GetColor)))

(fn OnRepIntensity
  (Rendering|Material|SetScalarParameterValueonMaterials (Variables|Default|GetPlane) "Intensity" (Variables|Default|GetIntensity)))