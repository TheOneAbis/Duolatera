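; BP_Lock is a key lock that takes a dropped-in BP_GrabbableSymbol and checks its glyph against the answer symbol.
; On server overlap it releases the symbol from player 0's right hand, snaps and locks it in place, then begins interaction or signals failure.
; Eject ends interaction and launches the symbol back out with physics.
; A Tick-driven, replicated cover progress gates overlap input and drives the cover's dissolve material through OnRep.
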(event OnComponentBeginOverlap(Box)
  (params (OverlappedComponent :type Primitive%20Component%20Object%20Reference) (OtherActor :type Actor%20Object%20Reference) (OtherComp :type Primitive%20Component%20Object%20Reference) (OtherBodyIndex :type Integer) (bFromSweep :type Boolean) (SweepResult :type Hit%20Result%20Structure%20%28by%20ref%29))
  (bind _box (Variables|Default|GetBox))
  (bind _returnvalue (Transformation|GetWorldTransform _box))
  (Networking|SwitchHasAuthority
    (:Authority
      (bind _asbp_grabbable_symbol (Utilities|Casting|CastToBP_GrabbableSymbol OtherActor))
      (Variables|Default|SetInputKeySymbol _asbp_grabbable_symbol)
      (Variables|/Script/Engine.PrimitiveComponent|SetbGenerateOverlapEvents (Variables|Default|GetBox) false)
      (bind _asvrpawn (Utilities|Casting|CastToVRPawn (Game|Player|GetPlayerPawn 0)))
      (Variables|/Game/Blueprints/Components/GrabComponent.GrabComponent_C|SetbSimulateOnDrop (Variables|/Game/Blueprints/Actors/Act3/BP_GrabbableSymbol.BP_GrabbableSymbol_C|GetGrabComponent (Variables|Default|GetInputKeySymbol)) false)
      (Default|RPCServerTryRelease _asvrpawn (Variables|/Game/Blueprints/Actors/Act3/BP_GrabbableSymbol.BP_GrabbableSymbol_C|GetGrabComponent (Variables|Default|GetInputKeySymbol)) false)
      (Utilities|FlowControl|Delay 0.2)
      (Transformation|SetActorLocationAndRotation (Variables|Default|GetInputKeySymbol) (.location _returnvalue) (.rotation _returnvalue))
      (Variables|/Game/Blueprints/Components/GrabComponent.GrabComponent_C|SetcanGrab (Variables|/Game/Blueprints/Actors/Act3/BP_GrabbableSymbol.BP_GrabbableSymbol_C|GetGrabComponent (Variables|Default|GetInputKeySymbol)) false)
      (Utilities|FlowControl|Delay 1.0)
      (CallFunction|CheckMatchingKey))))

(event Custom|Eject
  (bind _self self)
  (bind _self_2 self)
  (Utilities|IsValid (Variables|Default|GetInputKeySymbol)
    (:Is%20Valid
      (Class|Interactable|EndInteract 0)
      (Transformation|SetActorLocation (Variables|Default|GetInputKeySymbol) (+ (* (Transformation|GetActorForwardVector _self_2) -5e+01) (Transformation|GetWorldLocation (Variables|Default|GetDefaultSceneRoot _self_2))) false true)
      (Variables|/Game/Blueprints/Components/GrabComponent.GrabComponent_C|SetbSimulateOnDrop (Variables|/Game/Blueprints/Actors/Act3/BP_GrabbableSymbol.BP_GrabbableSymbol_C|GetGrabComponent (Variables|Default|GetInputKeySymbol)) true)
      (Physics|SetSimulatePhysics (Variables|/Game/Blueprints/Actors/BP_Symbol.BP_Symbol_C|GetFrame (Variables|Default|GetInputKeySymbol)) true)
      (Variables|/Game/Blueprints/Components/GrabComponent.GrabComponent_C|SetcanGrab (Variables|/Game/Blueprints/Actors/Act3/BP_GrabbableSymbol.BP_GrabbableSymbol_C|GetGrabComponent (Variables|Default|GetInputKeySymbol)) true)
      (Physics|SetPhysicsLinearVelocity (Variables|/Game/Blueprints/Actors/BP_Symbol.BP_Symbol_C|GetFrame (Variables|Default|GetInputKeySymbol)) (* (+ (Transformation|GetActorForwardVector _self) (* (Transformation|GetActorRightVector _self) (Math|Random|RandomFloatinRange -2.0 2.0))) -2e+02) false "None")
      (Variables|Default|SetInputKeySymbol 0))))

(event Custom|CheckMatchingKey
  (if (Utilities|Enum|Equal(Enum) (Variables|/Game/Blueprints/Actors/BP_Symbol.BP_Symbol_C|GetGlyph (Variables|Default|GetInputKeySymbol)) (Variables|/Game/Blueprints/Actors/Act2/Phase2/BP_HologramSymbol.BP_HologramSymbol_C|Getglyph (Variables|Default|GetAnswerKeySymbol)))
    (Class|Interactable|BeginInteract 0)
    (else
      (Default|CallOnFail))))

(event Custom|AllowLockInput
  (Actor|Tick|SetActorTickEnabled true)
  (Variables|Default|SetActivating true))

(event Custom|CloseLockInput
  (Actor|Tick|SetActorTickEnabled true)
  (Variables|Default|SetActivating false))

(event EventBeginPlay)

(event Collision|EventActorBeginOverlap
  (params (OtherActor :type Actor%20Object%20Reference)))

(event EventTick
  (params (DeltaSeconds :type Float%20%28single-precision%29))
  (bind _box (Variables|Default|GetBox))
  (bind _box_2 (Variables|Default|GetBox))
  (bind _progressiontime (Variables|Default|GetProgressionTime))
  (bind _returnvalue (/ DeltaSeconds _progressiontime))
  (if (Variables|Default|GetActivating)
    (if (> (+ (Variables|Default|GetLockcoverProgress) _returnvalue) 1.0)
      (Variables|Default|SetLockcoverProgress 1.0)
      (Variables|/Script/Engine.PrimitiveComponent|SetbGenerateOverlapEvents _box_2 true)
      (Actor|Tick|SetActorTickEnabled false)
      (else
        (Variables|Default|SetLockcoverProgress (+ (Variables|Default|GetLockcoverProgress) _returnvalue))
        (Variables|/Script/Engine.PrimitiveComponent|SetbGenerateOverlapEvents _box_2 false)))
    (elif (< (- (Variables|Default|GetLockcoverProgress) _returnvalue) 0.0)
      (Variables|Default|SetLockcoverProgress 0.0)
      (Variables|/Script/Engine.PrimitiveComponent|SetbGenerateOverlapEvents _box false)
      (Actor|Tick|SetActorTickEnabled false)
      (else
        (Variables|Default|SetLockcoverProgress (- (Variables|Default|GetLockcoverProgress) _returnvalue))
        (Variables|/Script/Engine.PrimitiveComponent|SetbGenerateOverlapEvents _box false)))))

(fn ConstructionScript)

(fn OnRepLockcoverProgress
  (Rendering|Material|SetScalarParameterValueonMaterials (Variables|Default|GetLockCover) "Dissolve" (+ (* (Math|Float|Sqrt (Variables|Default|GetLockcoverProgress)) 2.4) -0.8)))