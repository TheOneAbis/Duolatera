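; Electric beam emitter that fires a portal-aware laser and pushes physics objects it hits.
; Each tick it line-traces from the Electro component, storing impact point, portal state and beam points, with extra points when passing through a portal.
; RepNotifies feed those points to Niagara and set the ReceivePanel material's hit position and on state from portal pass-through.
; The replicated IsEmiterOn flag toggles both tick and effect.
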(event Custom|CalculateElectro
  (bind _electro (Variables|Default|GetElectro))
  (bind _electro_2 (Variables|Default|GetElectro))
  (bind _returnvalue (Math|Vector|GetForwardVector _electro_2))
  (bind _returnvalue_2 (* _returnvalue 1e+03))
  (bind (_outhit _outportalhit _tracedthroughportal _returnvalue_3) (Class|ExtraBlueprintFunctionLibrary|PortalLineTrace (Transformation|GetWorldLocation _electro) (Math|Vector|GetForwardVector _electro) 4e+03 "TraceTypeQuery1" false 0 "None" true "(R=1.000000,G=0.000000,B=0.000000,A=1.000000)" "(R=0.000000,G=1.000000,B=0.000000,A=1.000000)" 1.0))
  (if _returnvalue_3
    (Variables|Default|SetimpactPt (.ImpactPoint (Collision|BreakHitResult _outhit)))
    (Variables|Default|SetIsPortalOpen _tracedthroughportal)
    (Variables|Default|SetBeamPtsArray (select _tracedthroughportal (Utilities|Array|MakeArray (.TraceStart (Collision|BreakHitResult _outportalhit)) (.ImpactPoint (Collision|BreakHitResult _outportalhit)) (.TraceStart (Collision|BreakHitResult _outhit)) (.ImpactPoint (Collision|BreakHitResult _outhit))) (Utilities|Array|MakeArray (.TraceStart (Collision|BreakHitResult _outhit)) (.ImpactPoint (Collision|BreakHitResult _outhit)))))
    (if (Physics|IsSimulatingPhysics (.HitComponent (Collision|BreakHitResult _outhit)) "None")
      (Class|PrimitiveComponent|AddForceatLocation (.HitComponent (Collision|BreakHitResult _outhit)) _returnvalue_2 (.ImpactPoint (Collision|BreakHitResult _outhit)) "None")
      (Physics|AddImpulseatLocation (.HitComponent (Collision|BreakHitResult _outhit)) _returnvalue_2 (.ImpactPoint (Collision|BreakHitResult _outhit)) "None"))
    (else
      (Variables|Default|SetimpactPt "99999.000000,99999.000000,99999.000000")
      (Variables|Default|SetBeamPtsArray (select _tracedthroughportal (Utilities|Array|MakeArray (.TraceStart (Collision|BreakHitResult _outportalhit)) (.ImpactPoint (Collision|BreakHitResult _outportalhit)) (.TraceStart (Collision|BreakHitResult _outhit)) (.TraceEnd (Collision|BreakHitResult _outhit))) (Utilities|Array|MakeArray (.TraceStart (Collision|BreakHitResult _outhit)) (.TraceEnd (Collision|BreakHitResult _outhit))))))))

(event EventBeginPlay)

(event Collision|EventActorBeginOverlap
  (params (OtherActor :type Actor%20Object%20Reference)))

(event EventTick
  (params (DeltaSeconds :type Float%20%28single-precision%29))
  (CallFunction|CalculateElectro))

(fn ConstructionScript)

(fn OnRepImpactPt
  (if (Variables|Default|GetIsPortalOpen)
    (Rendering|Material|SetVectorParameterValueonMaterials (Variables|/Game/Blueprints/Actors/Act2/Phase2/BP_ElectroPanel.BP_ElectroPanel_C|GetPlane (Variables|Default|GetReceivePanel)) "HitPos" (Variables|Default|GetImpactPt))))

(fn OnRepBeamPtsArray
  (Class|NiagaraDataInterfaceArrayFunctionLibrary|SetNiagaraArrayVector (Variables|Default|GetElectro) "LaserPoints" (Variables|Default|GetBeamPtsArray)))

(fn OnRepIsPortalOpen
  (Rendering|Material|SetScalarParameterValueonMaterials (Variables|/Game/Blueprints/Actors/Act2/Phase2/BP_ElectroPanel.BP_ElectroPanel_C|GetPlane (Variables|Default|GetReceivePanel)) "IsOn" (Math|Conversions|ToFloat(Boolean) (Variables|Default|GetIsPortalOpen))))

(fn OnRepIsEmiteron
  (if (Variables|Default|GetIsEmiterOn)
    (Actor|Tick|SetActorTickEnabled true)
    (Components|Activation|SetActive (Variables|Default|GetElectro) true false)
    (else
      (Actor|Tick|SetActorTickEnabled false)
      (Components|Activation|SetActive (Variables|Default|GetElectro) false false))))