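; Replicated hologram symbol actor for Act 2 Phase 2 that shows one of four glyphs: Cycle, Life, Culture or Knowledge.
; The construction script applies a dynamic sprite material, then reassigns Glyph to itself to fire its RepNotify.
; OnRep_glyph swaps the Symbol component's sprite to match the glyph.
; BeginPlay hides the symbol, and nothing in this Blueprint reveals it again.
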(event EventBeginPlay
  (Rendering|SetVisibility (Variables|Default|GetSymbol) false false))

(event Collision|EventActorBeginOverlap
  (params (OtherActor :type Actor%20Object%20Reference)))

(event EventTick
  (params (DeltaSeconds :type Float%20%28single-precision%29)))

(fn ConstructionScript
  (bind _symbol (Variables|Default|GetSymbol))
  (bind _returnvalue (Rendering|Material|CreateDynamicMaterialInstance _symbol 0 "/Game/Assets/Materials/M_SymbolSprite.M_SymbolSprite" "MI_SymbolSprite" :!class /Script/Engine.PrimitiveComponent))
  (Rendering|Material|SetMaterial _symbol 0 _returnvalue)
  (Variables|Default|Setglyph (Variables|Default|Getglyph)))

(fn OnRepGlyph
  (bind _symbol (Variables|Default|GetSymbol))
  (switch Utilities|FlowControl|Switch|SwitchonGlyph (Variables|Default|Getglyph)
    (:NewEnumerator0
      (Rendering|Components|Sprite|SetSprite _symbol "/Game/Assets/png/SymbolGlyphs/Cycle_Sprite.Cycle_Sprite"))
    (:NewEnumerator1
      (Rendering|Components|Sprite|SetSprite _symbol "/Game/Assets/png/SymbolGlyphs/Life_Sprite.Life_Sprite"))
    (:NewEnumerator2
      (Rendering|Components|Sprite|SetSprite _symbol "/Game/Assets/png/SymbolGlyphs/Culture_Sprite.Culture_Sprite"))
    (:NewEnumerator3
      (Rendering|Components|Sprite|SetSprite _symbol "/Game/Assets/png/SymbolGlyphs/Knowledge_Sprite.Knowledge_Sprite"))))