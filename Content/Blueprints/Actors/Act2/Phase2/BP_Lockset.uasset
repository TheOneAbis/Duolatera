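; Lockset puzzle controller for Act 2 Phase 2 that coordinates a group of locks with a KeySet and reveals Phase 3 when completed.
; KeySet events open, close or eject the locks; any lock failure ejects all, blinks both holo planes red and reopens input.
; Activate blinks them green and sets replicated ShowPhase3, whose OnRep destroys listed objects and enables Tick to lower Act 3 portals and raise architecture before making portals portalable.
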(event Custom|ResetAllLock
  (CallFunction|EjectAllLocks)
  (for _array_element (Variables|Default|GetOverworldHoloPlane)
    (Default|BlinkRed _array_element))
  (for _array_element_2 (Variables|Default|GetUnderworldHoloPlane)
    (Default|BlinkRed _array_element_2))
  (CallFunction|AllowLocksetInput))

(event Custom|AllowLocksetInput
  (for _array_element (Variables|Default|GetLocks)
    (Default|AllowLockInput _array_element)))

(event Custom|CloseLocksetInput
  (for _array_element (Variables|Default|GetLocks)
    (Default|CloseLockInput _array_element)))

(event Custom|EjectAllLocks
  (for _array_element (Variables|Default|GetLocks)
    (Default|Eject _array_element)))

(event EventBeginPlay
  (bind _keyset (Variables|Default|GetKeySet))
  (for _array_element (Variables|Default|GetLocks)
    (EventDispatchers|BindEventtoOnFail _array_element (delegate Custom|ResetAllLock)))
  (EventDispatchers|BindEventtoAllowLockInput _keyset (delegate Custom|AllowLocksetInput))
  (EventDispatchers|BindEventtoCloseLockInput _keyset (delegate Custom|CloseLocksetInput))
  (EventDispatchers|BindEventtoEjectLockset _keyset (delegate Custom|EjectAllLocks))
  (CallFunction|CloseLocksetInput))

(event EventTick
  (params (DeltaSeconds :type Float%20%28single-precision%29))
  (Variables|Default|SetTimer (+ (Variables|Default|GetTimer) DeltaSeconds))
  (for _array_element (Variables|Default|GetAct3Portals)
    (Transformation|AddRelativeLocation (Variables|/Script/Engine.Actor|GetRootComponent _array_element) (Math|Vector|MakeVector 0.0 0.0 (* DeltaSeconds -115.0)) false true))
  (for _array_element_2 (Variables|Default|GetPhase3Architecture)
    (Transformation|AddRelativeLocation (Variables|/Script/Engine.Actor|GetRootComponent _array_element_2) (Math|Vector|MakeVector 0.0 0.0 (* DeltaSeconds 9e+01)) false true))
  (if (> (Variables|Default|GetTimer) 8.0)
    (for _array_element_3 (Variables|Default|GetAct3Portals)
      (Class|PortalCanvas|SetPortalable _array_element_3 true))
    (Actor|Tick|SetActorTickEnabled false)))

(event EventActivate
  (for _array_element (Variables|Default|GetOverworldHoloPlane)
    (Default|BlinkGreen _array_element))
  (for _array_element_2 (Variables|Default|GetUnderworldHoloPlane)
    (Default|BlinkGreen _array_element_2))
  (Variables|/Game/Blueprints/Actors/Act2/Phase2/BP_Keyset.BP_Keyset_C|SetIsPuzzleComplete (Variables|Default|GetKeySet) true)
  (Development|PrintString "phase2 complete ur gaming lets goooooooooooooooooooooo" true true "(R=1.000000,G=0.000000,B=0.800000,A=1.000000)" 2e+01)
  (Variables|Default|SetbShowPhase3 true))

(fn ConstructionScript)

(fn OnRepBShowPhase3
  (if (Variables|Default|GetbShowPhase3)
    (Actor|Tick|SetActorTickEnabled true)
    (for _array_element (Variables|Default|GetObjectsToDestroy)
      (Actor|DestroyActor _array_element))))