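; Keyset puzzle actor that shows and hides a randomized glyph sequence on holo symbols.
; A second after BeginPlay, the authority shuffles the over and under glyph pools and interleaves them across the symbols.
; Until the puzzle completes, Activate reveals symbols, lights both worlds' holo planes, powers electro emitters, ejects the lockset and closes lock input.
; Deactivate hides symbols, shuts emitters and their portals, and allows lock input.
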(event Custom|Shuffle
  (Networking|SwitchHasAuthority
    (:Authority
      (Utilities|Array|Shuffle (Variables|Default|GetGlyphsOver))
      (Utilities|Array|Shuffle (Variables|Default|GetGlyphsUnder))
      (for (_array_element _array_index) (Variables|Default|GetHoloSymbols)
        (Utilities|FlowControl|FlipFlop
          (:A
            (Variables|/Game/Blueprints/Actors/Act2/Phase2/BP_HologramSymbol.BP_HologramSymbol_C|Setglyph _array_element (Utilities|Array|Get(acopy) (Variables|Default|GetGlyphsUnder) (/ _array_index 2))))
          (:B
            (Variables|/Game/Blueprints/Actors/Act2/Phase2/BP_HologramSymbol.BP_HologramSymbol_C|Setglyph _array_element (Utilities|Array|Get(acopy) (Variables|Default|GetGlyphsOver) (/ _array_index 2)))))))))

(event Custom|Reset)

(event Custom|ShowSequence
  (for (_array_element _array_index) (Variables|Default|GetHoloSymbols)
    (Rendering|SetVisibility (Variables|/Game/Blueprints/Actors/Act2/Phase2/BP_HologramSymbol.BP_HologramSymbol_C|GetSymbol _array_element) true false)
    (Default|LightUp (Utilities|Array|Get(acopy) (Variables|Default|GetOverworldHoloPlane) _array_index))
    (Default|LightUp (Utilities|Array|Get(acopy) (Variables|Default|GetUnderworldHoloPlane) _array_index)))
  (Default|CallEjectLockset)
  (Default|CallCloseLockInput))

(event Custom|HideSequence
  (for (_array_element _array_index) (Variables|Default|GetHoloSymbols)
    (Rendering|SetVisibility (Variables|/Game/Blueprints/Actors/Act2/Phase2/BP_HologramSymbol.BP_HologramSymbol_C|GetSymbol _array_element) false false)
    (Utilities|FlowControl|FlipFlop
      (:A
        (Default|LightUp (Utilities|Array|Get(acopy) (Variables|Default|GetOverworldHoloPlane) _array_index)))
      (:B
        (Default|LightUp (Utilities|Array|Get(acopy) (Variables|Default|GetUnderworldHoloPlane) _array_index)))))
  (Default|CallAllowLockInput))

(event EventBeginPlay
  (Utilities|FlowControl|Delay 1.0)
  (CallFunction|Shuffle))

(event Collision|EventActorBeginOverlap
  (params (OtherActor :type Actor%20Object%20Reference)))

(event EventTick
  (params (DeltaSeconds :type Float%20%28single-precision%29)))

(event EventActivate
  (if (not (Variables|Default|GetIsPuzzleComplete))
    (CallFunction|ShowSequence)
    (for _array_element (Variables|Default|GetElectroEmitters)
      (Variables|/Game/Blueprints/Actors/Act2/Phase2/BP_ElectroEmitter.BP_ElectroEmitter_C|SetIsEmiterOn _array_element true))))

(event EventDeactivate
  (if (not (Variables|Default|GetIsPuzzleComplete))
    (CallFunction|HideSequence)
    (for _array_element (Variables|Default|GetElectroEmitters)
      (Variables|/Game/Blueprints/Actors/Act2/Phase2/BP_ElectroEmitter.BP_ElectroEmitter_C|SetIsEmiterOn _array_element false)
      (Variables|/Game/Blueprints/Actors/Act2/Phase2/BP_ElectroEmitter.BP_ElectroEmitter_C|SetIsPortalOpen _array_element false))))

(fn ConstructionScript)

(fn OnRepGlyphs)