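; Act 2 Phase 1 cannon that, on activation, plays a firing cutscene, locks the symbols in its activator slots and calls begin phase two.
; The timed sequence plays the cannon, fires charge and beam Niagara effects, breaks debris and launches a physics projectile, then cleans up.
; A portal-aware line trace pushes physics objects and sets replicated state, whose OnReps position the projectile, shape the beam and destroy debris.
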(event Custom|PlayCutScene
  (bind _projectile (Variables|Default|GetProjectile))
  (bind _ns_beam (Variables|Default|GetNS_Beam))
  (Development|PrintString "Cannon coming hahahahhaha" true true "(R=1.000000,G=0.000000,B=0.045352,A=1.000000)" 1e+01)
  (Audio|Components|Audio|Play (Variables|Default|GetCannon) false)
  (CallFunction|CalculateCannonBeam)
  (Utilities|FlowControl|Delay 3.0)
  (Components|Activation|Activate (Variables|Default|GetNS_Charge) false)
  (Utilities|FlowControl|Delay 3.8)
  (Components|Activation|Activate (Variables|Default|GetNS_Beam) false)
  (Default|EnableBreak (Variables|Default|GetDebris))
  (Physics|SetPhysicsLinearVelocity (Variables|Default|GetProjectile) (* (Math|Vector|GetForwardVector (Variables|Default|GetNS_Beam)) 2e+03) false "None")
  (Utilities|FlowControl|Delay 1.0)
  (Utilities|IsValid _projectile
    (:Is%20Valid
      (Components|DestroyComponent _projectile)
      (Utilities|FlowControl|Delay 2.0)
      (Components|Activation|Deactivate _ns_beam)
      (Rendering|SetVisibility _ns_beam false false)
      (Utilities|FlowControl|Delay 3.0)
      (Variables|Default|SetbDestroyDebris true))))

(event Custom|CalculateCannonBeam
  (bind _ns_beam (Variables|Default|GetNS_Beam))
  (bind _ns_beam_2 (Variables|Default|GetNS_Beam))
  (bind _returnvalue (Math|Vector|GetForwardVector _ns_beam))
  (bind _returnvalue_2 (* _returnvalue 1e+03))
  (bind (_outhit _outportalhit _tracedthroughportal _returnvalue_3) (Class|ExtraBlueprintFunctionLibrary|PortalLineTrace (Transformation|GetWorldLocation _ns_beam_2) (Math|Vector|GetForwardVector _ns_beam_2) 4e+03 "TraceTypeQuery1" false 0 "None" true "(R=1.000000,G=0.000000,B=0.000000,A=1.000000)" "(R=0.000000,G=1.000000,B=0.000000,A=1.000000)" 1.0))
  (if _returnvalue_3
    (Variables|Default|SetimpactPt (.ImpactPoint (Collision|BreakHitResult _outhit)))
    (Variables|Default|SetBeamPtsArray (select _tracedthroughportal (Utilities|Array|MakeArray (.TraceStart (Collision|BreakHitResult _outportalhit)) (.ImpactPoint (Collision|BreakHitResult _outportalhit)) (.TraceStart (Collision|BreakHitResult _outhit)) (.ImpactPoint (Collision|BreakHitResult _outhit))) (Utilities|Array|MakeArray (.TraceStart (Collision|BreakHitResult _outhit)) (.ImpactPoint (Collision|BreakHitResult _outhit)))))
    (if (Physics|IsSimulatingPhysics (.HitComponent (Collision|BreakHitResult _outhit)) "None")
      (Class|PrimitiveComponent|AddForceatLocation (.HitComponent (Collision|BreakHitResult _outhit)) _returnvalue_2 (.ImpactPoint (Collision|BreakHitResult _outhit)) "None")
      (Physics|AddImpulseatLocation (.HitComponent (Collision|BreakHitResult _outhit)) _returnvalue_2 (.ImpactPoint (Collision|BreakHitResult _outhit)) "None"))
    (else
      (Variables|Default|SetimpactPt "99999.000000,99999.000000,99999.000000")
      (Variables|Default|SetBeamPtsArray (select _tracedthroughportal (Utilities|Array|MakeArray (.TraceStart (Collision|BreakHitResult _outportalhit)) (.ImpactPoint (Collision|BreakHitResult _outportalhit)) (.TraceStart (Collision|BreakHitResult _outhit)) (.TraceEnd (Collision|BreakHitResult _outhit))) (Utilities|Array|MakeArray (.TraceStart (Collision|BreakHitResult _outhit)) (.TraceEnd (Collision|BreakHitResult _outhit))))))))

(event EventBeginPlay)

(event Collision|EventActorBeginOverlap
  (params (OtherActor :type Actor%20Object%20Reference)))

(event EventTick
  (params (DeltaSeconds :type Float%20%28single-precision%29)))

(event EventActivate
  (CallFunction|PlayCutScene)
  (for _array_element (Class|Activatable|GetActivatorList)
    (bind _asbp_slot (Utilities|Casting|CastToBP_Slot _array_element))
    (Variables|/Game/Blueprints/Components/GrabComponent.GrabComponent_C|SetcanGrab (Variables|/Game/Blueprints/Actors/Act3/BP_GrabbableSymbol.BP_GrabbableSymbol_C|GetGrabComponent (Variables|/Game/Blueprints/Actors/Act2/Phase1/BP_Slot.BP_Slot_C|GetGrabbableSymbol _asbp_slot)) false))
  (Default|CallBeginPhaseTwo))

(fn ConstructionScript)

(fn OnRepImpactPt
  (Transformation|SetWorldLocation (Variables|Default|GetProjectile) (- (Variables|Default|GetImpactPt) (* (Math|Vector|GetForwardVector (Variables|Default|GetNS_Beam)) 2e+02)) false false))

(fn OnRepBeamPtsArray
  (Class|NiagaraDataInterfaceArrayFunctionLibrary|SetNiagaraArrayVector (Variables|Default|GetNS_Beam) "LaserPoints" (Variables|Default|GetBeamPtsArray)))

(fn OnRepBDestroyDebris
  (bind _debris (Variables|Default|GetDebris))
  (if (Variables|Default|GetbDestroyDebris)
    (Utilities|FlowControl|Sequence
      (:then_0
        (Utilities|IsValid _debris
          (:Is%20Valid
            (Actor|DestroyActor _debris))))
      (:then_1
        (for _array_element (Variables|Default|GetObjectsToDestroy)
          (Utilities|IsValid _array_element
            (:Is%20Valid
              (Actor|DestroyActor _array_element))))))))

(fn OnRepObjectstoDestroy)

(fn OnRepDebris)