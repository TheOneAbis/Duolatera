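; BP_Slot is a VR puzzle slot that opens on activation and accepts a grabbable symbol to match against its activating BP_Symbol.
; Tick ramps SlotProgress, driving the cover's dissolve through OnRep, and enables box overlaps only when fully open.
; On authority, overlap releases and snaps the symbol, stops Tick and compares glyphs.
; Results set the symbol's state; matches register the slot as a Cannon activator until removal.
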(event OnComponentBeginOverlap(Box)
  (params (OverlappedComponent :type Primitive%20Component%20Object%20Reference) (OtherActor :type Actor%20Object%20Reference) (OtherComp :type Primitive%20Component%20Object%20Reference) (OtherBodyIndex :type Integer) (bFromSweep :type Boolean) (SweepResult :type Hit%20Result%20Structure%20%28by%20ref%29))
  (bind _box (Variables|Default|GetBox))
  (bind _returnvalue (Transformation|GetWorldTransform _box))
  ;[1 1 1] Check if Overlapping Actor is Grabbable Symbol, if yes, snap it on the slot, turn off tick so slot does not close
  (Networking|SwitchHasAuthority
    (:Authority
      (bind _asbp_grabbable_symbol (Utilities|Casting|CastToBP_GrabbableSymbol OtherActor))
      (if (not (Variables|Default|GetisInSlot))
        (Variables|Default|SetisInSlot true)
        (Variables|Default|SetGrabbableSymbol _asbp_grabbable_symbol)
        (bind _asvrpawn (Utilities|Casting|CastToVRPawn (Game|Player|GetPlayerPawn 0)))
        (Variables|/Game/Blueprints/Components/GrabComponent.GrabComponent_C|SetbSimulateOnDrop (Variables|/Game/Blueprints/Actors/Act3/BP_GrabbableSymbol.BP_GrabbableSymbol_C|GetGrabComponent (Variables|Default|GetGrabbableSymbol)) false)
        (Default|RPCServerTryRelease _asvrpawn (Variables|/Game/Blueprints/Actors/Act3/BP_GrabbableSymbol.BP_GrabbableSymbol_C|GetGrabComponent (Variables|Default|GetGrabbableSymbol)) false)
        (Utilities|FlowControl|Delay 0.2)
        (Transformation|SetActorLocationAndRotation (Variables|Default|GetGrabbableSymbol) (.location _returnvalue) (.rotation _returnvalue))
        (Actor|Tick|SetActorTickEnabled false)
        (CallFunction|CheckMatchingSymbols (Variables|Default|GetGrabbableSymbol))))))

(event OnComponentEndOverlap(Box)
  (params (OverlappedComponent :type Primitive%20Component%20Object%20Reference) (OtherActor :type Actor%20Object%20Reference) (OtherComp :type Primitive%20Component%20Object%20Reference) (OtherBodyIndex :type Integer))
  (Networking|SwitchHasAuthority
    (:Authority
      (bind _asbp_grabbable_symbol (Utilities|Casting|CastToBP_GrabbableSymbol OtherActor))
      (if (== _asbp_grabbable_symbol (Variables|Default|GetGrabbableSymbol))
        (if (Variables|Default|GetisInSlot)
          (Variables|Default|SetisInSlot false)
          (Variables|/Game/Blueprints/Components/GrabComponent.GrabComponent_C|SetbSimulateOnDrop (Variables|/Game/Blueprints/Actors/Act3/BP_GrabbableSymbol.BP_GrabbableSymbol_C|GetGrabComponent (Variables|Default|GetGrabbableSymbol)) true)
          (Actor|Tick|SetActorTickEnabled true)
          (Class|Activatable|SetRemainActive false)
          (Default|SetSymbolState (Variables|Default|GetSymbol) "NewEnumerator2")
          (CallFunction|UpdateFullfilledSlot false))))))

(event Custom|CheckMatchingSymbols
  (params (GrabbableSymbol :type BP%20Grabbable%20Symbol%20Object%20Reference))
  (bind _symbol (Variables|Default|GetSymbol))
  (if (Utilities|Enum|Equal(Enum) (Variables|/Game/Blueprints/Actors/BP_Symbol.BP_Symbol_C|GetGlyph GrabbableSymbol) (Variables|/Game/Blueprints/Actors/BP_Symbol.BP_Symbol_C|GetGlyph _symbol))
    (Class|Activatable|SetRemainActive true)
    (Default|SetSymbolState _symbol "NewEnumerator4")
    (CallFunction|UpdateFullfilledSlot true)
    (else
      (Class|Activatable|SetRemainActive true)
      (Default|SetSymbolState _symbol "NewEnumerator1"))))

(event Custom|UpdateFullfilledSlot
  (params (isfullfilled :type Boolean))
  (if (!= isfullfilled (Variables|Default|GetisFullfilled))
    (bind _output_get (Variables|Default|SetisFullfilled isfullfilled))
    (if _output_get
      (Class|Activatable|AddActivator (Variables|Default|GetCannon) self)
      (else
        (Class|Activatable|RemoveActivator (Variables|Default|GetCannon) self)))))

(event EventBeginPlay)

(event Collision|EventActorBeginOverlap
  (params (OtherActor :type Actor%20Object%20Reference)))

(event EventTick
  (params (DeltaSeconds :type Float%20%28single-precision%29))
  (bind _box (Variables|Default|GetBox))
  (bind _box_2 (Variables|Default|GetBox))
  (bind _progressiontime (Variables|Default|GetProgressionTime))
  (bind _returnvalue (/ DeltaSeconds _progressiontime))
  (if (Variables|Default|GetActivating)
    (if (> (+ (Variables|Default|GetSlotProgress) _returnvalue) 1.0)
      (Variables|Default|SetSlotProgress 1.0)
      (Variables|/Script/Engine.PrimitiveComponent|SetbGenerateOverlapEvents _box_2 true)
      (Actor|Tick|SetActorTickEnabled false)
      (else
        (Variables|Default|SetSlotProgress (+ (Variables|Default|GetSlotProgress) _returnvalue))
        (Variables|/Script/Engine.PrimitiveComponent|SetbGenerateOverlapEvents _box_2 false)))
    (elif (< (- (Variables|Default|GetSlotProgress) _returnvalue) 0.0)
      (Variables|Default|SetSlotProgress 0.0)
      (Variables|/Script/Engine.PrimitiveComponent|SetbGenerateOverlapEvents _box false)
      (Actor|Tick|SetActorTickEnabled false)
      (else
        (Variables|Default|SetSlotProgress (- (Variables|Default|GetSlotProgress) _returnvalue))
        (Variables|/Script/Engine.PrimitiveComponent|SetbGenerateOverlapEvents _box false)))))

(event EventActivate
  (Actor|Tick|SetActorTickEnabled true)
  (Variables|Default|SetActivating true)
  (bind _asbp_symbol (Utilities|Casting|CastToBP_Symbol (Utilities|Array|Get(acopy) (Class|Activatable|GetActivatorList))))
  (Variables|Default|SetSymbol _asbp_symbol))

(event EventDeactivate
  (Actor|Tick|SetActorTickEnabled true)
  (Variables|Default|SetActivating false))

(fn ConstructionScript)

(fn OnRepSlotProgress
  (Rendering|Material|SetScalarParameterValueonMaterials (Variables|Default|GetSlotCover) "Dissolve" (+ (* (Math|Float|Sqrt (Variables|Default|GetSlotProgress)) 2.4) -0.8)))

(fn OnRepSlotFilled)

(fn OnRepActivating)

(fn OnRepIsFullfilled)

(fn OnRepIsinSlot)

(fn OnRepSymbol)

(fn OnRepActivated)