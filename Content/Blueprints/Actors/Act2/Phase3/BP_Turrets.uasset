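; Turret actor that, once activated, plays its animation, then fires a Niagara laser while rotating for just over one full turn before shutting off.
; Each tick it runs a portal-aware line trace along the beam, pushing physics objects and, on authority, sending a tagged message to the hit actor.
; The trace builds the beam points, including the extra portal segment, which the ImpactPt RepNotify feeds into the Niagara array.
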(event Custom|TurretAnimation
  (Audio|Components|Audio|Play (Variables|Default|GetTurret) false)
  (Utilities|FlowControl|Delay 3.0)
  (Components|Activation|Activate (Variables|Default|GetNS_Beam) false))

(event Custom|CalculateTurretBeam
  (bind _ns_beam (Variables|Default|GetNS_Beam))
  (bind (_outhit _outportalhit _tracedthroughportal _returnvalue) (Class|ExtraBlueprintFunctionLibrary|PortalLineTrace (Transformation|GetWorldLocation _ns_beam) (Math|Vector|GetForwardVector _ns_beam) 4e+03 "TraceTypeQuery1" false 0 "None" true "(R=1.000000,G=0.000000,B=0.000000,A=1.000000)" "(R=0.000000,G=1.000000,B=0.000000,A=1.000000)" 1.0))
  (if _returnvalue
    (Variables|Default|SetimpactPt (.ImpactPoint (Collision|BreakHitResult _outhit)))
    (Variables|Default|SetBeamPtsArray (select _tracedthroughportal (Utilities|Array|MakeArray (.TraceStart (Collision|BreakHitResult _outportalhit)) (.ImpactPoint (Collision|BreakHitResult _outportalhit)) (.TraceStart (Collision|BreakHitResult _outhit)) (.ImpactPoint (Collision|BreakHitResult _outhit))) (Utilities|Array|MakeArray (.TraceStart (Collision|BreakHitResult _outhit)) (.ImpactPoint (Collision|BreakHitResult _outhit)))))
    (if (Physics|IsSimulatingPhysics (.HitComponent (Collision|BreakHitResult _outhit)) "None")
      (Class|PrimitiveComponent|AddForceatLocation (.HitComponent (Collision|BreakHitResult _outhit)) (* (Math|Vector|GetForwardVector (Variables|Default|GetNS_Beam)) 1e+03) (.ImpactPoint (Collision|BreakHitResult _outhit)) "None"))
    (Networking|SwitchHasAuthority
      (:Authority
        (Class|Taggable|OnTagged(Message) (.HitActor (Collision|BreakHitResult _outhit)) _outhit self)))
    (else
      (Variables|Default|SetimpactPt "99999.000000,99999.000000,99999.000000")
      (Variables|Default|SetBeamPtsArray (select _tracedthroughportal (Utilities|Array|MakeArray (.TraceStart (Collision|BreakHitResult _outportalhit)) (.ImpactPoint (Collision|BreakHitResult _outportalhit)) (.TraceStart (Collision|BreakHitResult _outhit)) (.TraceEnd (Collision|BreakHitResult _outhit))) (Utilities|Array|MakeArray (.TraceStart (Collision|BreakHitResult _outhit)) (.TraceEnd (Collision|BreakHitResult _outhit))))))))

(event EventBeginPlay)

(event Collision|EventActorBeginOverlap
  (params (OtherActor :type Actor%20Object%20Reference)))

(event EventTick
  (params (DeltaSeconds :type Float%20%28single-precision%29))
  (bind _returnvalue (* DeltaSeconds 6e+01))
  (bind _ns_beam (Variables|Default|GetNS_Beam))
  (Variables|Default|SetTotalDegree (+ _returnvalue (Variables|Default|GetTotalDegree)))
  (Transformation|AddWorldRotation (Variables|Default|GetSphere) (Math|Rotator|MakeRotator _returnvalue 0.0 0.0) false false)
  (CallFunction|CalculateTurretBeam)
  (if (> (Variables|Default|GetTotalDegree) 375.0)
    (Components|Activation|Deactivate _ns_beam)
    (Rendering|SetVisibility _ns_beam false false)
    (Actor|Tick|SetActorTickEnabled false)))

(event EventActivate
  (CallFunction|TurretAnimation)
  (Utilities|FlowControl|Delay 3.0)
  (Actor|Tick|SetActorTickEnabled true))

(fn ConstructionScript)

(fn OnRepImpactPt
  (Class|NiagaraDataInterfaceArrayFunctionLibrary|SetNiagaraArrayVector (Variables|Default|GetNS_Beam) "LaserPoints" (Variables|Default|GetBeamPtsArray)))

(fn OnRepBeamPtsArray)

(fn OnRepHit)