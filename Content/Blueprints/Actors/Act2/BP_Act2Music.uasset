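; Networked music actor for Act 2 that layers an adaptive soundtrack as puzzles progress.
; The server binds to portal, symbol, lock, keyset and final button events to update replicated Track and Act2Progress, with lock release or eject resetting progress to a midpoint.
; OnRep functions turn both values into audio parameters for track selection, layer gains and crossfades.
; Drawing the portal starts the music, a delay advances it, and the final button completes it.
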(event Custom|OnInteractBegin_Event
  (params (interactedActor :type Interactable%20Object%20Reference))
  (Variables|Default|SetAct2Progress (+ (Variables|Default|GetAct2Progress) 1)))

(event Custom|OnPortalDrawn_Event
  (params (newCanvas :type Portal%20Canvas%20Object%20Reference))
  (EventDispatchers|UnbindEventfromOnPortalDrawn (Variables|Default|GetGiantPortal) (delegate Custom|OnPortalDrawn_Event))
  (Variables|Default|SetTrack 1.0)
  (Utilities|FlowControl|Delay 51.0)
  (Variables|Default|SetTrack 2.0))

(event Custom|CompleteMusic
  (params (interactedActor :type Interactable%20Object%20Reference))
  (Variables|Default|SetTrack 3.0))

(event Custom|SymbolStateChanged
  (params (Old%20State :type SymbolState%20Enum :default "NewEnumerator0") (New%20State :type SymbolState%20Enum :default "NewEnumerator0") (ChangedSymbol :type BP%20Symbol%20Object%20Reference))
  (if (Utilities|Enum|Equal(Enum) New%20State "NewEnumerator4")
    (Variables|Default|SetAct2Progress (+ (Variables|Default|GetAct2Progress) 1))
    (elif (Utilities|Enum|Equal(Enum) Old%20State "NewEnumerator4")
      (Variables|Default|SetAct2Progress (- (Variables|Default|GetAct2Progress) 1)))))

(event Custom|EjectLockset_Event
  (Variables|Default|SetAct2Progress 4))

(event Custom|OnInteractEnd_Event
  (params (interactedActor :type Interactable%20Object%20Reference))
  (Variables|Default|SetAct2Progress 4))

(event EventBeginPlay
  (Networking|SwitchHasAuthority
    (:Authority
      (EventDispatchers|AssignOnPortalDrawn (Variables|Default|GetGiantPortal) (delegate Custom|OnPortalDrawn_Event))
      (for _array_element (Variables|Default|GetPhase1Symbols)
        (EventDispatchers|BindEventtoOnSymbolStateChanged _array_element (delegate Custom|SymbolStateChanged)))
      (for _array_element_2 (Variables|Default|GetPhase2Locks)
        (EventDispatchers|AssignOnInteractBegin _array_element_2 (delegate Custom|OnInteractBegin_Event))
        (EventDispatchers|BindEventtoOnInteractEnd _array_element_2 (delegate Custom|OnInteractEnd_Event)))
      (EventDispatchers|AssignEjectLockset (Variables|Default|Getkeyset) (delegate Custom|EjectLockset_Event))
      (EventDispatchers|AssignOnInteractBegin (Variables|Default|GetfinalButton) (delegate Custom|CompleteMusic)))))

(fn ConstructionScript)

(fn OnRepTrack
  (Audio|Parameter|SetFloatParameter (Variables|Default|GetAudioComponent) "Track" (Variables|Default|GetTrack) :!class /Script/Engine.AudioComponent))

(fn OnRepAct2Progress
  (bind _audiocomponent (Variables|Default|GetAudioComponent))
  (bind _audiocomponent_2 (Variables|Default|GetAudioComponent))
  (bind _act2progress (Variables|Default|GetAct2Progress))
  (for _index (range 0 _act2progress)
    (switch int _act2progress
      (:0
        (Audio|Parameter|SetFloatParameter _audiocomponent "L2Gain" 0.0 :!class /Script/Engine.AudioComponent))
      (:1
        (Audio|Parameter|SetFloatParameter _audiocomponent "L2Gain" 1.0 :!class /Script/Engine.AudioComponent)
        (Audio|Parameter|SetFloatParameter _audiocomponent "L3Gain" 0.0 :!class /Script/Engine.AudioComponent))
      (:2
        (Audio|Parameter|SetFloatParameter _audiocomponent "L3Gain" 1.0 :!class /Script/Engine.AudioComponent)
        (Audio|Parameter|SetFloatParameter _audiocomponent "L4Gain" 0.0 :!class /Script/Engine.AudioComponent))
      (:3
        (Audio|Parameter|SetFloatParameter _audiocomponent "L4Gain" 1.0 :!class /Script/Engine.AudioComponent)
        (Audio|Parameter|SetFloatParameter _audiocomponent "L5Gain" 0.0 :!class /Script/Engine.AudioComponent))
      (:4
        (Audio|Parameter|SetFloatParameter _audiocomponent_2 "L5Gain" 1.0 :!class /Script/Engine.AudioComponent :!label _label)
        (Audio|Parameter|SetFloatParameter _audiocomponent_2 "L1Crossfade" 0.0 :!class /Script/Engine.AudioComponent)
        (Audio|Parameter|SetFloatParameter _audiocomponent_2 "L6Gain" 0.0 :!class /Script/Engine.AudioComponent)
        (Audio|Parameter|SetFloatParameter _audiocomponent_2 "L5Crossfade" 0.0 :!class /Script/Engine.AudioComponent)
        (Audio|Parameter|SetFloatParameter _audiocomponent_2 "L7Gain" 0.0 :!class /Script/Engine.AudioComponent))
      (:5
        (goto _label))
      (:6
        (Audio|Parameter|SetFloatParameter _audiocomponent_2 "L1Crossfade" 1.0 :!class /Script/Engine.AudioComponent :!label _label_2))
      (:7
        (goto _label_2))
      (:8
        (Audio|Parameter|SetFloatParameter _audiocomponent_2 "L6Gain" 1.0 :!class /Script/Engine.AudioComponent :!label _label_3))
      (:9
        (goto _label_3))
      (:10
        (Audio|Parameter|SetFloatParameter _audiocomponent_2 "L5Crossfade" 1.0 :!class /Script/Engine.AudioComponent :!label _label_4))
      (:11
        (goto _label_4))
      (:12
        (Audio|Parameter|SetFloatParameter _audiocomponent_2 "L7Gain" 1.0 :!class /Script/Engine.AudioComponent)))))