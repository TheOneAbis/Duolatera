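; Checker piece actor that caches the BP_GridManager on BeginPlay and responds to constrained grabs.
; On grab it clears its current node and sets the Checker's relative Y once from the grabbing component's position in grid-origin space, clamped between zero and Offset.
; Release does nothing.
; Logic for snapping to a free adjacent node and a nearest-node debug print are present but disconnected.
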(event EventBeginPlay
  (bind _returnvalue (Actor|GetActorOfClass "/Game/Blueprints/Actors/BP_GridManager.BP_GridManager_C"))
  (Variables|Default|SetGridManager _returnvalue))

(event Collision|EventActorBeginOverlap
  (params (OtherActor :type Actor%20Object%20Reference)))

(event EventTick
  (params (DeltaSeconds :type Float%20%28single-precision%29)))

(event EventOnConstrainedGrabbed
  (params (grabbingCompRef :type Transform))
  (bind _checker (Variables|Default|GetChecker))
  (bind _relativelocation (Variables|/Script/Engine.SceneComponent|GetRelativeLocation _checker))
  (Variables|Default|SetGrabbing%20Comp%20Ref grabbingCompRef)
  (Variables|Default|SetCurrentGridNode 0)
  (Transformation|SetRelativeLocation _checker (Math|Vector|MakeVector (.x _relativelocation) (Math|Float|Clamp(Float) (.y (Math|Transform|InverseTransformLocation (Variables|/Game/Blueprints/Actors/BP_GridManager.BP_GridManager_C|GetGridOrigin (Variables|Default|GetGridManager)) (.location (Variables|Default|GetGrabbing%20Comp%20Ref)))) 0.0 (Variables|Default|GetOffset)) (.z _relativelocation)) false false))

(event EventOnConstrainedReleased)

(fn ConstructionScript)