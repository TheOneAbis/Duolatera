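; Replicated symbol actor that players activate by shooting it while its state allows tagging.
; OnTagged wakes a server-intended Tick that fills ActivationAmt, then latches or requires constant fire, resetting when hits stop.
; SetSymbolState fires interact and state-change calls, while RepNotifies drive frame, glyph, aura and opacity visuals, with timelines for fade, flash and highlight.
; Construction and BeginPlay reassign variables to themselves to trigger those RepNotifies.
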(event Custom|Highlight%20%28Multicast%29
  (bind _highlightsprite (Variables|Default|GetHighlightSprite))
  (bind _spritecolor (Variables|/Script/Paper2D.PaperSpriteComponent|GetSpriteColor _highlightsprite))
  (Rendering|SetVisibility (Variables|Default|GetHighlightSprite) true false)
  (bind _alpha (Timeline|HighlightTimeline PlayFromStart)
    (:Update
      (Sprite|SetSpriteColor _highlightsprite (Utilities|Struct|MakeLinearColor (.r _spritecolor) (.g _spritecolor) (.b _spritecolor) _alpha)))
    (:Finished
      (Rendering|SetVisibility _highlightsprite false false))))

(event Custom|Highlight
  (bind _highlightsprite (Variables|Default|GetHighlightSprite))
  (bind _spritecolor (Variables|/Script/Paper2D.PaperSpriteComponent|GetSpriteColor _highlightsprite))
  (Rendering|SetVisibility (Variables|Default|GetHighlightSprite) true false)
  (bind _alpha (Timeline|HighlightTimeline PlayFromStart)
    (:Update
      (Sprite|SetSpriteColor _highlightsprite (Utilities|Struct|MakeLinearColor (.r _spritecolor) (.g _spritecolor) (.b _spritecolor) _alpha)))
    (:Finished
      (Rendering|SetVisibility _highlightsprite false false))))

(event Custom|Flash
  (bind _state (Variables|Symbol|GetState))
  (bind _auramat (Variables|Default|GetauraMat))
  (bind _returnvalue (Math|Conversions|ToInteger(Byte) _state))
  (bind (_direction _radius _intensity) (Timeline|FlashTimeline PlayFromStart)
    (:Update
      (Rendering|Material|SetScalarParameterValue _auramat "Radius" _radius :!class /Script/Engine.MaterialInstanceDynamic)
      (Rendering|Material|SetScalarParameterValue _auramat "AuraIntensity" _intensity :!class /Script/Engine.MaterialInstanceDynamic))
    (:Finished
      (Rendering|Material|SetScalarParameterValue _auramat "Radius" 0.18 :!class /Script/Engine.MaterialInstanceDynamic)
      (Rendering|Material|SetScalarParameterValue _auramat "AuraIntensity" (Math|Float|SelectFloat 2e+01 0.0 (and (> _returnvalue 1) (< _returnvalue 4))) :!class /Script/Engine.MaterialInstanceDynamic))))

(event Custom|Fade%20Symbol
  (params (Fade%20in :type Boolean))
  (if Fade%20in
    (bind _alpha (Timeline|Symbol%20Fade%20In Play)
      (:Update
        (Rendering|Material|SetScalarParameterValue (Variables|Default|GetsymbolMat) "SymbolOpacity" _alpha :!class /Script/Engine.MaterialInstanceDynamic)))
    (else
      (Timeline|Symbol%20Fade%20In Reverse))))

(event EventBeginPlay
  (Variables|Symbol|SetState (Variables|Symbol|GetState)))

(event EventTick
  (params (DeltaSeconds :type Float%20%28single-precision%29))
  ;[1 1 1] Ticking should only happen on server
  (if (Variables|Default|GettaggedLastFrame)
    (Variables|Default|SettaggedLastFrame false)
    (Variables|Default|SetactivationAmt (Math|Float|Min(Float) (+ (Variables|Default|GetactivationAmt) (* DeltaSeconds 2.0)) 1.0))
    (if (== (Variables|Default|GetactivationAmt) 1.0)
      (CallFunction|SetSymbolState (select (Variables|Symbol|GetRequire%20Constant%20Activation) "NewEnumerator3" "NewEnumerator4")))
    (else
      ;;[1 0.4746 0.3646] Player stopped shooting; go back to state 2
      (Actor|Tick|SetActorTickEnabled false)
      (Variables|Default|SetactivationAmt 0.0)
      (if (== (Variables|Symbol|GetState) 3)
        (CallFunction|SetSymbolState "NewEnumerator2")))))

(event EventOnTagged
  (params (tagHit :type Hit%20Result%20Structure) (tagSource :type Actor%20Object%20Reference))
  (bind _state (Variables|Symbol|GetState))
  (if (or (== _state 2) (== _state 3))
    (Variables|Default|SettaggedLastFrame true)
    (if (not (Class|Actor|IsActorTickEnabled))
      (Actor|Tick|SetActorTickEnabled true))))

(fn ConstructionScript
  (bind _returnvalue (Rendering|Material|CreateDynamicMaterialInstance (Variables|Default|GetAura) 0 "/Game/Assets/Materials/M_Aura.M_Aura" "MI_SymbolAura" :!class /Script/Engine.PrimitiveComponent))
  (Variables|Default|SetauraMat _returnvalue)
  (bind _returnvalue_2 (Rendering|Material|CreateDynamicMaterialInstance (Variables|Default|GetSymbolSprite) 0 "/Game/Assets/Materials/M_SymbolSprite.M_SymbolSprite" "MI_SymbolSprite" :!class /Script/Engine.PrimitiveComponent))
  (bind _output_get (Variables|Default|SetsymbolMat _returnvalue_2))
  (Variables|Symbol|SetSymbol%20Type (Variables|Symbol|GetSymbol%20Type))
  (Variables|Symbol|SetGlyph (Variables|Symbol|GetGlyph))
  (Rendering|Material|SetScalarParameterValue _output_get "SymbolOpacity" (Math|Float|SelectFloat 0.0 1.0 (Utilities|Enum|Equal(Enum) (Variables|Symbol|GetState) "NewEnumerator0")) :!class /Script/Engine.MaterialInstanceDynamic))

(fn OnRepActivationAmt
  (Rendering|Material|SetScalarParameterValue (Variables|Default|GetsymbolMat) "SymbolIntensity" (Math|Float|SelectFloat (Math|Float|Lerp (Variables|Default|GetdimIntensity) 1.0 (Variables|Default|GetactivationAmt)) 1e+01 (< (Variables|Symbol|GetState) 3)) :!class /Script/Engine.MaterialInstanceDynamic)
  (Rendering|Material|SetScalarParameterValue (Variables|Default|GetauraMat) "ActivationAmt" (Variables|Default|GetactivationAmt) :!class /Script/Engine.MaterialInstanceDynamic))

(fn OnRepState
  (bind _state (Variables|Symbol|GetState))
  (bind _state_2 (Variables|Symbol|GetState))
  (bind _returnvalue (Math|Conversions|ToInteger(Byte) _state))
  (bind _returnvalue_2 (> _returnvalue 1))
  (bind _returnvalue_3 (< _returnvalue 4))
  (bind _returnvalue_4 (and _returnvalue_2 _returnvalue_3))
  (Rendering|Material|SetScalarParameterValue (Variables|Default|GetauraMat) "AuraIntensity" (Math|Float|SelectFloat 25.0 0.0 _returnvalue_4) :!class /Script/Engine.MaterialInstanceDynamic)
  (Rendering|Material|SetScalarParameterValue (Variables|Default|GetsymbolMat) "SymbolIntensity" (Math|Float|SelectFloat 1e+01 (Variables|Default|GetdimIntensity) (> _returnvalue 2)) :!class /Script/Engine.MaterialInstanceDynamic)
  (Rendering|Material|SetScalarParameterValueonMaterials (Variables|Default|GetFrame) "IsTaggable" (Math|Conversions|ToFloat(Boolean) _returnvalue_4))
  (Utilities|FlowControl|Sequence
    (:then_0
      (if (and (> (Variables|Symbol|GetState) 0) (== (Variables|Default|GetLastState) 0))
        (CallFunction|FadeSymbol true)
        (elif (and (== (Variables|Symbol|GetState) 0) (> (Variables|Default|GetLastState) 0))
          (CallFunction|FadeSymbol false))))
    (:then_1
      (if (Utilities|Enum|Equal(Enum) _state_2 "NewEnumerator4")
        (CallFunction|Flash)))
    (:then_2
      (Variables|Default|SetLastState _state_2))))

(fn OnRepSymbolType
  (bind _frame (Variables|Default|GetFrame))
  (bind _frame_2 (Variables|Default|GetFrame))
  (switch Utilities|FlowControl|Switch|SwitchonSymbolType (Variables|Symbol|GetSymbol%20Type)
    (:NewEnumerator0
      (Components|StaticMesh|SetStaticMesh _frame_2 "/Game/Assets/Models/SymbolFrames/SymbolFrame_Circular.SymbolFrame_Circular")
      (Rendering|Material|SetMaterial _frame_2 0 "/Game/Assets/Materials/MaterialInstance/PropMI/MI_Cel_CircleSymbol.MI_Cel_CircleSymbol")
      (Rendering|Material|SetMaterial _frame_2 1 "/Game/Assets/Materials/MaterialInstance/PropMI/MI_Cel_CircleSymbol_Inner.MI_Cel_CircleSymbol_Inner"))
    (:NewEnumerator1
      (Components|StaticMesh|SetStaticMesh _frame "/Game/Assets/Models/SymbolFrames/SymbolFrame_Triangular.SymbolFrame_Triangular")
      (Rendering|Material|SetMaterial _frame 0 "/Game/Assets/Materials/MaterialInstance/PropMI/MI_Cel_Gate_Blue.MI_Cel_Gate_Blue")
      (Rendering|Material|SetMaterial _frame 1 "/Game/Assets/Materials/MaterialInstance/MI_Cel_Sector.MI_Cel_Sector"))))

(fn OnRepGlyph
  (bind _symbolsprite (Variables|Default|GetSymbolSprite))
  (switch Utilities|FlowControl|Switch|SwitchonGlyph (Variables|Symbol|GetGlyph)
    (:NewEnumerator0
      (Rendering|Components|Sprite|SetSprite _symbolsprite "/Game/Assets/png/SymbolGlyphs/Cycle_Sprite.Cycle_Sprite"))
    (:NewEnumerator1
      (Rendering|Components|Sprite|SetSprite _symbolsprite "/Game/Assets/png/SymbolGlyphs/Life_Sprite.Life_Sprite"))
    (:NewEnumerator2
      (Rendering|Components|Sprite|SetSprite _symbolsprite "/Game/Assets/png/SymbolGlyphs/Culture_Sprite.Culture_Sprite"))
    (:NewEnumerator3
      (Rendering|Components|Sprite|SetSprite _symbolsprite "/Game/Assets/png/SymbolGlyphs/Knowledge_Sprite.Knowledge_Sprite"))))

(fn SetSymbolState
  (params (New%20State :type SymbolState%20Enum :default "NewEnumerator0"))
  (if (Utilities|Enum|NotEqual(Enum) (Variables|Symbol|GetState) New%20State)
    (LocalVariables|SetoldState (Variables|Symbol|GetState))
    (Variables|Symbol|SetState New%20State)
    (if (and (<= (LocalVariables|GetoldState) 2) (> New%20State 2))
      (Class|Interactable|BeginInteract 0)
      (elif (and (> (LocalVariables|GetoldState) 2) (<= New%20State 2))
        (Variables|Default|SetactivationAmt 0.0)
        (Class|Interactable|EndInteract 0)))
    (if (Utilities|Enum|Equal(Enum) (Variables|Symbol|GetState) "NewEnumerator4")
      (Actor|Tick|SetActorTickEnabled false))
    (Default|CallOnSymbolStateChanged (LocalVariables|GetoldState) (Variables|Symbol|GetState) self)))