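; Replicated VR laser pistol owned by one of two players, with material and grab restriction set by player ID.
; Trigger input enables Tick, which traces through portals, pushes physics objects and sends server-side tagged hit messages.
; RepNotifies drive beam points, sound and firing state.
; Overlapping underworld regions disables firing with spark and fizzle feedback; dropped tools snap or timeline-sweep back to the owner's chest holster.
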(event OnGrabbed(GrabComponentSnap)
  (Components|Activation|SetActive (Variables|Default|GetNS_LaserBeam) false false)
  (Class|PlayerController|StopHapticEffect (Game|GetPlayerController 0) (Default|GetHeldbyHand (Variables|Default|GetGrabComponentSnap)))
  (Audio|Components|Audio|Stop (Variables|Default|GetCue_LaserFireLoop))
  (Actor|Tick|SetActorTickEnabled false)
  (CallFunction|ServerSetFiring false))

(event OnDropped(GrabComponentSnap)
  (Components|Activation|SetActive (Variables|Default|GetNS_LaserBeam) false false)
  (Class|PlayerController|StopHapticEffect (Game|GetPlayerController 0) (Default|GetHeldbyHand (Variables|Default|GetGrabComponentSnap)))
  (Audio|Components|Audio|Stop (Variables|Default|GetCue_LaserFireLoop))
  (Actor|Tick|SetActorTickEnabled false)
  (CallFunction|ServerSetFiring false))

(event OnComponentBeginOverlap(SkeletalMeshGun)
  (params (OverlappedComponent :type Primitive%20Component%20Object%20Reference) (OtherActor :type Actor%20Object%20Reference) (OtherComp :type Primitive%20Component%20Object%20Reference) (OtherBodyIndex :type Integer) (bFromSweep :type Boolean) (SweepResult :type Hit%20Result%20Structure%20%28by%20ref%29))
  ;[1 0.4734 0.2717] Set laser fireable or not whether it enters or leaves the underworld
  (if (Components|ComponentHasTag OtherComp "UnderworldRegion")
    (Variables|Default|Setfireable false)
    (Components|Activation|SetActive (Variables|Default|GetNS_Spark_Lasertool) true false)))

(event OnComponentEndOverlap(SkeletalMeshGun)
  (params (OverlappedComponent :type Primitive%20Component%20Object%20Reference) (OtherActor :type Actor%20Object%20Reference) (OtherComp :type Primitive%20Component%20Object%20Reference) (OtherBodyIndex :type Integer))
  ;[1 0.4734 0.2717] Set laser fireable or not whether it enters or leaves the underworld
  (if (Components|ComponentHasTag OtherComp "UnderworldRegion")
    (Variables|Default|Setfireable true)
    (Components|Activation|Deactivate (Variables|Default|GetNS_Spark_Lasertool))
    (Components|Activation|Deactivate (Variables|Default|GetNS_Smoke_Lasertool))
    (Components|Activation|Deactivate (Variables|Default|GetNS_Smoke_Lasertool1))))

(event Custom|server%20set%20drawing%20id
  (Variables|Default|SetDrawingID (+ (Variables|Default|GetDrawingID) 1)))

(event Custom|OnPlayerLogoutDelegate_Event
  (Development|PrintString "Player Logout" true true "(R=0.000000,G=0.660000,B=1.000000,A=1.000000)" 1e+01)
  (Utilities|IsValid (Variables|Default|GetplayerReference)
    (:Is%20Not%20Valid
      (Actor|DestroyActor))))

(event Custom|OnLaserToolDropped
  (bind _skeletalmeshgun (Variables|Default|GetSkeletalMeshGun))
  ;[1 1 1] Holster Stuff
  (Utilities|IsValid (Variables|Default|GetplayerReference)
    (:Is%20Valid
      (if (<= (Math|Vector|VectorLength (- (Transformation|GetSocketLocation (Variables|/Game/Blueprints/Actors/VRPawn.VRPawn_C|GetPlayerSkeletalMesh (Variables|Default|GetplayerReference)) "ChestSocket") (Transformation|GetWorldLocation (Variables|Default|GetGrabComponentSnap)))) (Variables|Default|GetsnapHolsterRadius)) ; check within range
        (CallFunction|AttachtoHolster :!label _label)
        (else
          (Timeline|AutoSnapCooldown PlayFromStart
            (:Finished
              (bind _isheld (Default|CheckifHeld (Variables|Default|GetGrabComponentSnap)))
              (if (not _isheld)
                (Default|SetPrimitiveCompPhysics (Variables|Default|GetGrabComponentSnap) false)
                (Utilities|FlowControl|Sequence
                  (:then_0
                    ;;[1 1 1] set location & rotation for lerp
                    (Variables|Default|SettempWorldLocation (Transformation|GetWorldLocation (Variables|Default|GetSkeletalMeshGun))))
                  (:then_1
                    (Variables|Default|SettempWorldRotation (Transformation|GetWorldRotation (Variables|Default|GetSkeletalMeshGun))))
                  (:then_2
                    (bind _sweep (Timeline|SweepToHolster PlayFromStart)
                      (:Update
                        (bind _isheld_2 (Default|CheckifHeld (Variables|Default|GetGrabComponentSnap)))
                        (if _isheld_2
                          (Timeline|SweepToHolster Stop)
                          (else
                            (Utilities|FlowControl|Sequence
                              (:then_0
                                (Transformation|SetWorldLocation _skeletalmeshgun (Math|Vector|Lerp(Vector) (Variables|Default|GettempWorldLocation) (Transformation|GetSocketLocation (Variables|/Game/Blueprints/Actors/VRPawn.VRPawn_C|GetPlayerSkeletalMesh (Variables|Default|GetplayerReference)) "ChestSocket") _sweep) false true))
                              (:then_1
                                (Transformation|SetWorldRotation _skeletalmeshgun (Class|KismetMathLibrary|QuatRotator (Class|KismetMathLibrary|QuatSlerp (Math|Conversions|ToQuaternion(Rotator) (Variables|Default|GettempWorldRotation)) (Math|Conversions|ToQuaternion(Rotator) (Transformation|GetSocketRotation (Variables|/Game/Blueprints/Actors/VRPawn.VRPawn_C|GetPlayerSkeletalMesh (Variables|Default|GetplayerReference)) "ChestSocket")) _sweep)) false true))))))
                      (:Finished
                        (goto _label)))))))))))
    (:Is%20Not%20Valid
      (Development|PrintString "Error: This pistol could't find its lover" true true "(R=0.000000,G=0.660000,B=1.000000,A=1.000000)" 2e+01))))

(event Custom|PlaySmokeVFX
  ;[0.7838 1 0.4879] Begin firing the laser if it's fireable. If not, just play the fizzle sound.
  (Components|Activation|SetActive (Variables|Default|GetNS_Smoke_Lasertool) true true)
  (Components|Activation|SetActive (Variables|Default|GetNS_Smoke_Lasertool1) true true))

(event Custom|ConstructEvent
  (Utilities|FlowControl|Sequence
    (:then_0
      (bind _asvrgame_mode (Utilities|Casting|CastToVRGameMode (Game|GetGameMode)))
      (EventDispatchers|AssignOnPlayerLogoutDelegate _asvrgame_mode (delegate Custom|OnPlayerLogoutDelegate_Event)))
    (:then_1
      (EventDispatchers|AssignOnGrabbed (Variables|Default|GetGrabComponentSnap) (delegate Custom|OnGrabbed_Event)))
    (:then_2
      ;[1 1 1] Holster Stuff
      (EventDispatchers|BindEventtoOnDropped (Variables|Default|GetGrabComponentSnap) (delegate Custom|OnLaserToolDropped)))))

(event Custom|OnGrabbed_Event
  (Collision|SetCollisionEnabled (Variables|Default|GetSkeletalMeshGun) "QueryAndPhysics"))

(event Custom|ServerPlaySmokeVFX
  ;[0.7838 1 0.4879] Begin firing the laser if it's fireable. If not, just play the fizzle sound.
  (CallFunction|PlaySmokeVFX))

(event Custom|server%20set%20firing
  (params (enabled :type Boolean))
  (Variables|Default|Setfiring enabled))

(event EventTick
  (params (DeltaSeconds :type Float%20%28single-precision%29))
  (bind _muzzlelocation (Variables|Default|GetMuzzleLocation))
  (bind (_outhit _outportalhit _tracedthroughportal _returnvalue) (Class|ExtraBlueprintFunctionLibrary|PortalLineTrace (Transformation|GetWorldLocation _muzzlelocation) (Math|Vector|GetForwardVector _muzzlelocation) (Variables|LaserTool|GetlaserRange) "TraceTypeQuery1" false 0 "None" true "(R=1.000000,G=0.000000,B=0.000000,A=1.000000)" "(R=0.000000,G=1.000000,B=0.000000,A=1.000000)" 1.0))
  (if _returnvalue
    (Variables|Default|SetimpactPt (.ImpactPoint (Collision|BreakHitResult _outhit)))
    (Variables|Default|SetlaserPtsArray (select _tracedthroughportal (Utilities|Array|MakeArray (.TraceStart (Collision|BreakHitResult _outportalhit)) (.ImpactPoint (Collision|BreakHitResult _outportalhit)) (.TraceStart (Collision|BreakHitResult _outhit)) (.ImpactPoint (Collision|BreakHitResult _outhit))) (Utilities|Array|MakeArray (.TraceStart (Collision|BreakHitResult _outhit)) (.ImpactPoint (Collision|BreakHitResult _outhit)))))
    (if (Physics|IsSimulatingPhysics (.HitComponent (Collision|BreakHitResult _outhit)) "None")
      (Class|PrimitiveComponent|AddForceatLocation (.HitComponent (Collision|BreakHitResult _outhit)) (* (Math|Vector|GetForwardVector (Variables|Default|GetMuzzleLocation)) 1e+03) (.ImpactPoint (Collision|BreakHitResult _outhit)) "None"))
    (Networking|SwitchHasAuthority
      (:Authority
        (Class|Taggable|OnTagged(Message) (.HitActor (Collision|BreakHitResult _outhit)) _outhit self)))
    (else
      (Variables|Default|SetimpactPt "99999.000000,99999.000000,99999.000000")
      (Variables|Default|SetlaserPtsArray (select _tracedthroughportal (Utilities|Array|MakeArray (.TraceStart (Collision|BreakHitResult _outportalhit)) (.ImpactPoint (Collision|BreakHitResult _outportalhit)) (.TraceStart (Collision|BreakHitResult _outhit)) (.TraceEnd (Collision|BreakHitResult _outhit))) (Utilities|Array|MakeArray (.TraceStart (Collision|BreakHitResult _outhit)) (.TraceEnd (Collision|BreakHitResult _outhit))))))))

(event EventBeginInteract
  (params (heldController :type Motion%20Controller%20Component%20Object%20Reference))
  ;[0.7838 1 0.4879] Begin firing the laser if it's fireable. If not, just play the fizzle sound.
  (Utilities|FlowControl|DoOnce false :!label _label
    (:Completed
      (Utilities|FlowControl|Sequence
        (:then_0
          (Utilities|FlowControl|Delay 0.2)
          (goto _label Reset))
        (:then_1
          (if (Variables|Default|Getfireable)
            (Class|PlayerController|PlayHapticEffect (Game|GetPlayerController 0) "/Game/Haptics/PistolFireHapticEffect.PistolFireHapticEffect" (Default|GetHeldbyHand (Variables|Default|GetGrabComponentSnap)) 0.5 true)
            (Components|Activation|SetActive (Variables|Default|GetNS_LaserBeam) true false)
            (Networking|SwitchHasAuthority
              (:Authority
                _)
              (:Remote
                _))
            (Audio|Components|Audio|Play (Variables|Default|GetCue_LaserFireStart) 0.0)
            (Audio|Components|Audio|Play (Variables|Default|GetCue_LaserFireLoop) 0.0)
            (Actor|Tick|SetActorTickEnabled true)
            (CallFunction|ServerSetFiring true)
            (else
              (Class|PlayerController|PlayHapticEffect (Game|GetPlayerController 0) "/Game/Haptics/TriggerHapticEffect.TriggerHapticEffect" (Default|GetHeldbyHand (Variables|Default|GetGrabComponentSnap)) 3.0 false)
              (Audio|Components|Audio|Play (Variables|Default|GetCue_LaserFizzle) 0.0)
              (CallFunction|ServerPlaySmokeVFX))))))))

(event EventBeginPlay
  (bind _grabcomponentsnap (Variables|Default|GetGrabComponentSnap))
  (bind _grabbingcomponentref (Variables|/Game/Blueprints/Components/GrabComponent.GrabComponent_C|GetgrabbingComponentRef _grabcomponentsnap))
  (Networking|SwitchHasAuthority
    (:Authority
      (Utilities|FlowControl|DelayUntilNextTick)
      (bind _asvrpawn (Utilities|Casting|CastToVRPawn (Components|GetOwner))
        (:then
          (bind _output_get (Variables|Default|SetplayerReference _asvrpawn))
          (Variables|Default|SetPlayerID (Variables|/Game/Blueprints/Actors/VRPawn.VRPawn_C|GetPlayerID _output_get))
          (Variables|/Game/Blueprints/Components/GrabComponent.GrabComponent_C|SetbSimulateOnDrop (Variables|Default|GetGrabComponentSnap) true)
          (Utilities|IsValid (Variables|/Game/Blueprints/Components/GrabComponent.GrabComponent_C|GetgrabbingComponentRef (Variables|Default|GetGrabComponentSnap))
            (:Is%20Not%20Valid
              (CallFunction|AttachtoHolster))))
        (:CastFailed
          (Development|PrintString "ERROR: FAILED TO FIND OWNING PLAYER FOR LASER TOOL." true true "(R=1.000000,G=0.082119,B=0.000000,A=1.000000)" 1e+01))))
    (:Remote
      ;[1 1 1] If no player reference found, keep trying with a set amount of time, trail interval increment exponentially
      (Utilities|IsValid (Variables|Default|GetplayerReference) :!label _label
        (:Is%20Valid
          (Utilities|IsValid _grabbingcomponentref
            (:Is%20Valid
              (Transformation|SetActorLocation (Transformation|GetWorldLocation _grabbingcomponentref) false false))
            (:Is%20Not%20Valid
              (CallFunction|AttachtoHolster))))
        (:Is%20Not%20Valid
          (Utilities|FlowControl|Delay (Math|Float|Power 2.0 (Math|Conversions|ToFloat(Integer) (Variables|InitialSync|Gettrail))))
          (Math|Integer|IncrementInt (Variables|InitialSync|Gettrail)
            (:%20%20
              (if (> (Variables|InitialSync|Gettrail) (Variables|InitialSync|GettotalTrail))
                (Development|PrintString (Utilities|String|Append "No player reference for " (Utilities|GetDisplayName self)) true true "(R=1.000000,G=0.806373,B=0.000000,A=1.000000)" 1e+01)
                (else
                  (goto _label))))))))))

(event EventEndInteract
  (params (heldController :type Motion%20Controller%20Component%20Object%20Reference))
  (Components|Activation|SetActive (Variables|Default|GetNS_LaserBeam) false false)
  (Class|PlayerController|StopHapticEffect (Game|GetPlayerController 0) (Default|GetHeldbyHand (Variables|Default|GetGrabComponentSnap)))
  (Audio|Components|Audio|Stop (Variables|Default|GetCue_LaserFireLoop))
  (Actor|Tick|SetActorTickEnabled false)
  (CallFunction|ServerSetFiring false))

(fn ConstructionScript
  (CallFunction|ConstructEvent))

(fn OnRepGunMaterial
  (Rendering|Material|SetMaterial (Variables|Default|GetSkeletalMeshGun) 0 (Variables|Default|GetGunMaterial)))

(fn OnRepPlayerID
  (bind _skeletalmeshgun (Variables|Default|GetSkeletalMeshGun))
  (Utilities|FlowControl|Sequence
    (:then_0
      (switch int (Variables|Default|GetPlayerID)
        (:Default
          (Development|PrintString "Error from Pistol::InitializePistol, player ID is not 0 or 1, invliad ID" true true "(R=1.000000,G=0.013146,B=0.000000,A=1.000000)" 6e+01))
        (:0
          (Rendering|Material|SetMaterial _skeletalmeshgun 0 "/Game/Assets/Materials/MaterialInstance/CharacterMI/MI_Cel_LaserToolScientist.MI_Cel_LaserToolScientist")
          (Variables|/Game/Blueprints/Components/GrabComponent.GrabComponent_C|SetOnlyOnePlayerGrabbaleTag (Variables|Default|GetGrabComponentSnap) "(TagName=\"OnlyOnePlayerGrabbable.P1\")"))
        (:1
          (Rendering|Material|SetMaterial _skeletalmeshgun 0 "/Game/Assets/Materials/MaterialInstance/CharacterMI/MI_Cel_LaserToolEngineer.MI_Cel_LaserToolEngineer")
          (Variables|/Game/Blueprints/Components/GrabComponent.GrabComponent_C|SetOnlyOnePlayerGrabbaleTag (Variables|Default|GetGrabComponentSnap) "(TagName=\"OnlyOnePlayerGrabbable.P2\")"))))))

(fn OnRepImpactPt
  (bind _impactpt (Variables|Default|GetimpactPt))
  (Class|NiagaraComponent|SetVariablePosition (Variables|Default|GetNS_LaserBeam) "LaserEnd" _impactpt)
  (Class|NiagaraComponent|SetVariablePosition (Variables|Default|GetNS_LaserDrawPattern) "impactPos" _impactpt))

(fn OnRepLaserPtsArray
  (bind _laserptsarray (Variables|Default|GetlaserPtsArray))
  (bind _ns_laserbeam (Variables|Default|GetNS_LaserBeam))
  (bind _laserptsarray_2 (Variables|Default|GetlaserPtsArray))
  (Class|NiagaraDataInterfaceArrayFunctionLibrary|SetNiagaraArrayVector _ns_laserbeam "LaserPoints" _laserptsarray_2)
  (Niagara|SetNiagaraVariable(Float) _ns_laserbeam "LaserLength" (Math|Vector|VectorLength (- (Utilities|Array|Get(acopy) _laserptsarray_2 1) (Utilities|Array|Get(acopy) _laserptsarray_2))))
  (if (== (Utilities|Array|Length _laserptsarray) 4)
    (Niagara|SetNiagaraVariable(Vector3) _ns_laserbeam "SplashAxis" (Math|Vector|Normalize (Math|Transform|InverseTransformDirection (Transformation|GetActorTransform) (- (Utilities|Array|Get(acopy) _laserptsarray 2) (Utilities|Array|Get(acopy) _laserptsarray 3)))))
    (else
      (Niagara|SetNiagaraVariable(Vector3) _ns_laserbeam "SplashAxis" "0.000000,-1.000000,0.000000"))))

(fn OnRepFireable
  (bind _grabcomponentsnap (Variables|Default|GetGrabComponentSnap))
  (if (Variables|/Game/Blueprints/Components/GrabComponent.GrabComponent_C|GetbIsHeld _grabcomponentsnap)
    (Class|PlayerController|PlayHapticEffect (Game|GetPlayerController 0) "/Game/Haptics/TriggerHapticEffect.TriggerHapticEffect" (Default|GetHeldbyHand _grabcomponentsnap) 3.0 false))
  (if (not (Variables|Default|Getfireable))
    (Actor|Tick|SetActorTickEnabled false)
    (Audio|Components|Audio|Stop (Variables|Default|GetCue_LaserFireLoop))
    (Audio|Components|Audio|Play (Variables|Default|GetCue_LaserFizzle) 0.0)
    (Components|Activation|SetActive (Variables|Default|GetNS_LaserBeam) false false)))

(fn OnRepFiring
  (bind _firing (Variables|Default|Getfiring))
  (bind _cue_laserfireloop (Variables|Default|GetCue_LaserFireLoop))
  (Actor|Tick|SetActorTickEnabled (and (Variables|Default|Getfireable) _firing))
  (Components|Activation|SetActive (Variables|Default|GetNS_LaserBeam) _firing false)
  (if _firing
    (if (not (Audio|Components|Audio|IsPlaying _cue_laserfireloop))
      (Audio|Components|Audio|Play (Variables|Default|GetCue_LaserFireStart) 0.0)
      (Audio|Components|Audio|Play _cue_laserfireloop 0.0))
    (else
      (Audio|Components|Audio|Stop _cue_laserfireloop))))

(fn AttachtoHolster
  (bind _playerreference (Variables|Default|GetplayerReference))
  (bind _playerskeletalmesh (Variables|/Game/Blueprints/Actors/VRPawn.VRPawn_C|GetPlayerSkeletalMesh _playerreference))
  (bind _returnvalue (Transformation|GetSocketTransform _playerskeletalmesh "ChestSocket" "RTS_World"))
  (Default|SetPrimitiveCompPhysics (Variables|Default|GetGrabComponentSnap) false)
  (Collision|SetCollisionEnabled (Variables|Default|GetSkeletalMeshGun) "QueryOnly")
  (Transformation|AttachComponentToComponent (Variables|/Game/Blueprints/Actors/VRPawn.VRPawn_C|GetPlayerSkeletalMesh (Variables|Default|GetplayerReference)) "ChestSocket" "SnapToTarget" "SnapToTarget" "KeepWorld" false)
  (Transformation|SetActorLocationAndRotation (.location _returnvalue) (.rotation _returnvalue)))

(fn OnRepDrawingID
  (Class|NiagaraComponent|SetVariableInt (Variables|Default|GetNS_LaserDrawPattern) "CurrentID" (Variables|Default|GetDrawingID)))

(fn OnRepSmokeVFX)