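; VR onboarding prompt actor that shows dialogue text on a WB_OnboardingPrompt widget floating in front of the player's camera.
; It takes the VRCamera from VRGameMode's pawn-spawned event, then each Tick places the widget ahead of and below it, facing the camera.
; DisplayDialogue sets the text and ClearDialogueUI hides the widget.
; Debug keys feed simulated controller button names to HandlePlayerInput; Enhanced Input handlers and ShowPrompt are empty.
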(event Custom|HandleVRPawnSpawned
  (params (VRPawn :type Actor%20Object%20Reference))
  (bind _asvrpawn (Utilities|Casting|CastToVRPawn VRPawn))
  (Variables|Default|SetVRCamera (Variables|/Game/Blueprints/Actors/VRPawn.VRPawn_C|GetCamera _asvrpawn)))

(event Input|EnhancedActionEvents|EnhancedInputActionIA_Menu_Toggle_Left
  (params (ActionValue :type Boolean) (ElapsedSeconds :type Float%20%28double-precision%29) (TriggeredSeconds :type Float%20%28double-precision%29) (InputAction :type Input%20Action%20Object%20Reference :default "/Game/Input/Actions/IA_Menu_Toggle_Left.IA_Menu_Toggle_Left")))

(event Input|EnhancedActionEvents|EnhancedInputActionIA_Menu_Toggle_Right
  (params (ActionValue :type Boolean) (ElapsedSeconds :type Float%20%28double-precision%29) (TriggeredSeconds :type Float%20%28double-precision%29) (InputAction :type Input%20Action%20Object%20Reference :default "/Game/Input/Actions/IA_Menu_Toggle_Right.IA_Menu_Toggle_Right")))

(event Input|EnhancedActionEvents|EnhancedInputActionIA_Move
  (params (ActionValue :type Float%20%28double-precision%29) (ElapsedSeconds :type Float%20%28double-precision%29) (TriggeredSeconds :type Float%20%28double-precision%29) (InputAction :type Input%20Action%20Object%20Reference :default "/Game/Input/Actions/IA_Move.IA_Move")))

(event Input|EnhancedActionEvents|EnhancedInputActionIA_Turn
  (params (ActionValue :type Float%20%28double-precision%29) (ElapsedSeconds :type Float%20%28double-precision%29) (TriggeredSeconds :type Float%20%28double-precision%29) (InputAction :type Input%20Action%20Object%20Reference :default "/Game/Input/Actions/IA_Turn.IA_Turn")))

(event Input|EnhancedActionEvents|EnhancedInputActionIA_Grab_Left
  (params (ActionValue :type Float%20%28double-precision%29) (ElapsedSeconds :type Float%20%28double-precision%29) (TriggeredSeconds :type Float%20%28double-precision%29) (InputAction :type Input%20Action%20Object%20Reference :default "/Game/Input/Actions/IA_Grab_Left.IA_Grab_Left")))

(event Input|EnhancedActionEvents|EnhancedInputActionIA_Grab_Right
  (params (ActionValue :type Float%20%28double-precision%29) (ElapsedSeconds :type Float%20%28double-precision%29) (TriggeredSeconds :type Float%20%28double-precision%29) (InputAction :type Input%20Action%20Object%20Reference :default "/Game/Input/Actions/IA_Grab_Right.IA_Grab_Right")))

(event Input|EnhancedActionEvents|EnhancedInputActionIA_Left_Trigger
  (params (ActionValue :type Boolean) (ElapsedSeconds :type Float%20%28double-precision%29) (TriggeredSeconds :type Float%20%28double-precision%29) (InputAction :type Input%20Action%20Object%20Reference :default "/Game/Input/Actions/IA_Left_Trigger.IA_Left_Trigger")))

(event Input|EnhancedActionEvents|EnhancedInputActionIA_Right_Trigger
  (params (ActionValue :type Boolean) (ElapsedSeconds :type Float%20%28double-precision%29) (TriggeredSeconds :type Float%20%28double-precision%29) (InputAction :type Input%20Action%20Object%20Reference :default "/Game/Input/Actions/IA_Right_Trigger.IA_Right_Trigger")))

(event EventTick
  (params (DeltaSeconds :type Float%20%28single-precision%29))
  (bind _widget (Variables|Default|GetWidget))
  (bind _vrcamera (Variables|Default|GetVRCamera))
  (bind _returnvalue (Transformation|GetWorldLocation _vrcamera))
  (Transformation|SetWorldLocation _widget (+ (+ _returnvalue (* (Math|Vector|GetForwardVector _vrcamera) 3e+02)) "0.000000,0.000000,-100.000000") false false)
  (Transformation|SetWorldRotation _widget (Math|Rotator|FindLookatRotation (Transformation|GetWorldLocation _widget) _returnvalue) false false))

(event Collision|EventActorBeginOverlap
  (params (OtherActor :type Actor%20Object%20Reference)))

(event EventDisplayDialogue
  (params (Text :type String))
  (bind _aswb_onboarding_prompt (Utilities|Casting|CastToWB_OnboardingPrompt (UserInterface|GetUserWidgetObject (Variables|Default|GetWidget))))
  (Rendering|Components|TextRender|SetText (Variables|/Game/Blueprints/UI/WB_OnboardingPrompt.WB_OnboardingPrompt_C|GetPromptText _aswb_onboarding_prompt) (Utilities|Text|ToText(String) Text)))

(event EventBeginPlay
  (bind _returnvalue (Game|GetPlayerController 0))
  (bind _asvrgame_mode (Utilities|Casting|CastToVRGameMode (Game|GetGameMode)))
  (EventDispatchers|BindEventtoOnVRPawnSpawned _asvrgame_mode (delegate Custom|HandleVRPawnSpawned))
  (Input|EnableInput _returnvalue)
  (Input|AddMappingContext (PlayerController|LocalPlayerSubsystems|GetEnhancedInputLocalPlayerSubsystem _returnvalue) "/Game/Input/IMC_Default.IMC_Default" 0 "(bIgnoreAllPressedKeysUntilRelease=True,bForceImmediately=False,bNotifyUserSettings=False)"))

(event EventClearDialogueUI
  (bind _aswb_onboarding_prompt (Utilities|Casting|CastToWB_OnboardingPrompt (UserInterface|GetUserWidgetObject (Variables|Default|GetWidget))))
  (Widget|SetVisibility _aswb_onboarding_prompt "Hidden"))

(event Input|KeyboardEvents|DebugKeySpaceBar
  (params (Key :type Key%20Structure :default "None") (ActionValue :type Input%20Action%20Value%20Structure))
  (:Pressed
    (Class|DialogueManager|HandlePlayerInput "A/X_Button")))

(event Input|KeyboardEvents|DebugKeyB
  (params (Key :type Key%20Structure :default "None") (ActionValue :type Input%20Action%20Value%20Structure))
  (:Pressed
    (Class|DialogueManager|HandlePlayerInput "Teleport_BothButtons")))

(event Input|KeyboardEvents|DebugKeyN
  (params (Key :type Key%20Structure :default "None") (ActionValue :type Input%20Action%20Value%20Structure))
  (:Pressed
    (Class|DialogueManager|HandlePlayerInput "Teleport_BothButtons")))

(event Input|KeyboardEvents|DebugKeyV
  (params (Key :type Key%20Structure :default "None") (ActionValue :type Input%20Action%20Value%20Structure))
  (:Pressed
    (Class|DialogueManager|HandlePlayerInput "Grab_Button")))

(event Input|KeyboardEvents|DebugKeyM
  (params (Key :type Key%20Structure :default "None") (ActionValue :type Input%20Action%20Value%20Structure))
  (:Pressed
    (Class|DialogueManager|HandlePlayerInput "Trigger_Button")))

(fn ConstructionScript)

(fn ShowPrompt
  (params (IndexValue :type Integer)))