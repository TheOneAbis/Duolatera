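; BP_DialoguePrompt is a VR onboarding dialogue prompt that shows text and a controller image in a WB_OnboardingPromptHUD widget.
; On BeginPlay it attaches to the VRPawn, then each Tick eases toward a point in front of the camera, slightly below eye height, facing the player.
; DisplayDialogue fades text in via a timeline, hiding the widget when text is empty.
; DuringDialogue saves a game-instance checkpoint at one specific dialogue entry.
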(event EventTick
  (params (DeltaSeconds :type Float%20%28single-precision%29))
  (bind _vrpawnref (Variables|Default|GetVRPawnRef))
  (bind _uidistancetowardcamera (Variables|Default|GetUIDistanceTowardCamera))
  (bind _followspeed (Variables|Default|GetFollowSpeed))
  (bind _rootcomponent (Variables|Transformation|GetRootComponent))
  (bind _rootcomponent_2 (Variables|Transformation|GetRootComponent))
  (bind _returnvalue (Transformation|GetActorTransform _vrpawnref))
  (bind _returnvalue_2 (* DeltaSeconds _followspeed))
  (bind _camera (Variables|/Game/Blueprints/Actors/VRPawn.VRPawn_C|GetCamera _vrpawnref))
  (bind _relativelocation (Variables|/Script/Engine.SceneComponent|GetRelativeLocation _rootcomponent_2))
  (bind _relativelocation_2 (Variables|/Script/Engine.SceneComponent|GetRelativeLocation _rootcomponent))
  (bind _returnvalue_3 (Math|Vector|GetForwardVector _camera))
  (bind _relativelocation_3 (Variables|/Script/Engine.SceneComponent|GetRelativeLocation _camera))
  (bind _returnvalue_4 (Math|Transform|InverseTransformDirection _returnvalue _returnvalue_3))
  (bind _returnvalue_5 (+ _relativelocation_3 _returnvalue_4))
  (bind _returnvalue_6 (Math|Rotator|FindLookatRotation _relativelocation_3 _returnvalue_5))
  (bind _returnvalue_7 (Math|Vector|RotateVector (Math|Vector|MakeVector _uidistancetowardcamera 0.0 0.0) _returnvalue_6))
  (bind _returnvalue_8 (+ _relativelocation_3 _returnvalue_7))
  (bind _returnvalue_9 (- _returnvalue_8 _relativelocation))
  (bind _returnvalue_10 (* _returnvalue_9 _returnvalue_2))
  (bind _returnvalue_11 (+ _relativelocation_2 _returnvalue_10))
  ;[0.1094 0.349 0.05354] Float the menu toward in front of the player's view
  (Transformation|SetRelativeRotation _rootcomponent_2 (Math|Rotator|FindLookatRotation _relativelocation _relativelocation_3) false false)
  (Transformation|SetRelativeLocation _rootcomponent (Math|Vector|MakeVector (.x _returnvalue_11) (.y _returnvalue_11) (- (.z (Variables|/Script/Engine.SceneComponent|GetRelativeLocation (Variables|/Game/Blueprints/Actors/VRPawn.VRPawn_C|GetCamera (Variables|Default|GetVRPawnRef)))) 15.0)) false false))

(event EventDuringDialogue
  ;[1 1 1] Update Checkpoint
  (if (== (Variables|Default|GetCurrentEntryID) 8)
    (bind _asvrgame_instance (Utilities|Casting|CastToVRGameInstance (Game|GetGameInstance)))
    (Default|SavetoCheckpoint _asvrgame_instance 1)))

(event EventUpdateUIImage
  (params (image :type Texture%202D%20Object%20Reference))
  ;[0.9923 0.6317 1] Update UI Image here
  (bind _aswb_onboarding_prompt_hud (Utilities|Casting|CastToWB_OnboardingPromptHUD (UserInterface|GetUserWidgetObject (Variables|Default|GetWidget))))
  (Class|Image|SetBrush (Variables|/Game/Blueprints/UI/WB_OnboardingPromptHUD.WB_OnboardingPromptHUD_C|GetController_Texture _aswb_onboarding_prompt_hud) (Class|WidgetBlueprintLibrary|MakeBrushfromTexture image 1 1)))

(event EventDisplayDialogue
  (params (Text :type String))
  (bind _widget (Variables|Default|GetWidget))
  (bind _returnvalue (UserInterface|GetUserWidgetObject _widget))
  (if (Utilities|Array|IsEmpty Text)
    (bind _aswb_onboarding_prompt_hud (Utilities|Casting|CastToWB_OnboardingPromptHUD _returnvalue))
    (Widget|SetVisibility _aswb_onboarding_prompt_hud "Hidden")
    (else
      (bind _aswb_onboarding_prompt_hud_2 (Utilities|Casting|CastToWB_OnboardingPromptHUD _returnvalue))
      (Rendering|Components|TextRender|SetText (Variables|/Game/Blueprints/UI/WB_OnboardingPromptHUD.WB_OnboardingPromptHUD_C|GetPromptText _aswb_onboarding_prompt_hud_2) (Utilities|Text|ToText(String) Text))
      (Widget|SetVisibility _aswb_onboarding_prompt_hud_2 "Visible")
      (bind _time (Timeline|widget%20fade-in PlayFromStart)
        (:Update
          (Widget|SetRenderOpacity (UserInterface|GetWidget (Variables|Default|GetWidget)) _time))))))

(event EventBeginPlay
  ;[0.2815 0.4167 0.07157] Attach this dialogue prompt to the player's VR origin and enable input handling
  (bind _returnvalue (Actor|GetActorOfClass "/Game/Blueprints/Actors/VRPawn.VRPawn_C"))
  (bind _output_get (Variables|Default|SetVRPawnRef _returnvalue))
  (Transformation|AttachActorToActor _output_get "None" "KeepRelative" "KeepRelative" "KeepRelative" false)
  (Input|EnableInput (Game|GetPlayerController 0)))

(event EventClearDialogueUI
  (bind _aswb_onboarding_prompt_hud (Utilities|Casting|CastToWB_OnboardingPromptHUD (UserInterface|GetUserWidgetObject (Variables|Default|GetWidget))))
  (Widget|SetVisibility _aswb_onboarding_prompt_hud "Hidden"))

(fn ConstructionScript)