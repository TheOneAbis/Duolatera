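; Spline actor that lays a stripe of randomly picked glyphs along its path, built in the construction script.
; AdjustSplinePoint first adjusts the spline using detection, expansion and snapping settings.
; When GenerateMesh is set, fixed-length spline mesh sections follow it with a rotatable up vector.
; Each section gets a dynamic M_GlyphStripe material that picks a random sheet cell; the Event Graph holds only an unconnected older copy.
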(event EventBeginPlay)

(event Collision|EventActorBeginOverlap
  (params (OtherActor :type Actor%20Object%20Reference)))

(event EventTick
  (params (DeltaSeconds :type Float%20%28single-precision%29)))

(fn ConstructionScript
  (bind _spline (Variables|Default|GetSpline))
  (Utilities|FlowControl|Sequence
    (:then_0
      (Class|ExtraBlueprintFunctionLibrary|AdjustSplinePoint self (Variables|Default|GetSpline) (Variables|Default|GetDetectRadius) (Variables|Default|GetExpandDistance) (Variables|Default|GetSnappingMargin) (Variables|Default|GetbShowDebugDrawing)))
    (:then_1
      (if (Variables|Default|GetGenerateMesh)
        (for _index (range 0 (- (Math|Float|Truncate (/ (Spline|GetSplineLength (Variables|Default|GetSpline)) (Variables|Default|GetSectionLength))) 1))
          (bind _returnvalue (AddComponent|AddSplineMeshComponent false))
          (SplineMesh|SetForwardAxis _returnvalue "X" true)
          (SplineMesh|SetSplineUpDir _returnvalue (Math|Vector|RotateVectorAroundAxis (Class|SplineComponent|GetUpVectoratDistanceAlongSpline _spline (* _index (Variables|Default|GetSectionLength)) "Local") (Variables|Default|GetRotateSplineUp) (Spline|GetTangentatDistanceAlongSpline _spline (* _index (Variables|Default|GetSectionLength)) "Local")) true)
          (bind (_position _tangent) (CallFunction|GetPosTangent _index false))
          (bind (_position_2 _tangent_2) (CallFunction|GetPosTangent _index true))
          (Components|StaticMesh|SetStaticMesh _returnvalue (Variables|Default|GetSampleMesh))
          (bind _returnvalue_2 (Rendering|Material|CreateDynamicMaterialInstance "/Game/Assets/Materials/M_GlyphStripe.M_GlyphStripe" "None" "None" :!class /Script/Engine.KismetMaterialLibrary))
          (bind _returnvalue_3 (Rendering|Material|GetScalarParameterValue _returnvalue_2 "SheetDimension" :!class /Script/Engine.MaterialInstanceDynamic))
          (Rendering|Material|SetScalarParameterValue _returnvalue_2 "PickHeight" (Math|Conversions|ToFloat(Integer) (Math|Random|RandomInteger (Math|Float|Truncate _returnvalue_3))) :!class /Script/Engine.MaterialInstanceDynamic)
          (Rendering|Material|SetScalarParameterValue _returnvalue_2 "PickWidth" (Math|Conversions|ToFloat(Integer) (Math|Random|RandomInteger (Math|Float|Truncate _returnvalue_3))) :!class /Script/Engine.MaterialInstanceDynamic)
          (Rendering|Material|SetMaterial _returnvalue 0 _returnvalue_2)
          (SplineMesh|SetStartandEnd _returnvalue _position _tangent _position_2 _tangent_2 true :!class /Script/Engine.SplineMeshComponent))))))

(fn GetPosTangent
  (params (index :type Integer) (EndPoint :type Boolean))
  (bind _returnvalue (+ index EndPoint))
  (bind _sectionlength (Variables|Default|GetSectionLength))
  (bind _spline (Variables|Default|GetSpline))
  (bind _returnvalue_2 (* _returnvalue _sectionlength))
  (return (Spline|GetLocationatDistanceAlongSpline _spline _returnvalue_2 "Local") (Spline|GetTangentatDistanceAlongSpline _spline _returnvalue_2 "Local")))