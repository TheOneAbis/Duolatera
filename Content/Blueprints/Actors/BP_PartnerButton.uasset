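; BP_PartnerButton is a networked VR button that, when held at the same time as its linked partner button, opens two interactables.
; Box overlaps drive light glow and haptics, while the server sets IsPressed for VR pawns.
; The IsPressed OnRep slides the button and checks the partner's state.
; When both are pressed, it calls server RPCs marking both activated, sends door-open messages, and pins both buttons pressed and lit.
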(event OnComponentEndOverlap(Box)
  (params (OverlappedComponent :type Primitive%20Component%20Object%20Reference) (OtherActor :type Actor%20Object%20Reference) (OtherComp :type Primitive%20Component%20Object%20Reference) (OtherBodyIndex :type Integer))
  ;[0.6198 0.6198 0.6198] End Overlap
  (if (not (Variables|Default|GetbActorsActivated))
    (Rendering|Material|SetScalarParameterValueonMaterials (Variables|Default|GetLight) "Intensity" (Variables|Default|GetIntensity))
    (Utilities|FlowControl|Sequence
      (:then_0
        (CallFunction|TriggerPlaysHapticEffect OtherComp (Variables|Default|GetHapticEffect)))
      (:then_1
        (Utilities|Casting|CastToVRPawn OtherActor)
        (Networking|SwitchHasAuthority
          (:Authority
            (if (Variables|Default|GetbIsPressed)
              (Variables|Default|SetbIsPressed false))))))))

(event OnComponentBeginOverlap(Box)
  (params (OverlappedComponent :type Primitive%20Component%20Object%20Reference) (OtherActor :type Actor%20Object%20Reference) (OtherComp :type Primitive%20Component%20Object%20Reference) (OtherBodyIndex :type Integer) (bFromSweep :type Boolean) (SweepResult :type Hit%20Result%20Structure%20%28by%20ref%29))
  ;[0.6458 0.6458 0.6458] Begin Overlap
  (if (not (Variables|Default|GetbActorsActivated))
    (Rendering|Material|SetScalarParameterValueonMaterials (Variables|Default|GetLight) "Intensity" (+ (Variables|Default|GetIntensity) 3e+01))
    (Utilities|FlowControl|Sequence
      (:then_0
        (CallFunction|TriggerPlaysHapticEffect OtherComp (Variables|Default|GetHapticEffect)))
      (:then_1
        (Utilities|Casting|CastToVRPawn OtherActor)
        (Networking|SwitchHasAuthority
          (:Authority
            (if (not (Variables|Default|GetbIsPressed))
              (Variables|Default|SetbIsPressed true))))))))

(event Custom|RPC_Server_SetActorsActivated
  ;[0.6406 0.6406 0.6406] RPC Function
  (Variables|Default|SetbActorsActivated true))

(event Custom|PressButtonIn
  (bind _bp_partnerbutton (Variables|Default|GetBP_PartnerButton))
  ;[0.6198 0.6198 0.6198] OnRep Events
  (if (not (Variables|Default|GetbActorsActivated))
    (Components|MoveComponentTo (Variables|Default|GetButton) (- (Variables|Default|GetButtonStart) "0.000000,20.000000,0.000000") "0, 0, 0" false false 0.1 false)
    (if (Variables|BP_PartnerButton_C|GetbIsPressed _bp_partnerbutton)
      (CallFunction|RPCServerSetActorsActivated)
      (CallFunction|RPCServerSetActorsActivated _bp_partnerbutton)
      (Class|BPIDoorInteractable|DoorInteractOpen(Message) (Variables|Default|GetInteractable1))
      (Class|BPIDoorInteractable|DoorInteractOpen(Message) (Variables|Default|GetInteractable2))
      (Utilities|FlowControl|Delay 0.05)
      (CallFunction|SetBothButtonACtivated))))

(event Custom|PressButtonOut
  ;[0.6198 0.6198 0.6198] OnRep Events
  (if (not (Variables|Default|GetbActorsActivated))
    (Components|MoveComponentTo (Variables|Default|GetButton) (Variables|Default|GetButtonStart) "0, 0, 0" false false 0.1 false)))

(event Custom|SetBothButtonActivated
  (Utilities|FlowControl|Sequence
    (:then_0
      (Transformation|SetRelativeLocation (Variables|Default|GetButton) (- (Variables|Default|GetButtonStart) "0.000000,20.000000,0.000000") false false)
      (Rendering|Material|SetScalarParameterValueonMaterials (Variables|Default|GetLight) "Intensity" (+ (Variables|Default|GetIntensity) 3e+01)))
    (:then_1
      (Transformation|SetRelativeLocation (Variables|BP_PartnerButton_C|GetButton (Variables|Default|GetBP_PartnerButton)) (- (Variables|Default|GetButtonStart) "0.000000,20.000000,0.000000") false false)
      (Rendering|Material|SetScalarParameterValueonMaterials (Variables|BP_PartnerButton_C|GetLight (Variables|Default|GetBP_PartnerButton)) "Intensity" (+ (Variables|Default|GetIntensity) 3e+01)))))

(event EventBeginPlay
  ;[0.5365 0.5365 0.5365] Button Start Location
  (Variables|Default|SetButtonStart (Variables|/Script/Engine.SceneComponent|GetRelativeLocation (Variables|Default|GetButton))))

(fn ConstructionScript
  (Rendering|Material|SetScalarParameterValueonMaterials (Variables|Default|GetLight) "Intensity" (Variables|Default|GetIntensity)))

(fn OnRepBIsPressed
  (if (Variables|Default|GetbIsPressed)
    (CallFunction|PressButtonin)
    (else
      (CallFunction|PressButtonOut))))