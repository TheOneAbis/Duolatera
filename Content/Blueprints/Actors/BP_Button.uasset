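; Networked VR push button that a VRPawn presses by overlapping its capsule, triggering haptics on the touching motion controller.
; The authority sets IsPushed, whose RepNotify plays or reverses a timeline that moves the orb and toggles its emissive glow.
; The authority calls BeginInteract when the press completes and EndInteract on release.
; Leaving the capsule releases it unless the count of puzzle-activated events has reached the number of ObjectsToActivate, latching it down.
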(event OnComponentBeginOverlap(Capsule)
  (params (OverlappedComponent :type Primitive%20Component%20Object%20Reference) (OtherActor :type Actor%20Object%20Reference) (OtherComp :type Primitive%20Component%20Object%20Reference) (OtherBodyIndex :type Integer) (bFromSweep :type Boolean) (SweepResult :type Hit%20Result%20Structure%20%28by%20ref%29))
  ;[0.5573 0.5573 0.5573] Begin Overlap
  (Utilities|Casting|CastToVRPawn OtherActor)
  (if (not (Variables|Default|GetbIsPushed))
    (Utilities|FlowControl|Sequence
      (:then_0
        (bind _asmotion_controller_component (Utilities|Casting|CastToMotionControllerComponent (Transformation|GetAttachParent (Transformation|GetAttachParent OtherComp))))
        (CallFunction|TriggerPlaysHapticEffect _asmotion_controller_component (Variables|Default|GetHapticEffect)))
      (:then_1
        (Networking|SwitchHasAuthority
          (:Authority
            (if (not (Variables|Default|GetbIsPushed))
              (Variables|Default|SetbIsPushed true))))))))

(event OnComponentEndOverlap(Capsule)
  (params (OverlappedComponent :type Primitive%20Component%20Object%20Reference) (OtherActor :type Actor%20Object%20Reference) (OtherComp :type Primitive%20Component%20Object%20Reference) (OtherBodyIndex :type Integer))
  (Utilities|Casting|CastToVRPawn OtherActor)
  (Networking|SwitchHasAuthority
    (:Authority
      (if (Variables|Default|GetbIsPushed)
        (if (< (Variables|Default|GetActivatedPuzzles) (Utilities|Array|Length (Variables|Default|GetobjectsToActivate)))
          (Variables|Default|SetbIsPushed false))))))

(event Custom|PushButton
  (bind _buttonstart (Variables|Default|GetButtonStart))
  (bind (_direction _alpha) (Timeline|pressTimeline Play)
    (:Update
      (Transformation|SetRelativeLocation (Variables|Default|GetButtonOrb) (Math|Vector|Lerp(Vector) _buttonstart (- _buttonstart "0.000000,0.000000,15.000000") _alpha) false false))
    (:Finished
      (if (Utilities|Enum|Equal(Enum) _direction "Forward")
        (for _array_element (Variables|Default|Getlights)
          (Rendering|Material|SetScalarParameterValueonMaterials _array_element "Emissive Intensity" 5e+01)
          (Networking|SwitchHasAuthority
            (:Authority
              (Class|Interactable|BeginInteract 0))))))))

(event Custom|PopButton
  (bind _buttonstart (Variables|Default|GetButtonStart))
  (Utilities|FlowControl|Sequence
    (:then_0
      (for _array_element (Variables|Default|Getlights)
        (Rendering|Material|SetScalarParameterValueonMaterials _array_element "Emissive Intensity" 0.0)
        (Networking|SwitchHasAuthority
          (:Authority
            (Class|Interactable|EndInteract 0)))))
    (:then_1
      (bind (_direction _alpha) (Timeline|pressTimeline Reverse)
        (:Update
          (Transformation|SetRelativeLocation (Variables|Default|GetButtonOrb) (Math|Vector|Lerp(Vector) _buttonstart (- _buttonstart "0.000000,0.000000,15.000000") _alpha) false false))
        (:Finished
          (if (Utilities|Enum|Equal(Enum) _direction "Forward")
            (for _array_element_2 (Variables|Default|Getlights)
              (Rendering|Material|SetScalarParameterValueonMaterials _array_element_2 "Emissive Intensity" 5e+01)
              (Networking|SwitchHasAuthority
                (:Authority
                  (Class|Interactable|BeginInteract 0))))))))))

(event Custom|CountActivatedPuzzles
  (Variables|Default|SetActivatedPuzzles (+ 1 (Variables|Default|GetActivatedPuzzles))))

(event EventBeginPlay
  ;[1 1 1] Button Start Location
  (Variables|Default|Setlights (Utilities|Array|MakeArray (Variables|Default|GetButtonOrb)))
  (Variables|Default|SetButtonStart (Variables|/Script/Engine.SceneComponent|GetRelativeLocation (Variables|Default|GetButtonOrb)))
  (for _array_element (Variables|Default|GetobjectsToActivate)
    (EventDispatchers|BindEventtoOnPuzzleActivated _array_element (delegate Custom|CountActivatedPuzzles))))

(fn ConstructionScript)

(fn OnRepBIsPushed
  (if (Variables|Default|GetbIsPushed)
    (CallFunction|PushButton)
    (else
      (CallFunction|PopButton))))