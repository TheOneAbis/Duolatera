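; BP_GlyphStripe is a PCG actor that lays a stripe of randomized glyph meshes along a spline.
; On authority, its construction script either passes the spline to AdjustSplinePoint for detection and snapping while EditSpline is on, or builds fixed-length spline mesh sections.
; Sections take positions and length-clamped tangents from the spline.
; Each gets a dynamic MI_GlyphStripe instance with random PickWidth and PickHeight values to vary its glyph.
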(event EventBeginPlay)

(event Collision|EventActorBeginOverlap
  (params (OtherActor :type Actor%20Object%20Reference)))

(event EventTick
  (params (DeltaSeconds :type Float%20%28single-precision%29)))

(fn ConstructionScript
  (Networking|SwitchHasAuthority
    (:Authority
      (if (Variables|Default|GetbEditSpline)
        (Class|ExtraBlueprintFunctionLibrary|AdjustSplinePoint self (Variables|Default|GetSpline) (Variables|Default|GetDetectRadius) (Variables|Default|GetExpandDistance) (Variables|Default|GetSnappingMargin) (Variables|Default|GetbShowDebugDrawing))
        (else
          (for _index (range 0 (Math|Float|Truncate (/ (Spline|GetSplineLength (Variables|Default|GetSpline)) (Variables|Default|GetsectionLength))))
            (Variables|Default|SetloopIndex _index)
            (bind _returnvalue (AddComponent|AddSplineMeshComponent false))
            (Components|StaticMesh|SetStaticMesh _returnvalue (Variables|Default|GetsplineMesh))
            (bind (_position _tangent) (CallFunction|GetEndPosTan (Variables|Default|GetloopIndex)))
            (bind (_position_2 _tangent_2) (CallFunction|GetStartPosTan (Variables|Default|GetloopIndex)))
            (SplineMesh|SetStartandEnd _returnvalue _position_2 _tangent_2 _position _tangent true :!class /Script/Engine.SplineMeshComponent)
            (bind _returnvalue_2 (Rendering|Material|CreateDynamicMaterialInstance _returnvalue 0 "/Game/Assets/Materials/MaterialInstance/MI_GlyphStripe.MI_GlyphStripe" "None" :!class /Script/Engine.PrimitiveComponent))
            (Rendering|Material|SetScalarParameterValue _returnvalue_2 "PickWidth" (Math|Conversions|ToFloat(Integer) (Math|Random|RandomInteger 5)) :!class /Script/Engine.MaterialInstanceDynamic)
            (Rendering|Material|SetScalarParameterValue _returnvalue_2 "PickHeight" (Math|Conversions|ToFloat(Integer) (Math|Random|RandomInteger 5)) :!class /Script/Engine.MaterialInstanceDynamic)))))))

(fn GetStartPosTan
  (params (index :type Integer))
  (bind _sectionlength (Variables|Default|GetsectionLength))
  (bind _spline (Variables|Default|GetSpline))
  (bind _returnvalue (* index _sectionlength))
  (return (Spline|GetLocationatDistanceAlongSpline _spline _returnvalue "Local") (Math|Vector|ClampVectorSize (Spline|GetTangentatDistanceAlongSpline _spline _returnvalue "Local") 0.0 (Variables|Default|GetsectionLength))))

(fn GetEndPosTan
  (params (Index :type Integer))
  (bind _returnvalue (+ Index 1))
  (bind _sectionlength (Variables|Default|GetsectionLength))
  (bind _spline (Variables|Default|GetSpline))
  (bind _returnvalue_2 (* _returnvalue _sectionlength))
  (return (Spline|GetLocationatDistanceAlongSpline _spline _returnvalue_2 "Local") (Math|Vector|ClampVectorSize (Spline|GetTangentatDistanceAlongSpline _spline _returnvalue_2 "Local") 0.0 (Variables|Default|GetsectionLength))))